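; Trigger volume that animates the third-person character's camera to a new framing while the player is inside it.
; On overlap it saves the follow camera and boom transforms and arm length, substitutes them for unset New values, then lerps through nested timelines.
; On exit, separate timelines blend back.
; Both boom transform blends use the saved follow camera location and rotation as the old endpoint, not the saved boom values.
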(event OnComponentBeginOverlap(CameraHitbox)
  (params (OverlappedComponent :type Primitive%20Component%20Object%20Reference) (OtherActor :type Actor%20Object%20Reference) (OtherComp :type Primitive%20Component%20Object%20Reference) (OtherBodyIndex :type Integer) (bFromSweep :type Boolean) (SweepResult :type Hit%20Result%20Structure%20%28by%20ref%29))
  ;[1 1 1] Saving the default values
  (bind _asbp_third_person_character (Utilities|Casting|CastToBP_ThirdPersonCharacter OtherActor))
  (Variables|Default|SetPlayerRef _asbp_third_person_character)
  (Variables|Default|SetOldFollowCameraLocation (Variables|/Script/Engine.SceneComponent|GetRelativeLocation (Variables|/Game/ThirdPerson/Blueprints/BP_ThirdPersonCharacter.BP_ThirdPersonCharacter_C|GetFollowCamera (Variables|Default|GetPlayerRef))))
  (Variables|Default|SetOldFollowCameraRotation (Variables|/Script/Engine.SceneComponent|GetRelativeRotation (Variables|/Game/ThirdPerson/Blueprints/BP_ThirdPersonCharacter.BP_ThirdPersonCharacter_C|GetFollowCamera (Variables|Default|GetPlayerRef))))
  (Variables|Default|SetOldCameraBoomLocation (Variables|/Script/Engine.SceneComponent|GetRelativeLocation (Variables|/Game/ThirdPerson/Blueprints/BP_ThirdPersonCharacter.BP_ThirdPersonCharacter_C|GetCameraBoom (Variables|Default|GetPlayerRef))))
  (Variables|Default|SetOldCamerBoomRotation (Variables|/Script/Engine.SceneComponent|GetRelativeRotation (Variables|/Game/ThirdPerson/Blueprints/BP_ThirdPersonCharacter.BP_ThirdPersonCharacter_C|GetCameraBoom (Variables|Default|GetPlayerRef))))
  (Variables|Default|SetOldCameraBoomArmLength (Variables|/Script/Engine.SpringArmComponent|GetTargetArmLength (Variables|/Game/ThirdPerson/Blueprints/BP_ThirdPersonCharacter.BP_ThirdPersonCharacter_C|GetCameraBoom (Variables|Default|GetPlayerRef))))
  (CallFunction|SetNewValuesforCamera))

(event OnComponentEndOverlap(CameraHitbox)
  (params (OverlappedComponent :type Primitive%20Component%20Object%20Reference) (OtherActor :type Actor%20Object%20Reference) (OtherComp :type Primitive%20Component%20Object%20Reference) (OtherBodyIndex :type Integer))
  (bind _asbp_third_person_character (Utilities|Casting|CastToBP_ThirdPersonCharacter OtherActor))
  (Variables|Default|SetPlayerRef _asbp_third_person_character)
  (CallFunction|ResetBacktoDefaultValuesforCamera))

(event Custom|ResetBackToDefaultValuesForCamera
  ;[1 1 1] Resetting to old Values for the Camera
  ;;[1 1 1] Resetting to old Follow Camera Location and Rotation
  (bind _cameraanimation (Timeline|Timeline_4 Play)
    (:Update
      (Transformation|SetRelativeLocationAndRotation (Variables|/Game/ThirdPerson/Blueprints/BP_ThirdPersonCharacter.BP_ThirdPersonCharacter_C|GetFollowCamera (Variables|Default|GetPlayerRef)) (Math|Vector|Lerp(Vector) (Variables|Default|GetNewFollowCameraLocation) (Variables|Default|GetOldFollowCameraLocation) _cameraanimation) (Math|Rotator|Lerp(Rotator) (Variables|Default|GetNewFollowCameraRotation) (Variables|Default|GetOldFollowCameraRotation) _cameraanimation) false false)
      ;;[1 1 1] Resetting to old Camera Boom Location and Rotation
      (bind _cameraanimation_2 (Timeline|Timeline_3 Play)
        (:Update
          (Transformation|SetRelativeLocationAndRotation (Variables|/Game/ThirdPerson/Blueprints/BP_ThirdPersonCharacter.BP_ThirdPersonCharacter_C|GetCameraBoom (Variables|Default|GetPlayerRef)) (Math|Vector|Lerp(Vector) (Variables|Default|GetNewCameraBoomLocation) (Variables|Default|GetOldFollowCameraLocation) _cameraanimation_2) (Math|Rotator|Lerp(Rotator) (Variables|Default|GetNewCameraBoomRotation) (Variables|Default|GetOldFollowCameraRotation) _cameraanimation_2) false false)
          ;;[1 1 1] Resetting to old Arm Length
          (bind _cameraanimation_3 (Timeline|Timeline_0 Play)
            (:Update
              (Variables|/Script/Engine.SpringArmComponent|SetTargetArmLength (Variables|/Game/ThirdPerson/Blueprints/BP_ThirdPersonCharacter.BP_ThirdPersonCharacter_C|GetCameraBoom (Variables|Default|GetPlayerRef)) (Math|Float|Lerp (Variables|Default|GetNewCameraBoomArmLength) (Variables|Default|GetOldCameraBoomArmLength) _cameraanimation_3)))))))))

(event Custom|SetNewValuesForCamera
  ;[1 1 1] Setting the Values for the Camera
  (CallFunction|CheckFollowCamera)
  ;;[1 1 1] Setting the new Follow Camera Location and Rotation
  (bind _cameraanimation (Timeline|Timeline_1 Play)
    (:Update
      (Transformation|SetRelativeLocationAndRotation (Variables|/Game/ThirdPerson/Blueprints/BP_ThirdPersonCharacter.BP_ThirdPersonCharacter_C|GetFollowCamera (Variables|Default|GetPlayerRef)) (Math|Vector|Lerp(Vector) (Variables|Default|GetOldFollowCameraLocation) (Variables|Default|GetNewFollowCameraLocation) _cameraanimation) (Math|Rotator|Lerp(Rotator) (Variables|Default|GetOldFollowCameraRotation) (Variables|Default|GetNewFollowCameraRotation) _cameraanimation true) false false)
      (CallFunction|CheckCameraBoom)
      ;;[1 1 1] Setting the new Camera Boom Location and Rotation
      (bind _cameraanimation_2 (Timeline|Timeline_2 Play)
        (:Update
          (Transformation|SetRelativeLocationAndRotation (Variables|/Game/ThirdPerson/Blueprints/BP_ThirdPersonCharacter.BP_ThirdPersonCharacter_C|GetCameraBoom (Variables|Default|GetPlayerRef)) (Math|Vector|Lerp(Vector) (Variables|Default|GetOldFollowCameraLocation) (Variables|Default|GetNewCameraBoomLocation) _cameraanimation_2) (Math|Rotator|Lerp(Rotator) (Variables|Default|GetOldFollowCameraRotation) (Variables|Default|GetNewCameraBoomRotation) _cameraanimation_2 true) false false)
          ;;[1 1 1] Setting the new Arm Length
          (bind _cameraanimation_3 (Timeline|Timeline Play)
            (:Update
              (Variables|/Script/Engine.SpringArmComponent|SetTargetArmLength (Variables|/Game/ThirdPerson/Blueprints/BP_ThirdPersonCharacter.BP_ThirdPersonCharacter_C|GetCameraBoom (Variables|Default|GetPlayerRef)) (Math|Float|Lerp (Variables|Default|GetOldCameraBoomArmLength) (Variables|Default|GetNewCameraBoomArmLength) _cameraanimation_3)))))))))

(event Custom|CheckFollowCamera
  ;[1 1 1] Checking the Values of the Follow Camera that they are not empty
  (if (Utilities|Operators|NotEqual(!=) :A (Variables|Default|GetNewFollowCameraRotation))
    _
    (else
      (Variables|Default|SetNewFollowCameraRotation (Variables|Default|GetOldFollowCameraRotation))))
  (if (not (Utilities|Operators|NotEqual(!=) :A (Variables|Default|GetNewFollowCameraLocation)))
    (Variables|Default|SetNewFollowCameraLocation (Variables|Default|GetOldFollowCameraLocation))))

(event Custom|CheckArmLength
  ;[1 1 1] Making sure the Armlength does not get reset when no value change is necessary
  (if (not (> (Variables|Default|GetNewCameraBoomArmLength) 0.0))
    (if (> (Variables|Default|GetOldCameraBoomArmLength) 0.0)
      (Variables|Default|SetNewCameraBoomArmLength (Variables|Default|GetOldCameraBoomArmLength)))))

(event Custom|CheckCameraBoom
  ;[1 1 1] Checking the Values of the Camera Boom that they are not empty
  (if (Utilities|Operators|NotEqual(!=) :A (Variables|Default|GetNewCameraBoomRotation))
    _
    (else
      (Variables|Default|SetNewCameraBoomRotation (Variables|Default|GetOldCamerBoomRotation))))
  (if (Utilities|Operators|NotEqual(!=) :A (Variables|Default|GetNewCameraBoomLocation))
    _
    (else
      (Variables|Default|SetNewCameraBoomLocation (Variables|Default|GetOldCameraBoomLocation))))
  (CallFunction|CheckArmLength))

(fn ConstructionScript)