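; BP_Detect is a mechanics-playground Blueprint that detects when the player is near a BP_RevealBlock.
; Every Tick it gathers all reveal blocks, prints their distance to the player, and sets RevealPlatformIsNear when one is within a fixed range.
; The flag is never cleared or read here.
; BeginPlay caches a BP_LightOrb reference, but the delayed LightPulsing call that uses it is disconnected and never runs.
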(event EventBeginPlay
  (bind _returnvalue (Actor|GetActorOfClass "/Game/MechanicsPlayground/MechanincsBlueprints/BP_LightOrb.BP_LightOrb_C"))
  (Variables|Default|SetBP%20Light%20Orb%20Ref _returnvalue))

(event EventTick
  (params (DeltaSeconds :type Float%20%28single-precision%29))
  (bind _outactors (Actor|GetAllActorsOfClass "/Game/MechanicsPlayground/MechanincsBlueprints/BP_RevealBlock.BP_RevealBlock_C"))
  (for _array_element _outactors
    (Development|PrintString (Utilities|String|ToString(Float) (Math|Vector|Distance(Vector) (Transformation|GetActorLocation _array_element) (Transformation|GetActorLocation (Game|GetPlayerCharacter 0)))))
    (if (< (Math|Vector|Distance(Vector) (Transformation|GetActorLocation _array_element) (Transformation|GetActorLocation (Game|GetPlayerCharacter 0))) 1.5e+03)
      (Development|PrintString "I am detecting")
      (Variables|Default|SetbRevealPlatformIsNear true))))

(fn ConstructionScript)