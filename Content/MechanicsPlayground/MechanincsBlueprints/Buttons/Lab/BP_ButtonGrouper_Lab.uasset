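; BP_ButtonGrouper_Lab manages the group of lab buttons for one room in a sequence tracked by BP_Lab's ActiveGroup.
; When the player enters the Room volume and Position matches ActiveGroup, it activates every button in ButtonList and passes them the player reference.
; Button triggers are cast and forwarded to an empty ButtonTrigger event.
; Deactivate disables the buttons and steps ActiveGroup forward, activating ControlledDoor, or back.
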(event OnComponentBeginOverlap(Room)
  (params (OverlappedComponent :type Primitive%20Component%20Object%20Reference) (OtherActor :type Actor%20Object%20Reference) (OtherComp :type Primitive%20Component%20Object%20Reference) (OtherBodyIndex :type Integer) (bFromSweep :type Boolean) (SweepResult :type Hit%20Result%20Structure%20%28by%20ref%29))
  ;[1 1 1] Comment
  (bind _asbp_third_person_character (Utilities|Casting|CastToBP_ThirdPersonCharacter OtherActor))
  (if (== (Variables|/Game/MechanicsPlayground/MechanincsBlueprints/Buttons/Lab/BP_Lab.BP_Lab_C|GetActiveGroup (Variables|Default|GetLabRef)) (Variables|Default|GetPosition))
    (for _index (range 0 (- (Utilities|Map|Length (Variables|Default|GetButtonList)) 1))
      (if (.ReturnValue (Utilities|Map|Find (Variables|Default|GetButtonList) _index))
        (Variables|/Game/MechanicsPlayground/MechanincsBlueprints/Buttons/Bases/BP_BaseButton.BP_BaseButton_C|SetPlayerRef (.Value (Utilities|Map|Find (Variables|Default|GetButtonList) _index)) _asbp_third_person_character)
        (Variables|/Game/MechanicsPlayground/MechanincsBlueprints/Buttons/Bases/BP_Button_Teamworker_Base.BP_Button_Teamworker_Base_C|SetbIsActive (.Value (Utilities|Map|Find (Variables|Default|GetButtonList) _index)) true)))
    (if (== 1 (Variables|Default|GetPosition))
      (Variables|Default|SetCurrentLocation 0))))

(event Custom|Deactivate
  (params (isGoingForward :type Boolean))
  (bind _labref (Variables|Default|GetLabRef))
  (bind _position (Variables|Default|GetPosition))
  ;[1 1 1] Comment
  (for _index (range 0 (- (Utilities|Map|Length (Variables|Default|GetButtonList)) 1))
    (if (.ReturnValue (Utilities|Map|Find (Variables|Default|GetButtonList) _index))
      (Variables|/Game/MechanicsPlayground/MechanincsBlueprints/Buttons/Bases/BP_Button_Teamworker_Base.BP_Button_Teamworker_Base_C|SetbIsActive (.Value (Utilities|Map|Find (Variables|Default|GetButtonList) _index)) false)))
  (if isGoingForward
    (Variables|/Game/MechanicsPlayground/MechanincsBlueprints/Buttons/Lab/BP_Lab.BP_Lab_C|SetActiveGroup _labref (+ _position 1))
    (Class|BPILightFueledActivation|OnActivation(Message) (Variables|Default|GetControlledDoor))
    (else
      (Variables|/Game/MechanicsPlayground/MechanincsBlueprints/Buttons/Lab/BP_Lab.BP_Lab_C|SetActiveGroup _labref (- _position 1)))))

(event Custom|ButtonTrigger
  (params (TriggeredButton :type BP%20Button%20Teamworker%20Lab%20Base%20Object%20Reference))
  ;[1 1 1] Comment
)

(event EventBeginPlay
  ;[1 1 1] Comment
  (|CallParentFunction)
  (bind _returnvalue (Actor|GetActorOfClass "/Game/MechanicsPlayground/MechanincsBlueprints/Buttons/Lab/BP_Lab.BP_Lab_C"))
  (Variables|Default|SetLabRef _returnvalue))

(event Collision|EventActorBeginOverlap
  (params (OtherActor :type Actor%20Object%20Reference))
  (|CallParentFunction OtherActor) ; This node is disabled and will not be called.\nDrag off pins to build functionality.
)

(event EventTick
  (params (DeltaSeconds :type Float%20%28single-precision%29))
  (|CallParentFunction DeltaSeconds) ; This node is disabled and will not be called.\nDrag off pins to build functionality.
)

(event EventButtonTriggered
  (params (TriggeredButton :type BP%20Base%20Button%20Object%20Reference) (bIsTriggered :type Boolean))
  ;[1 1 1] Comment
  (bind _asbp_button_teamworker_lab_base (Utilities|Casting|CastToBP_Button_Teamworker_Lab_Base TriggeredButton))
  (CallFunction|ButtonTrigger _asbp_button_teamworker_lab_base))

(fn ConstructionScript
  (|CallParentFunction))