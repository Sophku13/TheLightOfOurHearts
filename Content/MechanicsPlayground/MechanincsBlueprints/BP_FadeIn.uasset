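; BP_FadeIn is an actor that fades its Cube mesh's material while a BP_BlowMechanic actor overlaps its Box trigger.
; BeginPlay creates a dynamic instance of M_Fade on the cube and initializes its Fade Amount parameter to 1.
; Entering the box plays the FadeInOut timeline, which drives Fade Amount, and leaving reverses it.
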(event OnComponentBeginOverlap(Box)
  (params (OverlappedComponent :type Primitive%20Component%20Object%20Reference) (OtherActor :type Actor%20Object%20Reference) (OtherComp :type Primitive%20Component%20Object%20Reference) (OtherBodyIndex :type Integer) (bFromSweep :type Boolean) (SweepResult :type Hit%20Result%20Structure%20%28by%20ref%29))
  (Utilities|Casting|CastToBP_BlowMechanic OtherActor)
  (bind _newtrack_0 (Timeline|FadeIn/Out Play)
    (:Update
      (Rendering|Material|SetScalarParameterValue (Variables|Default|GetDynamicMaterial) "Fade Amount" _newtrack_0 :!class /Script/Engine.MaterialInstanceDynamic))))

(event OnComponentEndOverlap(Box)
  (params (OverlappedComponent :type Primitive%20Component%20Object%20Reference) (OtherActor :type Actor%20Object%20Reference) (OtherComp :type Primitive%20Component%20Object%20Reference) (OtherBodyIndex :type Integer))
  (Utilities|Casting|CastToBP_BlowMechanic OtherActor)
  (bind _newtrack_0 (Timeline|FadeIn/Out Reverse)
    (:Update
      (Rendering|Material|SetScalarParameterValue (Variables|Default|GetDynamicMaterial) "Fade Amount" _newtrack_0 :!class /Script/Engine.MaterialInstanceDynamic))))

(event EventBeginPlay
  (bind _returnvalue (Rendering|Material|CreateDynamicMaterialInstance (Variables|Default|GetCube) 0 "/Game/MechanicsPlayground/MechanincsBlueprints/M_Fade.M_Fade" "None" :!class /Script/Engine.PrimitiveComponent))
  (bind _output_get (Variables|Default|SetDynamicMaterial _returnvalue))
  (Rendering|Material|SetScalarParameterValue _output_get "Fade Amount" 1.0 :!class /Script/Engine.MaterialInstanceDynamic))

(fn ConstructionScript)