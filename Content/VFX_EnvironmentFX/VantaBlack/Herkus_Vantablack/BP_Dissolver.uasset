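; BP_Dissolver is an actor that drives a dissolve volume for Vantablack VFX materials through the MPC_NewVanta Material Parameter Collection.
; Every Tick it writes the Sphere component's world location, scale and forward, right and up vectors into the collection as vector parameters.
; Materials reading the collection thus get an oriented, scaled volume that follows the actor at runtime; the same writes in the construction script are disconnected.
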(event EventBeginPlay)

(event Collision|EventActorBeginOverlap
  (params (OtherActor :type Actor%20Object%20Reference)))

(event EventTick
  (params (DeltaSeconds :type Float%20%28single-precision%29))
  (bind _sphere (Variables|Default|GetSphere))
  (bind _sphere_2 (Variables|Default|GetSphere))
  (Rendering|Material|SetVectorParameterValue "/Game/VFX_EnvironmentFX/VantaBlack/Herkus_Vantablack/MPC_NewVanta.MPC_NewVanta" "Location" (Math|Conversions|ToLinearColor(Vector) (Transformation|GetWorldLocation _sphere_2)) :!class /Script/Engine.KismetMaterialLibrary)
  (Rendering|Material|SetVectorParameterValue "/Game/VFX_EnvironmentFX/VantaBlack/Herkus_Vantablack/MPC_NewVanta.MPC_NewVanta" "Bounds" (Math|Conversions|ToLinearColor(Vector) (Transformation|GetWorldScale _sphere_2)) :!class /Script/Engine.KismetMaterialLibrary)
  (Rendering|Material|SetVectorParameterValue "/Game/VFX_EnvironmentFX/VantaBlack/Herkus_Vantablack/MPC_NewVanta.MPC_NewVanta" "X" (Math|Conversions|ToLinearColor(Vector) (Math|Vector|GetForwardVector _sphere)) :!class /Script/Engine.KismetMaterialLibrary)
  (Rendering|Material|SetVectorParameterValue "/Game/VFX_EnvironmentFX/VantaBlack/Herkus_Vantablack/MPC_NewVanta.MPC_NewVanta" "Y" (Math|Conversions|ToLinearColor(Vector) (Math|Vector|GetRightVector _sphere)) :!class /Script/Engine.KismetMaterialLibrary)
  (Rendering|Material|SetVectorParameterValue "/Game/VFX_EnvironmentFX/VantaBlack/Herkus_Vantablack/MPC_NewVanta.MPC_NewVanta" "Z" (Math|Conversions|ToLinearColor(Vector) (Math|Vector|GetUpVector _sphere)) :!class /Script/Engine.KismetMaterialLibrary))

(fn ConstructionScript)