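; Single interactable button that, going by its name, lowers a crane by sending an activation message to its referenced crane Blueprint.
; Interacting turns the button green, rotates its base, plays a lever sound and blocks re-presses for two seconds.
; Tick also applies the green material through a DoOnce while pressed.
; ProgressSaving restores the red, rotated-back look and resets that DoOnce unless RestoreProgress has set the saved flag.
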(event EventMoveButton
  (bind _button (Variables|Default|GetButton))
  ;[1 1 1] Comment
  (Rendering|Material|SetMaterial _button 0 "/Game/Materials/MI_Sphere_Emissive_Green.MI_Sphere_Emissive_Green")
  (Transformation|SetRelativeRotation (Variables|Default|GetButtonBase1) (Math|Rotator|MakeRotator 0.0 9e+01 0.0) false false)
  ;;[0 1 0.03888] Herkus was here
  (Audio|PlaySoundatLocation "/Game/Audio/Cues/lever6_by_mediatheksuche_Cue.lever6_by_mediatheksuche_Cue" (Variables|/Script/Engine.SceneComponent|GetRelativeLocation _button) "0, 0, 0" 1.0 1.0 0.0 0 0 0 0))

(event Collision|EventActorBeginOverlap
  (params (OtherActor :type Actor%20Object%20Reference))
  (|CallParentFunction OtherActor) ; This node is disabled and will not be called.\nDrag off pins to build functionality.
)

(event EventProgressSaving
  (if (not (Variables|Default|GetbIsSaved))
    (Rendering|Material|SetMaterial (Variables|Default|GetButton) 0 "/Game/Materials/MI_Sphere_Emissive_Red.MI_Sphere_Emissive_Red")
    (Transformation|SetRelativeRotation (Variables|Default|GetButtonBase1) (Math|Rotator|MakeRotator 0.0 -9e+01 0.0) false false)
    ;[0.1216 0.902 0.6627] Event Tick sets the material of the button only if the button is activatable in general and if the button is currently active or not
    (Utilities|FlowControl|DoOnce false) ; enters at Reset
  ))

(event EventRestoreProgress
  (Variables|Default|SetbIsSaved true))

(event EventTick
  (params (DeltaSeconds :type Float%20%28single-precision%29))
  ;[0.1216 0.902 0.6627] Event Tick sets the material of the button only if the button is activatable in general and if the button is currently active or not
  (if (Variables|Default|GetbIsButtonPressed)
    (Utilities|FlowControl|DoOnce false
      (:Completed
        (Rendering|Material|SetMaterial (Variables|Default|GetButton) 0 "/Game/Materials/MI_Sphere_Emissive_Green.MI_Sphere_Emissive_Green")))))

(event EventOnInteract
  ;[0.1216 0.902 0.6627] On Interacted it moves the button and calls the activation of the door. If it is an activatable button then the button has to be active for this to function
  (if (not (Variables|Default|GetbIsButtonPressed))
    (Variables|Default|SetbIsButtonPressed true)
    (CallFunction|MoveButton)
    (Class|BPILightFueledActivation|OnActivation(Message) (Variables|Default|GetCraneBPRef))
    (Utilities|FlowControl|Delay 2.0)
    (Variables|Default|SetbIsButtonPressed false)))

(event EventBeginPlay
  (|CallParentFunction) ; This node is disabled and will not be called.\nDrag off pins to build functionality.
)

(fn ConstructionScript
  (|CallParentFunction))

(fn IsInteractable
  (return true))