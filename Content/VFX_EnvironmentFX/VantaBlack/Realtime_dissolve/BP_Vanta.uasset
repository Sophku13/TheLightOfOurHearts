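; Vanta darkness hazard that periodically drains the player's HP on overlap, unless invincible, and can be dissolved by blowing light.
; Holding IA_BlowLight near and facing it plays a timeline driving a dynamic dissolve material, then destroys the player's HITVANTA target.
; Cancelling reverses the dissolve and removes energy sources.
; Destruction only hides it and disables collision, so RestoreProgress can respawn it unless progress was saved.
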(event Custom|SpawnVanta
  ;[1 1 1] Comment
  (Collision|SetCollisionEnabled (Variables|Default|GetCollisionBox) "QueryOnly")
  (Collision|SetCollisionEnabled (Variables|Default|GetCube) "QueryOnly")
  (Development|SetHiddeninGame (Variables|Default|GetCube) false false)
  (Rendering|Material|SetScalarParameterValue (Variables|Default|Getdy1) "Scale" 0.0 :!class /Script/Engine.MaterialInstanceDynamic)
  ;[0.9155 1 0.609] spread the scale (reverse if not finish)
  ;;[0 0 0] dynamic material
  (bind (_direction _scale) (Timeline|Timeline SetNewTime)
    (:Update
      (Rendering|Material|SetScalarParameterValue (Variables|Default|Getdy1) "Scale" _scale :!class /Script/Engine.MaterialInstanceDynamic))
    (:Finished
      ;;;[0 0 0] REVERSE FINISHED IS ALSO FINISHED!
      (if (Utilities|Enum|Equal(Enum) "Forward" _direction)
        ;;[0 0 0] DESTROY HIT_VANTA ONE BY ONE
        ;;;[0.09063 1 0.04957] placeholder SFX
        (Audio|PlaySound2D "/Game/crystal_dissolve1_Cue.crystal_dissolve1_Cue" 1.0 1.0 0.0 0 0)
        (bind _thirdpersoncharacter (Variables|Default|GetThirdPersonCharacter)
          (:then
            (bind _hit_vanta (Variables|/Game/ThirdPerson/Blueprints/BP_ThirdPersonCharacter.BP_ThirdPersonCharacter_C|GetHIT_VANTA _thirdpersoncharacter)
              (:then
                (Development|PrintString "IS VANTA VALID" false)
                (CallFunction|DestroyVanta _hit_vanta))
              (:else)))
          (:else))))))

(event Custom|DestroyVanta
  ;[1 1 1] Comment
  (Collision|SetCollisionEnabled (Variables|Default|GetCollisionBox) "NoCollision")
  (Collision|SetCollisionEnabled (Variables|Default|GetCube) "NoCollision")
  (Development|SetHiddeninGame (Variables|Default|GetCube) true false))

(event Input|EnhancedActionEvents|EnhancedInputActionIA_BlowLight
  (params (ActionValue :type Boolean) (ElapsedSeconds :type Float%20%28double-precision%29) (TriggeredSeconds :type Float%20%28double-precision%29) (InputAction :type Input%20Action%20Object%20Reference :default "/Game/MechanicsPlayground/MechanincsBlueprints/InputActions/IA_BlowLight.IA_BlowLight"))
  ;[0.9155 1 0.609] spread the scale (reverse if not finish)
  (:Ongoing
    ;;[0 0 0] can be destroyed?
    (bind _thirdpersoncharacter (Variables|Default|GetThirdPersonCharacter)
      (:then
        (if (Variables|/Game/ThirdPerson/Blueprints/BP_ThirdPersonCharacter.BP_ThirdPersonCharacter_C|GetIs%20near%20and%20faceing%20vanta? _thirdpersoncharacter)
          (Development|PrintString "Blowing" false)
          ;;[0 0 0] dynamic material
          (bind (_direction _scale) (Timeline|Timeline Play)
            (:Update
              (Rendering|Material|SetScalarParameterValue (Variables|Default|Getdy1) "Scale" _scale :!class /Script/Engine.MaterialInstanceDynamic))
            (:Finished
              ;;;[0 0 0] REVERSE FINISHED IS ALSO FINISHED!
              (if (Utilities|Enum|Equal(Enum) "Forward" _direction)
                ;;[0 0 0] DESTROY HIT_VANTA ONE BY ONE
                ;;;[0.09063 1 0.04957] placeholder SFX
                (Audio|PlaySound2D "/Game/crystal_dissolve1_Cue.crystal_dissolve1_Cue" 1.0 1.0 0.0 0 0)
                (bind _thirdpersoncharacter_2 (Variables|Default|GetThirdPersonCharacter)
                  (:then
                    (bind _hit_vanta (Variables|/Game/ThirdPerson/Blueprints/BP_ThirdPersonCharacter.BP_ThirdPersonCharacter_C|GetHIT_VANTA _thirdpersoncharacter_2)
                      (:then
                        (Development|PrintString "IS VANTA VALID" false)
                        (CallFunction|DestroyVanta _hit_vanta))
                      (:else)))
                  (:else)))))))
      (:else)))
  (:Canceled
    ;;[0 0 0] destroy energy source
    (bind _outactors (Actor|GetAllActorsOfClass "/Game/VFX_EnvironmentFX/VantaBlack/Realtime_dissolve/BP_EnergySource.BP_EnergySource_C"))
    (Actor|DestroyActor _outactors)
    (Development|PrintString "remove energy source" false)
    (Timeline|Timeline Reverse))
  (:Completed
    ;;[0 0 0] TO BE SAFE... (SEEMS USELESS CANCEL AND COMPLETE CAN CONNECT SAME THING AFTERWARDS)
    (bind _outactors_2 (Actor|GetAllActorsOfClass "/Game/VFX_EnvironmentFX/VantaBlack/Realtime_dissolve/BP_EnergySource.BP_EnergySource_C"))
    (Actor|DestroyActor _outactors_2)
    (Development|PrintString "remove energy source" false)
    (Timeline|Timeline SetNewTime)))

(event EventTick
  (params (DeltaSeconds :type Float%20%28single-precision%29))
  (bind _thirdpersoncharacter (Variables|Default|GetThirdPersonCharacter))
  ;[0.3024 0.6256 0.5622] Death when overlap (decays the light gradualy and doesnt kill it right away)
  (if (Variables|Default|GetPlayerHitByVanta)
    ;;[0.8396 1 0.4766] is eatlight?
    (bind _thirdpersoncharacter_2 (Variables|Default|GetThirdPersonCharacter)
      (:then
        (if (Variables|/Game/ThirdPerson/Blueprints/BP_ThirdPersonCharacter.BP_ThirdPersonCharacter_C|Getinvincible？ _thirdpersoncharacter_2)
          (Collision|SetCollisionEnabled (Variables|Default|GetCollisionBox) "NoCollision")
          (else
            (Development|PrintString "not invincible" false)
            (bind _result (Math|Integer|IncrementInt (Variables|Default|GetDecayCount))
              (:%20%20
                (if (== (Variables|Default|GetRange) _result)
                  (Variables|Default|SetDecayCount 0)
                  (Default|ReduceHP _thirdpersoncharacter (Math|Conversions|ToFloat(Integer) (Variables|Default|GetDamage)) (Variables|/Game/MechanicsPlayground/MechanincsBlueprints/BP_LightOrb.BP_LightOrb_C|GetbIsHeld (Variables|/Game/ThirdPerson/Blueprints/BP_ThirdPersonCharacter.BP_ThirdPersonCharacter_C|GetBP_LightOrbRef _thirdpersoncharacter)) self true)))))))
      (:else))))

(event EventBeginPlay
  ;[0.9423 1 0.4501] setting
  ;;[0 0 0] !!!without this F key not working in vanta black BP-only overlap can trigger changes, input needs to be activated in this BP
  (Input|EnableInput (Game|GetPlayerController 0))
  (bind _returnvalue (Actor|GetActorOfClass "/Game/ThirdPerson/Blueprints/BP_ThirdPersonCharacter.BP_ThirdPersonCharacter_C"))
  (Variables|Default|SetThirdPersonCharacter _returnvalue)
  (bind _returnvalue_2 (Rendering|Material|CreateDynamicMaterialInstance (Variables|Default|GetCube) 0 "/Game/VFX_EnvironmentFX/VantaBlack/Realtime_dissolve/M_dissolve_box.M_dissolve_box" "None" :!class /Script/Engine.PrimitiveComponent))
  (Variables|Default|Setdy1 _returnvalue_2))

(event EventInfluenceLightOrb
  (params (LightOrbRef :type BP%20Light%20Orb%20Object%20Reference) (IsActive :type Boolean))
  ;[0.3017 1 0.8766] Comment
  (Variables|Default|SetThirdPersonCharacter (Variables|/Game/MechanicsPlayground/MechanincsBlueprints/BP_LightOrb.BP_LightOrb_C|GetPlayerRef LightOrbRef))
  (Variables|Default|SetVantaIsInluencingLight IsActive)
  (Default|LightPulsing LightOrbRef))

(event EventInfluencingPlayer
  (params (PlayerRef :type BP%20Third%20Person%20Character%20Object%20Reference) (bIsInRange :type Boolean))
  ;[1 1 1] Comment
  (Variables|Default|SetThirdPersonCharacter PlayerRef)
  (Variables|Default|SetPlayerHitByVanta bIsInRange))

(event EventPlayerDeath
  (params (DyingPlayerReference :type BP%20Third%20Person%20Character%20Object%20Reference))
  ;[1 1 1] Comment
  (Variables|Default|SetThirdPersonCharacter DyingPlayerReference)
  (Default|VantaDeath (Variables|/Game/ThirdPerson/Blueprints/BP_ThirdPersonCharacter.BP_ThirdPersonCharacter_C|GetDeathManagerRef DyingPlayerReference) DyingPlayerReference))

(event EventRestoreProgress
  ;[1 1 1] Comment
  (if (not (Variables|Default|GetbIsSaved))
    (CallFunction|SpawnVanta)))

(event EventProgressSaving
  ;[1 1 1] Comment
  (Variables|Default|SetbIsSaved true))

(fn ConstructionScript)

(fn IsInfluencingthePlayer
  (params (PlayerRef :type BP%20Third%20Person%20Character%20Object%20Reference))
  (return true))