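; A placeable level camera that takes over the player's view from the follow camera through trigger boxes, or at BeginPlay as the default.
; Overlaps blend to it or restore the character's default camera, and it registers itself with the character.
; While active, Tick optionally eases rotation toward the player, flipping the yaw offset by facing, and narrows FOV with distance.
; A Forward component, re-oriented by another trigger, can supply the forward rotation.
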(event OnComponentBeginOverlap(EnableCamera)
  (params (OverlappedComponent :type Primitive%20Component%20Object%20Reference) (OtherActor :type Actor%20Object%20Reference) (OtherComp :type Primitive%20Component%20Object%20Reference) (OtherBodyIndex :type Integer) (bFromSweep :type Boolean) (SweepResult :type Hit%20Result%20Structure%20%28by%20ref%29))
  ;[1 1 1] Enabling This Camera When Player overlapsy the Trigger box
  (bind _yes (Class|BPIPlayer|IsPlayer(Message) OtherActor))
  (if _yes
    (Game|Player|SetViewTargetwithBlend (Game|GetPlayerController 0) self (Variables|Default|GetCameraBlendTime) "VTBlend_Linear" 0.0 false)
    (Class|BPIPlayer|UpdateCameraComponent(Message) (Game|GetPlayerCharacter 0) self)))

(event OnComponentEndOverlap(EnableCamera)
  (params (OverlappedComponent :type Primitive%20Component%20Object%20Reference) (OtherActor :type Actor%20Object%20Reference) (OtherComp :type Primitive%20Component%20Object%20Reference) (OtherBodyIndex :type Integer))
  ;[1 1 1] Comment
  (if (not (Variables|Default|GetDon'tDisable))
    (bind _yes (Class|BPIPlayer|IsPlayer(Message) OtherActor))
    (if _yes
      (Class|BPIPlayer|EnableDefaultCharacterCamera(Message) OtherActor))))

(event OnComponentBeginOverlap(SwitchForwardVectoBox)
  (params (OverlappedComponent :type Primitive%20Component%20Object%20Reference) (OtherActor :type Actor%20Object%20Reference) (OtherComp :type Primitive%20Component%20Object%20Reference) (OtherBodyIndex :type Integer) (bFromSweep :type Boolean) (SweepResult :type Hit%20Result%20Structure%20%28by%20ref%29))
  (bind _yes (Class|BPIPlayer|IsPlayer(Message) OtherActor))
  (if _yes
    (Transformation|SetRelativeRotation (Variables|Default|GetForward) (Variables|Default|GetSetNewForwardRotation) false false)))

(event OnComponentBeginOverlap(BackToFollowCamera)
  (params (OverlappedComponent :type Primitive%20Component%20Object%20Reference) (OtherActor :type Actor%20Object%20Reference) (OtherComp :type Primitive%20Component%20Object%20Reference) (OtherBodyIndex :type Integer) (bFromSweep :type Boolean) (SweepResult :type Hit%20Result%20Structure%20%28by%20ref%29))
  ;[1 1 1] Creating a Trigerbox to Get back to default Camera
  (if (Variables|Default|GetActiveCamera)
    (bind _yes (Class|BPIPlayer|IsPlayer(Message) OtherActor))
    (if _yes
      (Class|BPIPlayer|EnableDefaultCharacterCamera(Message) OtherActor))))

(event OnComponentEndOverlap(SwitchForwardVectoBox)
  (params (OverlappedComponent :type Primitive%20Component%20Object%20Reference) (OtherActor :type Actor%20Object%20Reference) (OtherComp :type Primitive%20Component%20Object%20Reference) (OtherBodyIndex :type Integer))
  (bind _yes (Class|BPIPlayer|IsPlayer(Message) OtherActor))
  (if _yes
    (Transformation|SetRelativeRotation (Variables|Default|GetForward) (Variables|Default|GetOriginalForwardRotation) false false)))

(event EventBeginPlay
  ;[1 1 1] Making it possible to Set this Cameras as Default Cameras
  (Variables|Default|SetOriginalFieldOfView (Variables|/Script/Engine.CameraComponent|GetFieldOfView (Variables|Default|GetCamera)))
  (if (Variables|Default|GetDefaultCamera)
    (Game|Player|SetViewTargetwithBlend (Game|GetPlayerController 0) self 0.0 "VTBlend_Linear" 0.0 false)
    (Class|BPIPlayer|UpdateCameraComponent(Message) (Game|GetPlayerCharacter 0) self)))

(event EventTick
  (params (DeltaSeconds :type Float%20%28single-precision%29))
  (bind _returnvalue (Utilities|Time|GetWorldDeltaSeconds))
  (bind _returnvalue_2 (Game|GetPlayerCharacter 0))
  (bind _camera (Variables|Default|GetCamera))
  (bind _addrotationtocamera (Variables|Default|GetAddRotationToCamera))
  (bind _camera_2 (Variables|Default|GetCamera))
  (bind _returnvalue_3 (Transformation|GetWorldRotation _camera_2))
  (bind _returnvalue_4 (Transformation|GetActorLocation _returnvalue_2))
  (bind _returnvalue_5 (Transformation|GetWorldLocation _camera))
  (bind _returnvalue_6 (Math|Rotator|FindLookatRotation _returnvalue_5 _returnvalue_4))
  ;[1 1 1] Make the Camera Focus on the Character
  (if (and (Variables|Default|GetActiveCamera) (Variables|Default|GetFocusOnPlayer))
    (if (> (.x (Transformation|GetActorForwardVector (Game|GetPlayerCharacter 0))) (.x (Math|Vector|GetForwardVector (Variables|Default|GetForward))))
      (Transformation|SetWorldRotation _camera_2 (Math|Interpolation|RInterpTo _returnvalue_3 (Math|Rotator|CombineRotators _returnvalue_6 (Variables|Default|GetAddRotationToCamera)) _returnvalue 1.5) false false)
      (else
        (Transformation|SetWorldRotation _camera_2 (Math|Interpolation|RInterpTo _returnvalue_3 (Math|Rotator|CombineRotators _returnvalue_6 (Math|Rotator|MakeRotator (.roll _addrotationtocamera) (.pitch _addrotationtocamera) (* (.yaw _addrotationtocamera) -1.0))) _returnvalue 1.5) false false)))
    ;[1 1 1] Camera Zooms in when character is getting further
    (if (Variables|Default|GetZoomInOn)
      (Camera|SetFieldOfView (Variables|Default|GetCamera) (Math|Float|MapRangeClamped (Math|Vector|Distance(Vector) (Transformation|GetWorldLocation (Variables|Default|GetCamera)) (Transformation|GetWorldLocation (Variables|/Script/Engine.Character|GetCapsuleComponent (Game|GetPlayerCharacter 0)))) 0.0 5e+03 1e+02 1e+01)))))

(event EventOnBecomeViewTarget
  (params (PC :type Player%20Controller%20Object%20Reference))
  ;[1 1 1] Setting This Camera as ActiveCamera when Triggered
  (Variables|Default|SetActiveCamera true)
  ;[1 1 1] Saving the active camera to adjust it outside of the code.
  (Utilities|FlowControl|DoOnce false
    (:Completed
      (bind _asbp_third_person_character (Utilities|Casting|CastToBP_ThirdPersonCharacter (Game|GetPlayerCharacter 0)))
      (Variables|/Game/ThirdPerson/Blueprints/BP_ThirdPersonCharacter.BP_ThirdPersonCharacter_C|SetActive%20Camera _asbp_third_person_character self)
      (Variables|Default|SetZoomInOn (Variables|Default|GetZoomInOn)))))

(event EventOnEndViewTarget
  (params (PC :type Player%20Controller%20Object%20Reference))
  ;[1 1 1] Setting This Camera as ActiveCamera when Triggered
  (Variables|Default|SetActiveCamera false)
  ;[1 1 1] Saving the active camera to adjust it outside of the code.
  (Utilities|FlowControl|DoOnce false) ; enters at Reset
)

(fn ConstructionScript)

(fn CallBlowingCameraAnimation
  (return (Variables|Default|GetCamera)))

(fn GeForwardtotation
  (if (Variables|Default|GetUsePrePlannedMovement)
    (return (Transformation|GetWorldRotation (Variables|Default|GetForward)))
    (else
      (return (Transformation|GetWorldRotation (Variables|Default|GetCamera))))))