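; Bunker puzzle button that must be activated in sequence with the other buttons in its group, according to its PuzzlePosition.
; ButtonTask records progress in the ActivationArray map on BP_ButtonGrouper_Bunker.
; Position 1 restarts the sequence; later positions activate only if every earlier one is set, otherwise they clear the whole map.
; CorrectOrder is set back to true only in the position 1 branch.
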(event EventBeginPlay
  (|CallParentFunction) ; This node is disabled and will not be called.\nDrag off pins to build functionality.
)

(event Collision|EventActorBeginOverlap
  (params (OtherActor :type Actor%20Object%20Reference))
  (|CallParentFunction OtherActor) ; This node is disabled and will not be called.\nDrag off pins to build functionality.
)

(event EventTick
  (params (DeltaSeconds :type Float%20%28single-precision%29))
  (|CallParentFunction DeltaSeconds) ; This node is disabled and will not be called.\nDrag off pins to build functionality.
)

(event EventButtonTask
  (params (ButtonGroup :type BP%20Button%20Grouper%20Base%20Object%20Reference))
  (bind _puzzleposition (Variables|Default|GetPuzzlePosition))
  (bind _returnvalue (- _puzzleposition 2))
  (bind _asbp_button_grouper_bunker (Utilities|Casting|CastToBP_ButtonGrouper_Bunker ButtonGroup))
  (if (not (== _puzzleposition 1))
    (for _index (range 0 _returnvalue)
      (if (not (.Value (Utilities|Map|Find (Variables|/Game/MechanicsPlayground/MechanincsBlueprints/Buttons/Bunker/BP_ButtonGrouper_Bunker.BP_ButtonGrouper_Bunker_C|GetactivationArray _asbp_button_grouper_bunker) _index)))
        (Variables|Default|SetbCorrectOrder false)))
    (if (Variables|Default|GetbCorrectOrder)
      (Utilities|Map|Add (Variables|/Game/MechanicsPlayground/MechanincsBlueprints/Buttons/Bunker/BP_ButtonGrouper_Bunker.BP_ButtonGrouper_Bunker_C|GetactivationArray _asbp_button_grouper_bunker) (+ _returnvalue 1) true)
      (else
        (for _index_2 (range 0 (- (Utilities|Map|Length (Variables|/Game/MechanicsPlayground/MechanincsBlueprints/Buttons/Bunker/BP_ButtonGrouper_Bunker.BP_ButtonGrouper_Bunker_C|GetactivationArray _asbp_button_grouper_bunker)) 1))
          (Utilities|Map|Add (Variables|/Game/MechanicsPlayground/MechanincsBlueprints/Buttons/Bunker/BP_ButtonGrouper_Bunker.BP_ButtonGrouper_Bunker_C|GetactivationArray _asbp_button_grouper_bunker) _index_2 false))))
    (else
      (for _index_3 (range 0 (- (Utilities|Map|Length (Variables|/Game/MechanicsPlayground/MechanincsBlueprints/Buttons/Bunker/BP_ButtonGrouper_Bunker.BP_ButtonGrouper_Bunker_C|GetactivationArray _asbp_button_grouper_bunker)) 1))
        (Utilities|Map|Add (Variables|/Game/MechanicsPlayground/MechanincsBlueprints/Buttons/Bunker/BP_ButtonGrouper_Bunker.BP_ButtonGrouper_Bunker_C|GetactivationArray _asbp_button_grouper_bunker) _index_3 false))
      (Utilities|Map|Add (Variables|/Game/MechanicsPlayground/MechanincsBlueprints/Buttons/Bunker/BP_ButtonGrouper_Bunker.BP_ButtonGrouper_Bunker_C|GetactivationArray _asbp_button_grouper_bunker) 0 true)
      (Variables|Default|SetbCorrectOrder true))))

(fn ConstructionScript
  (|CallParentFunction))