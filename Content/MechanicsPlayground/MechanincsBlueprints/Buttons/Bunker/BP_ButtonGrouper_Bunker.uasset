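; Bunker button grouper actor that manages the buttons in ButtonList and activates them when the player enters its Room volume.
; On BeginPlay it deactivates each button, looked up by index in a map, and binds an event to its trigger.
; A third-person character overlapping Room is passed to every button as PlayerRef, and each button becomes active.
; Nothing deactivates them on exit, and the ButtonTriggered handler is empty.
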(event OnComponentBeginOverlap(Room)
  (params (OverlappedComponent :type Primitive%20Component%20Object%20Reference) (OtherActor :type Actor%20Object%20Reference) (OtherComp :type Primitive%20Component%20Object%20Reference) (OtherBodyIndex :type Integer) (bFromSweep :type Boolean) (SweepResult :type Hit%20Result%20Structure%20%28by%20ref%29))
  (bind _asbp_third_person_character (Utilities|Casting|CastToBP_ThirdPersonCharacter OtherActor))
  (for _index (range 0 (- (Utilities|Map|Length (Variables|Default|GetButtonList)) 1))
    (if (.ReturnValue (Utilities|Map|Find (Variables|Default|GetButtonList) _index))
      (Variables|/Game/MechanicsPlayground/MechanincsBlueprints/Buttons/Bases/BP_BaseButton.BP_BaseButton_C|SetPlayerRef (.Value (Utilities|Map|Find (Variables|Default|GetButtonList) _index)) _asbp_third_person_character)
      (Variables|/Game/MechanicsPlayground/MechanincsBlueprints/Buttons/Bases/BP_Button_Teamworker_Base.BP_Button_Teamworker_Base_C|SetbIsActive (.Value (Utilities|Map|Find (Variables|Default|GetButtonList) _index)) true))))

(event Custom|ButtonTriggered
  (params (TriggeredButton :type BP%20Base%20Button%20Object%20Reference) (bIsTriggered :type Boolean)))

(event EventBeginPlay
  (for _index (range 0 (- (Utilities|Map|Length (Variables|Default|GetButtonList)) 1))
    (if (.ReturnValue (Utilities|Map|Find (Variables|Default|GetButtonList) _index))
      (Variables|/Game/MechanicsPlayground/MechanincsBlueprints/Buttons/Bases/BP_Button_Teamworker_Base.BP_Button_Teamworker_Base_C|SetbIsActive (.Value (Utilities|Map|Find (Variables|Default|GetButtonList) _index)) false)
      (EventDispatchers|BindEventtoButtonTriggered (.Value (Utilities|Map|Find (Variables|Default|GetButtonList) _index)) (EventDispatchers|CreateEvent :!event Custom|ButtonTriggered)))))

(event Collision|EventActorBeginOverlap
  (params (OtherActor :type Actor%20Object%20Reference)))

(event EventTick
  (params (DeltaSeconds :type Float%20%28single-precision%29)))

(fn ConstructionScript)