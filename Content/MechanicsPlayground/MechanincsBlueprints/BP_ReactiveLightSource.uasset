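; BP_ReactiveLightSource is a light actor that appears and lights up when a BP_LightOrb begins overlapping its LightReceptor, then switches itself off.
; The overlap unhides the actor and its PointLight and enables Tick.
; Tick uses IsActive as a one-tick delay: it sets the flag when false, and when true clears it, hides both and disables ticking.
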(event OnComponentBeginOverlap(LightReceptor)
  (params (OverlappedComponent :type Primitive%20Component%20Object%20Reference) (OtherActor :type Actor%20Object%20Reference) (OtherComp :type Primitive%20Component%20Object%20Reference) (OtherBodyIndex :type Integer) (bFromSweep :type Boolean) (SweepResult :type Hit%20Result%20Structure%20%28by%20ref%29))
  (Utilities|Casting|CastToBP_LightOrb OtherActor)
  (Rendering|SetActorHiddenInGame false)
  (Development|SetHiddeninGame (Variables|Default|GetPointLight) false false)
  (Actor|Tick|SetActorTickEnabled true))

(event EventTick
  (params (DeltaSeconds :type Float%20%28single-precision%29))
  (if (Variables|Default|GetbIsActive)
    (Variables|Default|SetbIsActive false)
    (Rendering|SetActorHiddenInGame true)
    (Development|SetHiddeninGame (Variables|Default|GetPointLight) true false)
    (Actor|Tick|SetActorTickEnabled false)
    (else
      (Variables|Default|SetbIsActive true))))

(fn ConstructionScript)