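; BP_Hints is a hint sprite actor whose plane becomes more visible as a BP_LightOrb gets closer to it.
; When the orb begins overlapping the plane, it stores the orb and starts a fast looping timer instead of using Tick.
; Each timer call maps orb distance to the material's Opacity parameter, fading to zero at DistanceOfDissapear.
; Any end overlap on the plane pauses the timer, without checking which actor left.
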(event OnComponentBeginOverlap(Plane)
  (params (OverlappedComponent :type Primitive%20Component%20Object%20Reference) (OtherActor :type Actor%20Object%20Reference) (OtherComp :type Primitive%20Component%20Object%20Reference) (OtherBodyIndex :type Integer) (bFromSweep :type Boolean) (SweepResult :type Hit%20Result%20Structure%20%28by%20ref%29))
  (bind _asbp_light_orb (Utilities|Casting|CastToBP_LightOrb OtherActor))
  (Variables|Default|SetLightOrbRef! _asbp_light_orb)
  (bind _returnvalue (Utilities|Time|SetTimerbyEvent (delegate Custom|UpdateOpacity) 0.01 true))
  (Variables|Default|SetTimer _returnvalue))

(event OnComponentEndOverlap(Plane)
  (params (OverlappedComponent :type Primitive%20Component%20Object%20Reference) (OtherActor :type Actor%20Object%20Reference) (OtherComp :type Primitive%20Component%20Object%20Reference) (OtherBodyIndex :type Integer))
  (Utilities|Time|PauseTimerbyHandle (Variables|Default|GetTimer)))

(event Custom|UpdateOpacity
  (Rendering|Material|SetScalarParameterValueonMaterials (Variables|Default|GetPlane) "Opacity" (Math|Float|MapRangeClamped (Math|Vector|Distance(Vector) (Transformation|GetActorLocation (Variables|Default|GetLightOrbRef!)) (Transformation|GetActorLocation)) 0.0 (Variables|Default|GetDistanceOfDissapear) 1.0 0.0)))

(event Collision|EventActorBeginOverlap
  (params (OtherActor :type Actor%20Object%20Reference)))

(event EventTick
  (params (DeltaSeconds :type Float%20%28single-precision%29)))

(event EventBeginPlay
  (Variables|Default|SetDistanceOfDissapear (Variables|Default|GetDistanceOfDissapear)))

(fn ConstructionScript)