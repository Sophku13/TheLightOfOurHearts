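; Socket actor where the player's light orb can be placed, tracking how long the orb stays in it.
; Box overlap registers it as the character's nearest socket and enables Tick; orb overlap toggles a Niagara highlight.
; While occupied, Tick increments a counter and a timeline spins and bobs the orb.
; When empty, the counter drains per tick, and Tick can disable itself once it reaches zero.
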(event OnComponentBeginOverlap(Box)
  (params (OverlappedComponent :type Primitive%20Component%20Object%20Reference) (OtherActor :type Actor%20Object%20Reference) (OtherComp :type Primitive%20Component%20Object%20Reference) (OtherBodyIndex :type Integer) (bFromSweep :type Boolean) (SweepResult :type Hit%20Result%20Structure%20%28by%20ref%29))
  ;[0.1216 0.902 0.6627] Updates the Player Reference when a Character is entering the range and get a reference to Light.
  (bind _asbp_third_person_character (Utilities|Casting|CastToBP_ThirdPersonCharacter OtherActor))
  (bind _output_get (Variables|Default|SetPlayerRef _asbp_third_person_character))
  (Variables|Default|SetLightOrbRef (Variables|/Game/ThirdPerson/Blueprints/BP_ThirdPersonCharacter.BP_ThirdPersonCharacter_C|GetBP_LightOrbRef _output_get))
  (Variables|/Game/ThirdPerson/Blueprints/BP_ThirdPersonCharacter.BP_ThirdPersonCharacter_C|SetbNearSocket (Variables|Default|GetPlayerRef) true)
  ;;[0.1216 0.902 0.6627] Saves itself as the nearest Light Socket in the ThirdPersonCharacter and starts ticking
  (Variables|/Game/ThirdPerson/Blueprints/BP_ThirdPersonCharacter.BP_ThirdPersonCharacter_C|SetNearestLightSocketRef (Variables|Default|GetPlayerRef) self)
  (Actor|Tick|SetActorTickEnabled true))

(event OnComponentEndOverlap(Box)
  (params (OverlappedComponent :type Primitive%20Component%20Object%20Reference) (OtherActor :type Actor%20Object%20Reference) (OtherComp :type Primitive%20Component%20Object%20Reference) (OtherBodyIndex :type Integer))
  ;[0.1216 0.902 0.6627] Fires when the Character leaves the location of the socket
  (bind _asbp_third_person_character (Utilities|Casting|CastToBP_ThirdPersonCharacter OtherActor))
  (bind _output_get (Variables|Default|SetPlayerRef _asbp_third_person_character))
  (Variables|/Game/ThirdPerson/Blueprints/BP_ThirdPersonCharacter.BP_ThirdPersonCharacter_C|SetbNearSocket _output_get false))

(event OnComponentBeginOverlap(NS_LightHighlight)
  (params (OverlappedComponent :type Primitive%20Component%20Object%20Reference) (OtherActor :type Actor%20Object%20Reference) (OtherComp :type Primitive%20Component%20Object%20Reference) (OtherBodyIndex :type Integer) (bFromSweep :type Boolean) (SweepResult :type Hit%20Result%20Structure%20%28by%20ref%29))
  (Utilities|Casting|CastToBP_LightOrb OtherActor)
  (Development|SetHiddeninGame (Variables|Default|GetNS_LightHighlight) false false))

(event OnComponentEndOverlap(NS_LightHighlight)
  (params (OverlappedComponent :type Primitive%20Component%20Object%20Reference) (OtherActor :type Actor%20Object%20Reference) (OtherComp :type Primitive%20Component%20Object%20Reference) (OtherBodyIndex :type Integer))
  (Utilities|Casting|CastToBP_LightOrb OtherActor)
  (Development|SetHiddeninGame (Variables|Default|GetNS_LightHighlight) true false))

(event Custom|Reset
  (Variables|Default|SetbLightOnSocket false)
  (Variables|Default|SetTimeOfLightInSocket 0)
  (Variables|Default|SetTimeSave 0.0)
  (Variables|Default|SetbMoveUp true)
  (bind _asbp_third_person_character (Utilities|Casting|CastToBP_ThirdPersonCharacter (Game|GetPlayerCharacter 0)))
  (bind _output_get (Variables|Default|SetPlayerRef _asbp_third_person_character))
  (Variables|Default|SetLightOrbRef (Variables|/Game/ThirdPerson/Blueprints/BP_ThirdPersonCharacter.BP_ThirdPersonCharacter_C|GetBP_LightOrbRef _output_get)))

(event EventBeginPlay
  ;[0.1216 0.902 0.6627] Initializing the socket and saving its location in the world and saving references for self and the player character
  (Variables|Default|SetLocationOfSocket (Transformation|GetWorldLocation (Variables|Default|GetOrbSocket)))
  (Variables|Default|SetSelfReference self)
  (bind _asbp_third_person_character (Utilities|Casting|CastToBP_ThirdPersonCharacter (Game|GetPlayerCharacter 0)))
  (bind _output_get (Variables|Default|SetPlayerRef _asbp_third_person_character))
  (Variables|Default|SetLightOrbRef (Variables|/Game/ThirdPerson/Blueprints/BP_ThirdPersonCharacter.BP_ThirdPersonCharacter_C|GetBP_LightOrbRef _output_get)))

(event EventInfluenceLightOrb
  (params (LightOrbRef :type BP%20Light%20Orb%20Object%20Reference) (IsActive :type Boolean))
  ;[0.1216 0.902 0.6627] Making the Light React
  (Default|LightPulsing LightOrbRef))

(event EventTick
  (params (DeltaSeconds :type Float%20%28single-precision%29))
  (bind _lightorbref (Variables|Default|GetLightOrbRef))
  ;[0.1216 0.902 0.6627] Event Tick
  ;;[0.1216 0.902 0.6627] Checks if the light is on the socket or not
  (if (Variables|Default|GetbLightOnSocket)
    ;;[0.1216 0.902 0.6627] Counts the seconds that the Light has been on the socket
    (Variables|Default|SetTimeOfLightInSocket (+ (Variables|Default|GetTimeOfLightInSocket) 1))
    (bind _lightorbref_2 (Variables|Default|GetLightOrbRef)
      (:then
        (bind _newtrack_0 (Timeline|RotateTheLight PlayFromStart)
          (:Update
            (Transformation|SetActorRotation _lightorbref_2 (Math|Rotator|MakeRotator (.roll (.rotation (Transformation|GetActorTransform _lightorbref_2))) (.pitch (.rotation (Transformation|GetActorTransform _lightorbref_2))) (Math|Float|Lerp (.yaw (.rotation (Transformation|GetActorTransform _lightorbref_2))) (+ (.yaw (.rotation (Transformation|GetActorTransform _lightorbref_2))) 1e+01) _newtrack_0)))
            (if (Variables|Default|GetbMoveUp)
              (Transformation|SetActorLocation _lightorbref (Math|Vector|MakeVector (.X (Math|Vector|BreakVector (.location (Transformation|GetActorTransform _lightorbref_2)))) (.Y (Math|Vector|BreakVector (.location (Transformation|GetActorTransform _lightorbref_2)))) (Math|Float|Lerp (.Z (Math|Vector|BreakVector (.location (Transformation|GetActorTransform _lightorbref_2)))) (+ (.Z (Math|Vector|BreakVector (.location (Transformation|GetActorTransform _lightorbref_2)))) 0.5) _newtrack_0)) false false)
              (else
                (Transformation|SetActorLocation _lightorbref (Math|Vector|MakeVector (.X (Math|Vector|BreakVector (.location (Transformation|GetActorTransform _lightorbref_2)))) (.Y (Math|Vector|BreakVector (.location (Transformation|GetActorTransform _lightorbref_2)))) (Math|Float|Lerp (.Z (Math|Vector|BreakVector (.location (Transformation|GetActorTransform _lightorbref_2)))) (- (.Z (Math|Vector|BreakVector (.location (Transformation|GetActorTransform _lightorbref_2)))) 0.5) _newtrack_0)) false false))))
          (:Finished
            (if (Variables|Default|GetbMoveUp)
              (Variables|Default|SetbMoveUp false)
              (else
                (Variables|Default|SetbMoveUp true))))))
      (:else))
    (else
      (Variables|Default|SetbMoveUp true)
      ;;[0.1216 0.902 0.6627] Reducing the time the Light has spent in the socket over time
      (if (>= (Variables|Default|GetTimeOfLightInSocket) 1)
        (Variables|Default|SetTimeOfLightInSocket (- (Variables|Default|GetTimeOfLightInSocket) 1))
        (Variables|Default|SetTimeSave (Math|Conversions|ToFloat(Integer) (Variables|Default|GetTimeOfLightInSocket)))
        (elif (> (Variables|Default|GetTimeSave) 0.0)
          (Variables|Default|SetTimeSave (- (Variables|Default|GetTimeSave) (Variables|Default|GetReductionValue)))
          (Actor|Tick|SetActorTickEnabled false)
          (else
            (Variables|Default|SetTimeSave 0.0)))))))

(fn ConstructionScript)

(fn LightSocketState
  (bind _output_get (Variables|Default|SetbLightOnSocket (Variables|Default|GetbLightOnSocket)))
  (return _output_get))