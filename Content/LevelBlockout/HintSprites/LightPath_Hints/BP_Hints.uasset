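; BP_Hints is a light-path hint plane whose opacity and emission respond to the distance of the BP_LightOrb.
; Overlapping its sphere starts a fast looping timer that maps orb distance onto both material parameters, strongest when close; leaving pauses it.
; Pressing or releasing the I key creates a fresh dynamic material, sets its opacity from a timeline and switches plane collision on or off respectively.
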(event OnComponentBeginOverlap(Sphere)
  (params (OverlappedComponent :type Primitive%20Component%20Object%20Reference) (OtherActor :type Actor%20Object%20Reference) (OtherComp :type Primitive%20Component%20Object%20Reference) (OtherBodyIndex :type Integer) (bFromSweep :type Boolean) (SweepResult :type Hit%20Result%20Structure%20%28by%20ref%29))
  (bind _asbp_light_orb (Utilities|Casting|CastToBP_LightOrb OtherActor))
  (Variables|Default|SetLightOrbRef! _asbp_light_orb)
  (bind _returnvalue (Utilities|Time|SetTimerbyEvent (delegate Custom|UpdateOpacity) 0.001 true))
  (Variables|Default|SetTimer _returnvalue))

(event OnComponentEndOverlap(Sphere)
  (params (OverlappedComponent :type Primitive%20Component%20Object%20Reference) (OtherActor :type Actor%20Object%20Reference) (OtherComp :type Primitive%20Component%20Object%20Reference) (OtherBodyIndex :type Integer))
  (Utilities|Time|PauseTimerbyHandle (Variables|Default|GetTimer)))

(event Custom|UpdateOpacity
  (bind _distanceofdissapear (Variables|Default|GetDistanceOfDissapear))
  (bind _plane (Variables|Default|GetPlane))
  (bind _plane_2 (Variables|Default|GetPlane))
  (bind _lightorbref_ (Variables|Default|GetLightOrbRef!))
  (bind _returnvalue (Transformation|GetActorLocation _lightorbref_))
  (bind _returnvalue_2 (Transformation|GetWorldLocation _plane))
  (bind _returnvalue_3 (Math|Vector|Distance(Vector) _returnvalue _returnvalue_2))
  (Rendering|Material|SetScalarParameterValueonMaterials _plane_2 "Opacity" (Math|Float|MapRangeClamped _returnvalue_3 0.0 _distanceofdissapear 1.0 0.0))
  (Rendering|Material|SetScalarParameterValueonMaterials _plane_2 "Emission" (Math|Float|MapRangeClamped _returnvalue_3 0.0 _distanceofdissapear 1e+01 0.0)))

(event EventBeginPlay
  (Rendering|Material|CreateDynamicMaterialInstance (Variables|Default|GetPlane) 0 (Variables|Default|GetMaterialToFind) "None" :!class /Script/Engine.PrimitiveComponent)
  (Variables|Default|SetDistanceOfDissapear (Variables|Default|GetDistanceOfDissapear)))

(event Input|KeyboardEvents|I
  (params (Key :type Key%20Structure :default "None"))
  (bind _plane (Variables|Default|GetPlane))
  (:Pressed
    (bind _returnvalue (Rendering|Material|CreateDynamicMaterialInstance _plane 0 "/Game/LevelBlockout/HintSprites/LightPath_Hints/MATERIALS/M_LightPath7.M_LightPath7" "None" :!class /Script/Engine.PrimitiveComponent))
    (bind _opacity_change (Timeline|Visible PlayFromStart)
      (:Finished
        (Rendering|Material|SetScalarParameterValue _returnvalue "Dynamic_opacity" _opacity_change :!class /Script/Engine.MaterialInstanceDynamic)
        (Collision|SetCollisionEnabled _plane "QueryAndPhysics"))))
  (:Released
    (bind _returnvalue_2 (Rendering|Material|CreateDynamicMaterialInstance _plane 0 "/Game/LevelBlockout/HintSprites/LightPath_Hints/MATERIALS/M_LightPath7.M_LightPath7" "None" :!class /Script/Engine.PrimitiveComponent))
    (bind _opacity_change_2 (Timeline|Opacity PlayFromStart)
      (:Update
        (Rendering|Material|SetScalarParameterValue _returnvalue_2 "Dynamic_opacity" _opacity_change_2 :!class /Script/Engine.MaterialInstanceDynamic)
        (Collision|SetCollisionEnabled _plane "NoCollision")))))

(fn ConstructionScript)