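; Crane platform that lowers once when activated, with a camera cutaway and a scraping MetaSound.
; OnActivation blends the view to CameraToFind while timelines lerp the platform to NewLocation and Z-scale two hook meshes, then restores the player's camera and mutes the scrape.
; Later activations only play a platform noise.
; RestoreProgress resets platform, hooks and activation for respawn unless ProgressSaving has marked it saved.
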(event EventBeginPlay
  (Variables|Components|SetInitialLocation (Variables|/Script/Engine.SceneComponent|GetRelativeLocation (Variables|Default|GetPlatform)))
  (Variables|Components|SetNewLocation (Variables|Components|GetNewLocation))
  (bind _returnvalue (Audio|SpawnSoundAttached "/Game/Audio/Metasounds/Metasound_Concretescrape.Metasound_Concretescrape" (Variables|Default|GetPlatform) "None" "0, 0, 0" "0, 0, 0" "KeepRelativeOffset" false 1.0 1.0 0.0 0 0))
  (bind _output_get (Variables|Default|SetScrapeSound _returnvalue))
  (Audio|Parameter|SetFloatParameter _output_get "GainScrape" 0.0 :!class /Script/Engine.AudioComponent))

(event EventOnActivation
  (bind _asbp_third_person_character (Utilities|Casting|CastToBP_ThirdPersonCharacter (Game|GetPlayerCharacter 0)))
  (bind _output_get (Variables|Default|SetAs%20BP%20Third%20Person%20Character _asbp_third_person_character))
  (Variables|Default|SetCameraToReturnTo (Variables|/Game/ThirdPerson/Blueprints/BP_ThirdPersonCharacter.BP_ThirdPersonCharacter_C|GetActive%20Camera _output_get))
  (if (not (Variables|Default|GetbIsActivated))
    (Utilities|FlowControl|DoOnce false
      (:Completed
        (Variables|Default|SetbIsActivated true)
        (Game|Player|SetViewTargetwithBlend (Game|GetPlayerController 0) (Variables|Default|GetCameraToFind) 1.0 "VTBlend_Linear" 0.0 false)
        ;[1 1 1] audio
        (Audio|Parameter|SetFloatParameter (Variables|Default|GetScrapeSound) "GainScrape" 0.8 :!class /Script/Engine.AudioComponent)
        ;[1 1 1] moving version 1
        (Utilities|FlowControl|Sequence
          (:then_0
            (bind _movement (Timeline|Timeline Play)
              (:Update
                (Transformation|SetRelativeLocation (Variables|Default|GetPlatform) (Math|Vector|Lerp(Vector) (Variables|Components|GetInitialLocation) (Variables|Components|GetNewLocation) _movement) false false))
              (:Finished
                (Utilities|FlowControl|Delay 1.0)
                (Game|Player|SetViewTargetwithBlend (Game|GetPlayerController 0) (Variables|Default|GetCameraToReturnTo) 1.0 "VTBlend_Linear" 0.0 false)
                (Audio|Parameter|SetFloatParameter (Variables|Default|GetScrapeSound) "GainScrape" 0.0 :!class /Script/Engine.AudioComponent))))
          (:then_1
            ;[1 0.935 0.4766] adjustable length
            (bind _movement_2 (Timeline|Timeline_0 Play)
              (:Update
                (Transformation|SetRelativeScale3D (Variables|Default|Gethook_1unit1) (Math|Vector|MakeVector 1.0 1.0 _movement_2))))))))
    (else
      ;[0 1 0.0655] Herkus wuz here too!
      (Audio|PlaySoundatLocation "/Game/Audio/Cues/B3_platformNoise5_by_newagesoup_Cue.B3_platformNoise5_by_newagesoup_Cue" (Variables|/Script/Engine.SceneComponent|GetRelativeLocation (Variables|Default|GetPlatform)) "0, 0, 0" 1.0 1.0 0.0 0 0 0 0))))

(event EventRestoreProgress
  ;[1 1 1] Saving and Restoring at Respawn
  (if (not (Variables|Default|GetbIsSaved))
    (Transformation|SetRelativeLocation (Variables|Default|GetPlatform) (Variables|Components|GetInitialLocation) false true)
    (Development|PrintString "Restore Original Postion/State of CraneGoingDown")
    (Variables|Default|SetbIsActivated false)
    (Transformation|SetRelativeScale3D (Variables|Default|Gethook_1unit1) (Math|Vector|MakeVector 1.0 1.0 1.0))
    (Utilities|FlowControl|DoOnce false) ; enters at Reset
  ))

(event EventProgressSaving
  ;[1 1 1] Saving and Restoring at Respawn
  (Variables|Default|SetbIsSaved true))

(event Input|KeyboardEvents|5
  (params (Key :type Key%20Structure :default "None"))
  ;[0.859 1 0.4972] placeholder debug test
)

(fn ConstructionScript)