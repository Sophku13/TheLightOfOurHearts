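; BP_SubLevelLoader is a two-trigger actor that swaps a pair of streamed sublevels at a transition point.
; Overlapping LoadNext loads LevelToLoad and unloads LevelToUnload, while LoadPrev does the reverse, both without blocking.
; Ending overlap on either trigger disables its overlap events and enables the other's, so the two alternate.
; The overlap handlers do not filter which actor triggers them.
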(event OnComponentBeginOverlap(LoadNext)
  (params (OverlappedComponent :type Primitive%20Component%20Object%20Reference) (OtherActor :type Actor%20Object%20Reference) (OtherComp :type Primitive%20Component%20Object%20Reference) (OtherBodyIndex :type Integer) (bFromSweep :type Boolean) (SweepResult :type Hit%20Result%20Structure%20%28by%20ref%29))
  (Game|LoadStreamLevel(byName) (Variables|Default|GetLevelToLoad) true)
  (Game|UnloadStreamLevel(byName) (Variables|Default|GetLevelToUnload) false))

(event OnComponentEndOverlap(LoadNext)
  (params (OverlappedComponent :type Primitive%20Component%20Object%20Reference) (OtherActor :type Actor%20Object%20Reference) (OtherComp :type Primitive%20Component%20Object%20Reference) (OtherBodyIndex :type Integer))
  (Variables|/Script/Engine.PrimitiveComponent|SetbGenerateOverlapEvents (Variables|Default|GetLoadPrev) true)
  (Variables|/Script/Engine.PrimitiveComponent|SetbGenerateOverlapEvents (Variables|Default|GetLoadNext) false))

(event OnComponentBeginOverlap(LoadPrev)
  (params (OverlappedComponent :type Primitive%20Component%20Object%20Reference) (OtherActor :type Actor%20Object%20Reference) (OtherComp :type Primitive%20Component%20Object%20Reference) (OtherBodyIndex :type Integer) (bFromSweep :type Boolean) (SweepResult :type Hit%20Result%20Structure%20%28by%20ref%29))
  (Game|LoadStreamLevel(byName) (Variables|Default|GetLevelToUnload) true)
  (Game|UnloadStreamLevel(byName) (Variables|Default|GetLevelToLoad) false))

(event OnComponentEndOverlap(LoadPrev)
  (params (OverlappedComponent :type Primitive%20Component%20Object%20Reference) (OtherActor :type Actor%20Object%20Reference) (OtherComp :type Primitive%20Component%20Object%20Reference) (OtherBodyIndex :type Integer))
  (Variables|/Script/Engine.PrimitiveComponent|SetbGenerateOverlapEvents (Variables|Default|GetLoadNext) true)
  (Variables|/Script/Engine.PrimitiveComponent|SetbGenerateOverlapEvents (Variables|Default|GetLoadPrev) false))

(fn ConstructionScript)