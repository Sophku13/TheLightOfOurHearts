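; Platform that tips to a new rotation when the third-person character overlaps its trigger box.
; The overlap plays a timeline that lerps the Cube's relative rotation from the pose saved at BeginPlay to NewRotation; location is stored but never animated.
; It also attaches a concrete-scrape MetaSound to the Cube, setting its GainScrape parameter to zero at both start and finish.
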(event OnComponentBeginOverlap(Box)
  (params (OverlappedComponent :type Primitive%20Component%20Object%20Reference) (OtherActor :type Actor%20Object%20Reference) (OtherComp :type Primitive%20Component%20Object%20Reference) (OtherBodyIndex :type Integer) (bFromSweep :type Boolean) (SweepResult :type Hit%20Result%20Structure%20%28by%20ref%29))
  (Utilities|Casting|CastToBP_ThirdPersonCharacter OtherActor)
  (bind _returnvalue (Audio|SpawnSoundAttached "/Game/Audio/Metasound_ConcretescrapeLimited.Metasound_ConcretescrapeLimited" (Variables|Default|GetCube) "None" "0, 0, 0" "0, 0, 0" "KeepRelativeOffset" false 1.0 1.0 0.0 0 0))
  (Audio|Parameter|SetFloatParameter _returnvalue "GainScrape" 0.0 :!class /Script/Engine.AudioComponent)
  (bind _newtrack_0 (Timeline|Timeline Play)
    (:Update
      (Transformation|SetRelativeRotation (Variables|Default|GetCube) (Math|Rotator|Lerp(Rotator) (Variables|Default|GetInitialRotation) (Variables|Default|GetNewRotation) _newtrack_0) false false))
    (:Finished
      (Audio|Parameter|SetFloatParameter _returnvalue "GainScrape" 0.0 :!class /Script/Engine.AudioComponent))))

(event EventBeginPlay
  (bind _cube (Variables|Default|GetCube))
  (Variables|Default|SetInitialRotation (Variables|/Script/Engine.SceneComponent|GetRelativeRotation _cube))
  (Variables|Default|SetInitialLocation (Variables|/Script/Engine.SceneComponent|GetRelativeLocation _cube))
  (Variables|Default|SetNewRotation (Variables|Default|GetNewRotation))
  (Variables|Default|SetNewLocation (Variables|Default|GetNewLocation)))

(event Collision|EventActorBeginOverlap
  (params (OtherActor :type Actor%20Object%20Reference)))

(event EventTick
  (params (DeltaSeconds :type Float%20%28single-precision%29)))

(fn ConstructionScript)