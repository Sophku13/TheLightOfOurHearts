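; BP_BlowMechanic is a short-lived hazard actor that damages what overlaps its trigger boxes, sparing the player.
; On overlap, it casts the first player character to BP_ThirdPersonCharacter and compares it against the other actor.
; Non-player actors receive BaseDamage through ApplyDamage when the DoesDamage flag is set.
; The actor destroys itself after a fixed delay from BeginPlay.
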(event EventBeginPlay
  ;[0.1216 0.902 0.6627] Destroys Actor after completion
  (Utilities|FlowControl|Delay 6.0)
  (Actor|DestroyActor))

(event Collision|EventActorBeginOverlap
  (params (OtherActor :type Actor%20Object%20Reference))
  ;[0.1216 0.902 0.6627] Applies damage to everything in the triggerboxes that is not the player
  (bind _asbp_third_person_character (Utilities|Casting|CastToBP_ThirdPersonCharacter (Game|GetPlayerCharacter 0)))
  (if (!= OtherActor _asbp_third_person_character)
    (if (Variables|Default|GetbDoesDamage)
      (Game|Damage|ApplyDamage OtherActor (Variables|Default|GetBaseDamage) 0 0))))

(fn ConstructionScript)