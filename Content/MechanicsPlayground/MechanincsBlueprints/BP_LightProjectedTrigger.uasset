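; BP_LightProjectedTrigger is a trigger volume that temporarily hands player control to a light orb pawn at a linked projection.
; When BP_ThirdPersonCharacter overlaps the box, its movement stops and a BP_PawnLightOrb spawns at the projection's OrbLocation.
; Player controller 0 possesses the orb and blends the view to the projection actor.
; After a fixed delay, the view blends back and the character is repossessed; the orb is not destroyed here.
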(event OnComponentBeginOverlap(Box)
  (params (OverlappedComponent :type Primitive%20Component%20Object%20Reference) (OtherActor :type Actor%20Object%20Reference) (OtherComp :type Primitive%20Component%20Object%20Reference) (OtherBodyIndex :type Integer) (bFromSweep :type Boolean) (SweepResult :type Hit%20Result%20Structure%20%28by%20ref%29))
  (bind _returnvalue (Game|GetPlayerController 0))
  (bind _connectedprojectionref (Variables|Default|GetConnectedProjectionRef))
  (bind _orblocation (Variables|/Game/MechanicsPlayground/MechanincsBlueprints/BP_LightProjectedMechanic.BP_LightProjectedMechanic_C|GetOrbLocation _connectedprojectionref))
  (bind _returnvalue_2 (Transformation|GetWorldTransform _orblocation))
  (bind _asbp_third_person_character (Utilities|Casting|CastToBP_ThirdPersonCharacter OtherActor))
  (bind _output_get (Variables|Default|SetPlayerRef _asbp_third_person_character))
  (Class|NavMovementComponent|StopActiveMovement (Variables|/Script/Engine.Character|GetCharacterMovement _output_get))
  (bind _returnvalue_3 (Game|SpawnActorfromClass "/Game/MechanicsPlayground/MechanincsBlueprints/BP_PawnLightOrb.BP_PawnLightOrb_C" (Math|Transform|MakeTransform (.location _returnvalue_2) (.rotation _returnvalue_2) "1.000000,1.000000,1.000000") "Undefined" "MultiplyWithRoot" 0 0))
  (Pawn|Possess _returnvalue _returnvalue_3)
  (Game|Player|SetViewTargetwithBlend _returnvalue (Variables|Default|GetConnectedProjectionRef) 1.0 "VTBlend_EaseIn" 0.0 false)
  (Utilities|FlowControl|Delay 1e+01)
  (Game|Player|SetViewTargetwithBlend (Game|GetPlayerController 0) (Variables|Default|GetPlayerRef) 1.0 "VTBlend_EaseOut" 0.0 false)
  (Pawn|Possess (Game|GetPlayerController 0) (Variables|Default|GetPlayerRef)))

(event EventBeginPlay)

(event Collision|EventActorBeginOverlap
  (params (OtherActor :type Actor%20Object%20Reference)))

(event EventTick
  (params (DeltaSeconds :type Float%20%28single-precision%29)))

(fn ConstructionScript)