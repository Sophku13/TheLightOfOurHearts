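; Pushable object Blueprint that switches the player into a slowed pushing state while they overlap its Box.
; BeginPlay caches the third-person character, and Box overlap events toggle a flag that gates Tick.
; While gated on, Tick uses nonzero world X velocity to set IsPushing and lower MaxWalkSpeed, otherwise restoring both.
; Ending overlap only clears the flag, leaving pushing state and speed as last set.
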(event OnComponentBeginOverlap(Box)
  (params (OverlappedComponent :type Primitive%20Component%20Object%20Reference) (OtherActor :type Actor%20Object%20Reference) (OtherComp :type Primitive%20Component%20Object%20Reference) (OtherBodyIndex :type Integer) (bFromSweep :type Boolean) (SweepResult :type Hit%20Result%20Structure%20%28by%20ref%29))
  (if (== OtherActor (Variables|Default|GetPlayerRef))
    (Variables|Default|SetTick true)
    (else
      (Variables|Default|SetTick false))))

(event OnComponentEndOverlap(Box)
  (params (OverlappedComponent :type Primitive%20Component%20Object%20Reference) (OtherActor :type Actor%20Object%20Reference) (OtherComp :type Primitive%20Component%20Object%20Reference) (OtherBodyIndex :type Integer))
  (if (== OtherActor (Variables|Default|GetPlayerRef))
    (Variables|Default|SetTick false)))

(event EventBeginPlay
  (bind _asbp_third_person_character (Utilities|Casting|CastToBP_ThirdPersonCharacter (Game|GetPlayerCharacter 0)))
  (Variables|Default|SetPlayerRef _asbp_third_person_character))

(event EventTick
  (params (DeltaSeconds :type Float%20%28single-precision%29))
  (bind _playerref (Variables|Default|GetPlayerRef))
  (bind _charactermovement (Variables|/Script/Engine.Character|GetCharacterMovement _playerref))
  (if (Variables|Default|GetTick)
    (if (!= (.X (Math|Vector|BreakVector (Variables|/Script/Engine.MovementComponent|GetVelocity (Variables|/Script/Engine.Character|GetCharacterMovement (Variables|Default|GetPlayerRef))))) 0.0)
      (Variables|/Game/ThirdPerson/Blueprints/BP_ThirdPersonCharacter.BP_ThirdPersonCharacter_C|SetbIsPushing _playerref true)
      (Variables|/Script/Engine.CharacterMovementComponent|SetMaxWalkSpeed _charactermovement 1e+02)
      (else
        (Variables|/Game/ThirdPerson/Blueprints/BP_ThirdPersonCharacter.BP_ThirdPersonCharacter_C|SetbIsPushing _playerref false)
        (Variables|/Script/Engine.CharacterMovementComponent|SetMaxWalkSpeed _charactermovement 3.4e+02)))))

(fn ConstructionScript)