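; BP_BaseButton is the base class for interactable buttons, with an optional sign that gets a spawned glow actor when a sign material is set.
; Overlapping its box sets the character's CloseToButton flag and toggles the button's Tick.
; OnInteract uses a FlipFlop move to press the button down and green, then up and red after a delay, blocking re-interaction meanwhile.
; Children can override interaction and click events; another event triggers Light Orb pulsing.
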(event OnComponentBeginOverlap(Button_Box)
  (params (OverlappedComponent :type Primitive%20Component%20Object%20Reference) (OtherActor :type Actor%20Object%20Reference) (OtherComp :type Primitive%20Component%20Object%20Reference) (OtherBodyIndex :type Integer) (bFromSweep :type Boolean) (SweepResult :type Hit%20Result%20Structure%20%28by%20ref%29))
  ;[0.1216 0.902 0.6627] Enabling the Tick of the buttons when the player enters the button range
  (bind _asbp_third_person_character (Utilities|Casting|CastToBP_ThirdPersonCharacter OtherActor))
  (bind _output_get (Variables|Default|SetPlayerRef _asbp_third_person_character))
  (bind _output_get_2 (Variables|/Game/ThirdPerson/Blueprints/BP_ThirdPersonCharacter.BP_ThirdPersonCharacter_C|SetbCloseToButton _output_get true))
  (Variables|Default|SetbPlayerInRange _output_get_2)
  (Actor|Tick|SetActorTickEnabled true))

(event OnComponentEndOverlap(Button_Box)
  (params (OverlappedComponent :type Primitive%20Component%20Object%20Reference) (OtherActor :type Actor%20Object%20Reference) (OtherComp :type Primitive%20Component%20Object%20Reference) (OtherBodyIndex :type Integer))
  ;[0.1216 0.902 0.6627] Disabling the Tick of the buttons when the player leaves the button range
  (Utilities|Casting|CastToBP_ThirdPersonCharacter OtherActor)
  (bind _output_get (Variables|/Game/ThirdPerson/Blueprints/BP_ThirdPersonCharacter.BP_ThirdPersonCharacter_C|SetbCloseToButton (Variables|Default|GetPlayerRef) false))
  (Variables|Default|SetbPlayerInRange _output_get)
  (Actor|Tick|SetActorTickEnabled false))

(event Custom|MoveButton
  (bind _button (Variables|Default|GetButton))
  (bind _button_2 (Variables|Default|GetButton))
  ;[0.1216 0.902 0.6627] Event to give to child classes that tells all buttons what to do if it is moved. Either down and green or up again and turning red
  (Utilities|FlowControl|FlipFlop
    (:A
      ;;[0.1216 0.902 0.6627] Down Move
      (Transformation|SetRelativeLocation _button_2 (+ (Variables|/Script/Engine.SceneComponent|GetRelativeLocation _button_2) "0.000000,0.000000,-0.500000") false false)
      (Rendering|Material|SetMaterial (Variables|Default|GetButton) 0 "/Game/Materials/MI_Sphere_Emissive_Green.MI_Sphere_Emissive_Green"))
    (:B
      ;;[0.1216 0.902 0.6627] Up Move
      (Transformation|SetRelativeLocation _button (+ (Variables|/Script/Engine.SceneComponent|GetRelativeLocation _button) "0.000000,0.000000,0.500000") false false)
      (Rendering|Material|SetMaterial (Variables|Default|GetButton) 0 "/Game/Materials/MI_Sphere_Emissive_Red.MI_Sphere_Emissive_Red"))))

(event Custom|ButtonClick
  ;[0.1216 0.902 0.6627] Implementing the "ButtonClick" event to have it in all child blueprints
  (Development|PrintString "This Button is Clicked"))

(event EventBeginPlay
  (bind _signbase (Variables|Default|GetSignBase))
  (bind _returnvalue (Transformation|GetWorldTransform _signbase))
  ;[0.1216 0.902 0.6627] Begin Play
  ;;[0.1216 0.902 0.6627] Spawning a GlowSprite in front of the sign
  (bind _returnvalue_2 (Game|SpawnActorfromClass "/Game/MechanicsPlayground/MechanincsBlueprints/GlowTextures/BP_TEMPLATE_BlowGlow_Base.BP_TEMPLATE_BlowGlow_Base_C" (Math|Transform|MakeTransform (+ (.location _returnvalue) "5.000000,0.000000,0.000000") (.rotation _returnvalue) "1.000000,1.000000,1.000000") "AlwaysSpawn" "MultiplyWithRoot" 0 0))
  (Variables|Default|SetSignGlow _returnvalue_2)
  (bind _signmaterial (Variables|Default|GetSignMaterial)
    (:then
      (Class|NiagaraComponent|SetAsset (Variables|/Game/MechanicsPlayground/MechanincsBlueprints/GlowTextures/BP_TEMPLATE_BlowGlow_Base.BP_TEMPLATE_BlowGlow_Base_C|GetTextureGlow (Variables|Default|GetSignGlow)) _signmaterial false))
    (:else
      (Actor|DestroyActor (Variables|Default|GetSignGlow)))))

(event Collision|EventActorBeginOverlap
  (params (OtherActor :type Actor%20Object%20Reference)))

(event EventInfluenceLightOrb
  (params (LightOrbRef :type BP%20Light%20Orb%20Object%20Reference) (IsActive :type Boolean))
  ;[0.1216 0.902 0.6627] Sending a Signal to make the Light Orb pulse when close
  (Default|LightPulsing LightOrbRef))

(event EventOnInteract
  ;[0.1216 0.902 0.6627] Basic Action of a button that moves it if pressed. Can be overwritten by child blueprints
  (Variables|Default|SetbIsButtonPressed true)
  (CallFunction|MoveButton)
  (Utilities|FlowControl|Delay 2.0)
  (CallFunction|MoveButton)
  (Variables|Default|SetbIsButtonPressed false))

(fn ConstructionScript
  (bind _signbasematerial (Variables|Default|GetSignBaseMaterial)
    (:then
      (Rendering|Material|SetMaterial (Variables|Default|GetSignBase) 0 _signbasematerial))
    (:else)))

(fn IsInteractable
  (return (not (Variables|Default|GetbIsButtonPressed))))