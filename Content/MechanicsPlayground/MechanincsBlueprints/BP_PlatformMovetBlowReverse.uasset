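; BP_PlatformMovetBlowReverse is a moving platform that responds to the blow mechanic and returns when that contact ends.
; BeginPlay stores the Platform's relative location as the start point for a move toward NewLocation.
; When a BP_BlowMechanic actor overlaps the Box, the MoveUpDown timeline lerps the Platform between those points.
; End of overlap reverses the timeline from its current position.
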(event OnComponentBeginOverlap(Box)
  (params (OverlappedComponent :type Primitive%20Component%20Object%20Reference) (OtherActor :type Actor%20Object%20Reference) (OtherComp :type Primitive%20Component%20Object%20Reference) (OtherBodyIndex :type Integer) (bFromSweep :type Boolean) (SweepResult :type Hit%20Result%20Structure%20%28by%20ref%29))
  (Utilities|Casting|CastToBP_BlowMechanic OtherActor)
  (Development|PrintString "IsOverlapping")
  (bind _movement (Timeline|MoveUpDown Play)
    (:Update
      (Transformation|SetRelativeLocation (Variables|Default|GetPlatform) (Math|Vector|Lerp(Vector) (Variables|Default|GetInitialLocation) (Variables|Default|GetNewLocation) _movement) false false))))

(event OnComponentEndOverlap(Box)
  (params (OverlappedComponent :type Primitive%20Component%20Object%20Reference) (OtherActor :type Actor%20Object%20Reference) (OtherComp :type Primitive%20Component%20Object%20Reference) (OtherBodyIndex :type Integer))
  (Utilities|Casting|CastToBP_BlowMechanic OtherActor)
  (bind _movement (Timeline|MoveUpDown Reverse)
    (:Update
      (Transformation|SetRelativeLocation (Variables|Default|GetPlatform) (Math|Vector|Lerp(Vector) (Variables|Default|GetInitialLocation) (Variables|Default|GetNewLocation) _movement) false false))))

(event EventBeginPlay
  (Variables|Default|SetInitialLocation (Variables|/Script/Engine.SceneComponent|GetRelativeLocation (Variables|Default|GetPlatform)))
  (Variables|Default|SetNewLocation (Variables|Default|GetNewLocation)))

(fn ConstructionScript)