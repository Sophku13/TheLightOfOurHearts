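; Base Blueprint for a Teamworker button in the mechanics playground, extending a parent button class and interactable only while active.
; IsInteractable returns IsActive, and click and interact events pass straight through to the parent.
; Tick sets the button's red emissive material to its lit or off variant from IsActive every frame, rather than on state change.
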(event EventBeginPlay
  (|CallParentFunction) ; This node is disabled and will not be called.\nDrag off pins to build functionality.
)

(event Collision|EventActorBeginOverlap
  (params (OtherActor :type Actor%20Object%20Reference))
  (|CallParentFunction OtherActor) ; This node is disabled and will not be called.\nDrag off pins to build functionality.
)

(event EventTick
  (params (DeltaSeconds :type Float%20%28single-precision%29))
  (if (Variables|Default|GetbIsActive)
    (Rendering|Material|SetMaterial (Variables|Default|GetButton) 0 "/Game/Materials/MI_Sphere_Emissive_Red.MI_Sphere_Emissive_Red")
    (else
      (Rendering|Material|SetMaterial (Variables|Default|GetButton) 0 "/Game/Materials/MI_Sphere_Emissive_Red_Off.MI_Sphere_Emissive_Red_Off")))
  (|CallParentFunction DeltaSeconds))

(event EventButtonClick
  (|CallParentFunction))

(event EventOnInteract
  (|CallParentFunction))

(fn ConstructionScript
  (|CallParentFunction))

(fn IsInteractable
  (return (Variables|Default|GetbIsActive)))