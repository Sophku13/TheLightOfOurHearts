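; Dissolve box actor that publishes the transform of its Cube component to the PC_BoxData Material Parameter Collection, apparently for a box-shaped dissolve effect in materials.
; The Construction Script writes the cube's world location, world scale as bounds, and forward, right and up vectors, defining an oriented box.
; The event graph holds only disabled stubs, so it has no per-frame update.
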(event EventBeginPlay)

(event Collision|EventActorBeginOverlap
  (params (OtherActor :type Actor%20Object%20Reference)))

(event EventTick
  (params (DeltaSeconds :type Float%20%28single-precision%29)))

(fn ConstructionScript
  (bind _cube (Variables|Default|GetCube))
  (bind _cube_2 (Variables|Default|GetCube))
  (Rendering|Material|SetVectorParameterValue "/Game/MechanicsPlayground/MechanincsBlueprints/DissolveBox/PC_BoxData.PC_BoxData" "Location" (Math|Conversions|ToLinearColor(Vector) (Transformation|GetWorldLocation _cube)) :!class /Script/Engine.KismetMaterialLibrary)
  (Rendering|Material|SetVectorParameterValue "/Game/MechanicsPlayground/MechanincsBlueprints/DissolveBox/PC_BoxData.PC_BoxData" "Bounds" (Math|Conversions|ToLinearColor(Vector) (Transformation|GetWorldScale _cube)) :!class /Script/Engine.KismetMaterialLibrary)
  (Rendering|Material|SetVectorParameterValue "/Game/MechanicsPlayground/MechanincsBlueprints/DissolveBox/PC_BoxData.PC_BoxData" "X" (Math|Conversions|ToLinearColor(Vector) (Math|Vector|GetForwardVector _cube_2)) :!class /Script/Engine.KismetMaterialLibrary)
  (Rendering|Material|SetVectorParameterValue "/Game/MechanicsPlayground/MechanincsBlueprints/DissolveBox/PC_BoxData.PC_BoxData" "Y" (Math|Conversions|ToLinearColor(Vector) (Math|Vector|GetRightVector _cube_2)) :!class /Script/Engine.KismetMaterialLibrary)
  (Rendering|Material|SetVectorParameterValue "/Game/MechanicsPlayground/MechanincsBlueprints/DissolveBox/PC_BoxData.PC_BoxData" "Z" (Math|Conversions|ToLinearColor(Vector) (Math|Vector|GetUpVector _cube_2)) :!class /Script/Engine.KismetMaterialLibrary))