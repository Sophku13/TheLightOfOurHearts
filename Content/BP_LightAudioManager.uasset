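; Adaptive audio manager that layers 2D MetaSounds according to the strength of the player's light orb.
; BeginPlay spawns four layer sounds plus a master audio component and sets initial layer gains from a threshold array.
; Tick compares orb strength to the thresholds, stepping the light level and fading layers through gain timelines.
; Events toggle flanger and crusher parameters on the master component and sweep layer filter cutoffs with timelines.
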(event Custom|FadeEventEnd
  (params (AudioInput :type Audio%20Component%20Object%20Reference))
  (bind _timeline2 (Timeline|Timeline_0 PlayFromStart)
    (:Update
      (Audio|Parameter|SetFloatParameter AudioInput "GainA" _timeline2 :!class /Script/Engine.AudioComponent))))

(event Custom|FadeEventStart
  (params (AudioInput :type Audio%20Component%20Object%20Reference))
  (bind _timeline1 (Timeline|Timeline PlayFromStart)
    (:Update
      (Audio|Parameter|SetFloatParameter AudioInput "GainA" _timeline1 :!class /Script/Engine.AudioComponent))))

(event Custom|FilterEffectEnd
  (params (NewParam :type Audio%20Component%20Object%20Reference))
  (bind _filter_increase (Timeline|Timeline_2 PlayFromStart)
    (:Update
      (for _index (range 1 (- (Utilities|Array|Length (Variables|Default|GetAudioArray)) 1))
        (Audio|Parameter|SetFloatParameter (Utilities|Array|Get(acopy) (Variables|Default|GetAudioArray) _index) "CutoffA" _filter_increase :!class /Script/Engine.AudioComponent)))))

(event Custom|FilterEffectStart
  (params (NewParam :type Audio%20Component%20Object%20Reference))
  (bind _filterdecrease (Timeline|Timeline_1 PlayFromStart)
    (:Update
      (for _index (range 1 (- (Utilities|Array|Length (Variables|Default|GetAudioArray)) 1))
        (Audio|Parameter|SetFloatParameter (Utilities|Array|Get(acopy) (Variables|Default|GetAudioArray) _index) "CutoffA" _filterdecrease :!class /Script/Engine.AudioComponent)))))

(event Custom|CrusherEffectEnd
  (params (NewParam :type Audio%20Parameter%20Structure))
  (bind _mastersoundcomponent (Variables|Default|GetMasterSoundComponent))
  (Audio|Parameter|SetFloatParameter _mastersoundcomponent "CRate" 1.6e+04 :!class /Script/Engine.AudioComponent)
  (Audio|Parameter|SetFloatParameter _mastersoundcomponent "CDepth" 8.0 :!class /Script/Engine.AudioComponent))

(event Custom|FlangerEffectStart
  (params (NewParam :type Audio%20Parameter%20Structure))
  (bind _mastersoundcomponent (Variables|Default|GetMasterSoundComponent))
  (Audio|Parameter|SetFloatParameter _mastersoundcomponent "FRate" 76.0 :!class /Script/Engine.AudioComponent)
  (Audio|Parameter|SetFloatParameter _mastersoundcomponent "FDepth" 1e+01 :!class /Script/Engine.AudioComponent)
  (Audio|Parameter|SetFloatParameter _mastersoundcomponent "FDelay" 1.28 :!class /Script/Engine.AudioComponent))

(event Custom|FlangerEffectEnd
  (params (NewParam :type Audio%20Parameter%20Structure))
  (bind _mastersoundcomponent (Variables|Default|GetMasterSoundComponent))
  (Audio|Parameter|SetFloatParameter _mastersoundcomponent "FRate" 0.0 :!class /Script/Engine.AudioComponent)
  (Audio|Parameter|SetFloatParameter _mastersoundcomponent "FDepth" 0.0 :!class /Script/Engine.AudioComponent)
  (Audio|Parameter|SetFloatParameter _mastersoundcomponent "FDelay" 0.0 :!class /Script/Engine.AudioComponent))

(event Custom|CrusherEffectStart
  (params (NewParam :type Audio%20Parameter%20Structure))
  (bind _mastersoundcomponent (Variables|Default|GetMasterSoundComponent))
  (Audio|Parameter|SetFloatParameter _mastersoundcomponent "CRate" 1e+04 :!class /Script/Engine.AudioComponent)
  (Audio|Parameter|SetFloatParameter _mastersoundcomponent "CDepth" 4.0 :!class /Script/Engine.AudioComponent))

(event EventBeginPlay
  (bind _audioarray (Variables|Default|GetAudioArray))
  (Variables|Default|SetbIsReady false)
  (Utilities|FlowControl|Delay 0.2)
  (Variables|Default|SetbIsReady true)
  (Variables|Default|SetLightLevelInt 1)
  (Utilities|FlowControl|Sequence
    (:then_0
      (bind _asbp_third_person_character (Utilities|Casting|CastToBP_ThirdPersonCharacter (Game|GetPlayerCharacter 0)))
      (bind _output_get (Variables|Default|SetPlayerRef _asbp_third_person_character))
      (Default|GetLightOrbStrength (Variables|/Game/ThirdPerson/Blueprints/BP_ThirdPersonCharacter.BP_ThirdPersonCharacter_C|GetBP_LightOrbRef _output_get)))
    (:then_1
      (bind _returnvalue (Audio|SpawnSound2D "/Game/Metasound_LayerLight1.Metasound_LayerLight1" 1.0 1.0 0.0 0))
      (Utilities|Array|Add _audioarray _returnvalue)
      (bind _returnvalue_2 (Audio|SpawnSound2D "/Game/Metasound_LayerLight2.Metasound_LayerLight2" 1.0 1.0 0.0 0))
      (Utilities|Array|Add _audioarray _returnvalue_2)
      (bind _returnvalue_3 (Audio|SpawnSound2D "/Game/Metasound_LayerLight3.Metasound_LayerLight3" 1.0 1.0 0.0 0))
      (Utilities|Array|Add _audioarray _returnvalue_3)
      (bind _returnvalue_4 (Audio|SpawnSound2D "/Game/Metasound_LayerLight4.Metasound_LayerLight4" 1.0 1.0 0.0 0))
      (Utilities|Array|Add _audioarray _returnvalue_4)
      (bind _returnvalue_5 (AddComponent|AddAudioComponent false))
      (Variables|Default|SetMasterSoundComponent _returnvalue_5))
    (:then_2
      (for _index (range 1 (- (Utilities|Array|Length (Variables|Default|GetAudioArray)) 1))
        (bind _lightorbstatus (Default|GetLightOrbStrength (Variables|/Game/ThirdPerson/Blueprints/BP_ThirdPersonCharacter.BP_ThirdPersonCharacter_C|GetBP_LightOrbRef (Variables|Default|GetPlayerRef))))
        (if (> _lightorbstatus (Utilities|Array|Get(acopy) (Variables|Default|GetThresholdArray) _index))
          (Audio|Parameter|SetFloatParameter (Utilities|Array|Get(acopy) (Variables|Default|GetAudioArray) _index) "GainA" 0.25 :!class /Script/Engine.AudioComponent)
          (Variables|Default|SetLightLevelInt (+ (Variables|Default|GetLightLevelInt) 1))
          (else
            (Audio|Parameter|SetFloatParameter (Utilities|Array|Get(acopy) (Variables|Default|GetAudioArray) _index) "GainA" 0.0 :!class /Script/Engine.AudioComponent)))))))

(event EventTick
  (params (DeltaSeconds :type Float%20%28single-precision%29))
  (if (Variables|Default|GetbIsReady)
    (bind _lightorbstatus (Default|GetLightOrbStrength (Variables|/Game/ThirdPerson/Blueprints/BP_ThirdPersonCharacter.BP_ThirdPersonCharacter_C|GetBP_LightOrbRef (Variables|Default|GetPlayerRef))))
    (if (> _lightorbstatus (Utilities|Array|Get(acopy) (Variables|Default|GetThresholdArray) (Math|Integer|Clamp(Integer) (Variables|Default|GetLightLevelInt) 0 (- (Utilities|Array|Length (Variables|Default|GetThresholdArray)) 1))))
      (if (<= (+ (Variables|Default|GetLightLevelInt) 0) (- (Utilities|Array|Length (Variables|Default|GetThresholdArray)) 1))
        (Development|PrintString "New Light sound added" true true "(R=0.000000,G=0.660000,B=1.000000,A=1.000000)" 5.0)
        (CallFunction|FadeEventStart (Utilities|Array|Get(acopy) (Variables|Default|GetAudioArray) (Variables|Default|GetLightLevelInt)))
        (Variables|Default|SetLightLevelInt (Math|Integer|Clamp(Integer) (+ (Variables|Default|GetLightLevelInt) 1) 0 (- (Utilities|Array|Length (Variables|Default|GetThresholdArray)) 0))))
      (elif (not (== (Variables|Default|GetLightLevelInt) 0))
        (if (< _lightorbstatus (Utilities|Array|Get(acopy) (Variables|Default|GetThresholdArray) (- (Variables|Default|GetLightLevelInt) 1)))
          (CallFunction|FadeEventEnd (Utilities|Array|Get(acopy) (Variables|Default|GetAudioArray) (- (Variables|Default|GetLightLevelInt) 1)))
          (Variables|Default|SetLightLevelInt (- (Variables|Default|GetLightLevelInt) 1))
          (Development|PrintString "Removed light sound"))))))

(fn ConstructionScript)