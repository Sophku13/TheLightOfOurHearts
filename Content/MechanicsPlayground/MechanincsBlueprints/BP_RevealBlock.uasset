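; BP_RevealBlock is a hidden block that becomes visible and solid while a BP_LightOrb is within its Box trigger.
; Overlap begin and end play timelines that fade a dynamic M_ghost_reveal material's opacity, then toggle collision on completion, with a sound on reveal.
; IsVisible and InProgress guard transitions, so overlap changes during a fade are ignored.
; InfluenceLightOrb separately makes a given orb pulse its light.
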(event OnComponentBeginOverlap(Box)
  (params (OverlappedComponent :type Primitive%20Component%20Object%20Reference) (OtherActor :type Actor%20Object%20Reference) (OtherComp :type Primitive%20Component%20Object%20Reference) (OtherBodyIndex :type Integer) (bFromSweep :type Boolean) (SweepResult :type Hit%20Result%20Structure%20%28by%20ref%29))
  (bind _revealcube (Variables|Default|GetRevealCube))
  ;[0.1216 0.902 0.6627] Checks if the LightOrb enters the range of the blocks collision box
  (Utilities|Casting|CastToBP_LightOrb OtherActor)
  ;[0.1216 0.902 0.6627] On Hitbox Collision the Cube reveals itself and becomes collidable
  (if (not (Variables|Default|GetIsVisible))
    (if (not (Variables|Default|GetInProgress))
      (Variables|Default|SetInProgress true)
      ;[0.9978 1 0.452] Gradually visible
      (Rendering|SetVisibility _revealcube true false)
      (bind _returnvalue (Rendering|Material|CreateDynamicMaterialInstance _revealcube 0 "/Game/VFX_EnvironmentFX/GhostOutliner/ParentMaterial/M_ghost_reveal.M_ghost_reveal" "None" :!class /Script/Engine.PrimitiveComponent))
      (bind _opacity_change (Timeline|Timeline_0 Play)
        (:Update
          (Rendering|Material|SetScalarParameterValue _returnvalue "Dynamic_opacity" _opacity_change :!class /Script/Engine.MaterialInstanceDynamic))
        (:Finished
          ;;[0.1216 0.902 0.6627] Activating the Collision of the Block
          (Variables|/Script/Engine.PrimitiveComponent|SetbGenerateOverlapEvents (Variables|Default|GetRevealCube) true)
          (Collision|SetCollisionResponsetoChannel (Variables|Default|GetRevealCube) "ECC_GameTraceChannel1" "ECR_Block")
          (Collision|SetCollisionResponsetoChannel (Variables|Default|GetRevealCube) "ECC_Pawn" "ECR_Block")
          (Collision|SetCollisionEnabled (Variables|Default|GetRevealCube) "QueryAndPhysics")
          (Variables|Default|SetIsVisible true)
          (Variables|Default|SetInProgress false)
          (Audio|PlaySoundatLocation "/Game/B2_platform_reveal2_Cue.B2_platform_reveal2_Cue" (Transformation|GetActorLocation) "0, 0, 0" 1.0 1.0 0.0 0 0 0 0))))))

(event OnComponentEndOverlap(Box)
  (params (OverlappedComponent :type Primitive%20Component%20Object%20Reference) (OtherActor :type Actor%20Object%20Reference) (OtherComp :type Primitive%20Component%20Object%20Reference) (OtherBodyIndex :type Integer))
  ;[0.1216 0.902 0.6627] Checks if the LightOrb leaves the Range of the BlockCollisionBox
  (Utilities|Casting|CastToBP_LightOrb OtherActor)
  ;[0.1216 0.902 0.6627] On the end of the Hitbox Collision the Cube hides itself and becomes non collidable
  (if (Variables|Default|GetIsVisible)
    (if (not (Variables|Default|GetInProgress))
      (Variables|Default|SetInProgress true)
      ;[1 0.9833 0.5045] Gradually invisible
      (bind _returnvalue (Rendering|Material|CreateDynamicMaterialInstance (Variables|Default|GetRevealCube) 0 "/Game/VFX_EnvironmentFX/GhostOutliner/ParentMaterial/M_ghost_reveal.M_ghost_reveal" "None" :!class /Script/Engine.PrimitiveComponent))
      (bind _opacity_change (Timeline|Timeline PlayFromStart)
        (:Update
          (Rendering|Material|SetScalarParameterValue _returnvalue "Dynamic_opacity" _opacity_change :!class /Script/Engine.MaterialInstanceDynamic))
        (:Finished
          ;;[0.1216 0.902 0.6627] Disabling the collision of the platform
          (Variables|/Script/Engine.PrimitiveComponent|SetbGenerateOverlapEvents (Variables|Default|GetRevealCube) false)
          (Collision|SetCollisionResponsetoChannel (Variables|Default|GetRevealCube) "ECC_GameTraceChannel1" "ECR_Ignore")
          (Collision|SetCollisionResponsetoChannel (Variables|Default|GetRevealCube) "ECC_Pawn" "ECR_Ignore")
          (Collision|SetCollisionEnabled (Variables|Default|GetRevealCube) "NoCollision")
          (Variables|Default|SetIsVisible false)
          (Variables|Default|SetInProgress false))))))

(event EventBeginPlay
  ;[0.1216 0.902 0.6627] Begin Play set Invisible
  (Rendering|SetVisibility (Variables|Default|GetRevealCube) false false))

(event EventInfluenceLightOrb
  (params (LightOrbRef :type BP%20Light%20Orb%20Object%20Reference) (IsActive :type Boolean))
  ;[0.1216 0.902 0.6627] Makes the Light Orb React to itself
  (Default|LightPulsing LightOrbRef))

(fn ConstructionScript)