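; BP_RespawnPointSewers is a checkpoint that updates the respawn transform when an actor overlaps its RespawnTriggerBox.
; On overlap it casts the game mode to BP_ThirdPersonGameMode and writes the overlapping actor's transform to TSpawnTransform, with no filter on which actor.
; It keeps location and scale but forces any non-zero rotation to zero, then prints a confirmation string.
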(event OnComponentBeginOverlap(RespawnTriggerBox)
  (params (OverlappedComponent :type Primitive%20Component%20Object%20Reference) (OtherActor :type Actor%20Object%20Reference) (OtherComp :type Primitive%20Component%20Object%20Reference) (OtherBodyIndex :type Integer) (bFromSweep :type Boolean) (SweepResult :type Hit%20Result%20Structure%20%28by%20ref%29))
  (bind _returnvalue (Math|Rotator|MakeRotator 0.0 0.0 0.0))
  (bind _returnvalue_2 (Transformation|GetActorTransform OtherActor))
  (bind (_location _rotation _scale) (Math|Transform|BreakTransform _returnvalue_2))
  ;[0.1216 0.902 0.6627] Setting the Respawn Point when hitting the TriggerBox.
  (bind _asbp_third_person_game_mode (Utilities|Casting|CastToBP_ThirdPersonGameMode (Game|GetGameMode)))
  (if (Utilities|Operators|NotEqual(!=) _rotation _returnvalue 0.0)
    (Variables|/Game/ThirdPerson/Blueprints/BP_ThirdPersonGameMode.BP_ThirdPersonGameMode_C|SettSpawnTransform _asbp_third_person_game_mode (Math|Transform|MakeTransform _location _returnvalue _scale))
    (else
      (Variables|/Game/ThirdPerson/Blueprints/BP_ThirdPersonGameMode.BP_ThirdPersonGameMode_C|SettSpawnTransform _asbp_third_person_game_mode _returnvalue_2)))
  (Development|PrintString "RespawnLocationSet"))

(event EventTick
  (params (DeltaSeconds :type Float%20%28single-precision%29)))

(fn ConstructionScript)