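; Elevator actor that carries the third-person character up and down, powered by the light orb at its lever.
; Lever and platform overlaps flag the player and enable Tick, which, while activated, turns the lever, holds orb decay and shifts the floor through VInterpTo.
; End overlaps on top and bottom triggers halt travel and reset the lever, while a stopper overlap sets the state for upward movement.
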(event OnComponentBeginOverlap(LeverCollision)
  (params (OverlappedComponent :type Primitive%20Component%20Object%20Reference) (OtherActor :type Actor%20Object%20Reference) (OtherComp :type Primitive%20Component%20Object%20Reference) (OtherBodyIndex :type Integer) (bFromSweep :type Boolean) (SweepResult :type Hit%20Result%20Structure%20%28by%20ref%29))
  ;[0.1216 0.902 0.6627] Contacting the Elevator
  ;;[0.1216 0.902 0.6627] Activating Elevator with Light
  (bind _returnvalue (Actor|GetActorOfClass "/Game/ThirdPerson/Blueprints/BP_ThirdPersonCharacter.BP_ThirdPersonCharacter_C"))
  (bind _output_get (Variables|Default|SetPlayerRef _returnvalue))
  (bind _asbp_light_orb (Utilities|Casting|CastToBP_LightOrb OtherActor))
  (Variables|Default|SetBPLightOrbRef _asbp_light_orb)
  (Variables|/Game/ThirdPerson/Blueprints/BP_ThirdPersonCharacter.BP_ThirdPersonCharacter_C|SetbNearElevator _output_get true)
  (Rendering|SetVisibility (Variables|Default|GetPointLight) true false)
  (Actor|Tick|SetActorTickEnabled true))

(event OnComponentEndOverlap(LeverCollision)
  (params (OverlappedComponent :type Primitive%20Component%20Object%20Reference) (OtherActor :type Actor%20Object%20Reference) (OtherComp :type Primitive%20Component%20Object%20Reference) (OtherBodyIndex :type Integer))
  (bind _playerref (Variables|Default|GetPlayerRef))
  ;[0.1216 0.902 0.6627] Ending Conditions for the Elevator and the Movement
  ;;[0.1216 0.902 0.6627] Removing all Connections and Activations, when leaving the elevator behind
  (Rendering|SetVisibility (Variables|Default|GetPointLight) false false)
  (Rendering|SetVisibility (Variables|Default|GetHighlight%20FX) false false)
  (Variables|/Game/ThirdPerson/Blueprints/BP_ThirdPersonCharacter.BP_ThirdPersonCharacter_C|SetbNearElevator _playerref false)
  (Variables|/Game/ThirdPerson/Blueprints/BP_ThirdPersonCharacter.BP_ThirdPersonCharacter_C|SetbCharacterOnElevator _playerref false)
  (Variables|/Game/MechanicsPlayground/MechanincsBlueprints/BP_LightOrb.BP_LightOrb_C|SetbDecayIsOnHold (Variables|Default|GetBPLightOrbRef) false)
  (Actor|Tick|SetActorTickEnabled false)
  (Components|Activation|Deactivate (Variables|Default|GetTop%20Collision)))

(event OnComponentEndOverlap(BottomCollision)
  (params (OverlappedComponent :type Primitive%20Component%20Object%20Reference) (OtherActor :type Actor%20Object%20Reference) (OtherComp :type Primitive%20Component%20Object%20Reference) (OtherBodyIndex :type Integer))
  ;[0.1216 0.902 0.6627] Ending Conditions for the Elevator and the Movement
  ;;[0.1216 0.902 0.6627] Reaching the Bottom
  (Utilities|Casting|CastToBP_ThirdPersonCharacter OtherActor
    (:then
      (Variables|Default|SetbIsMoving false)
      (Variables|Default|SetbIsActivated false)
      (Actor|Tick|SetActorTickEnabled false))
    (:CastFailed
      (Variables|Default|SetbIsMoving false)
      (Variables|Default|SetbIsActivated false)
      (Actor|Tick|SetActorTickEnabled false)))
  (Transformation|SetRelativeRotation (Variables|Default|GetLeverPull) "0.000000,-90.000000,140.000000" false false))

(event OnComponentEndOverlap(TopCollision)
  (params (OverlappedComponent :type Primitive%20Component%20Object%20Reference) (OtherActor :type Actor%20Object%20Reference) (OtherComp :type Primitive%20Component%20Object%20Reference) (OtherBodyIndex :type Integer))
  ;[0.1216 0.902 0.6627] Ending Conditions for the Elevator and the Movement
  ;;[0.1216 0.902 0.6627] Reaching the Top
  (Variables|Default|SetbIsAtTop true)
  (Variables|Default|SetbIsMoving false)
  (Components|Activation|Deactivate (Variables|Default|GetTop%20Collision))
  (Variables|Default|SetbIsActivated false)
  (Actor|Tick|SetActorTickEnabled false)
  (Transformation|SetRelativeRotation (Variables|Default|GetLeverPull) "0.000000,-90.000000,140.000000" false false))

(event OnComponentBeginOverlap(BottomCollision)
  (params (OverlappedComponent :type Primitive%20Component%20Object%20Reference) (OtherActor :type Actor%20Object%20Reference) (OtherComp :type Primitive%20Component%20Object%20Reference) (OtherBodyIndex :type Integer) (bFromSweep :type Boolean) (SweepResult :type Hit%20Result%20Structure%20%28by%20ref%29))
  ;[0.1216 0.902 0.6627] Contacting the Elevator
  ;;[0.1216 0.902 0.6627] Activating the Movement Possibility with Char
  (bind _asbp_third_person_character (Utilities|Casting|CastToBP_ThirdPersonCharacter OtherActor))
  (bind _output_get (Variables|Default|SetPlayerRef _asbp_third_person_character))
  (Variables|/Game/ThirdPerson/Blueprints/BP_ThirdPersonCharacter.BP_ThirdPersonCharacter_C|SetbCharacterOnElevator _output_get true)
  (Rendering|SetVisibility (Variables|Default|GetHighlight%20FX) true false)
  (if true
    _))

(event OnComponentBeginOverlap(ElevatorStopper)
  (params (OverlappedComponent :type Primitive%20Component%20Object%20Reference) (OtherActor :type Actor%20Object%20Reference) (OtherComp :type Primitive%20Component%20Object%20Reference) (OtherBodyIndex :type Integer) (bFromSweep :type Boolean) (SweepResult :type Hit%20Result%20Structure%20%28by%20ref%29))
  ;[0.1216 0.902 0.6627] Ending Conditions for the Elevator and the Movement
  ;;[0.1216 0.902 0.6627] An Elevator Stopper that bounces the Platform back up when it goes into the ground
  (Variables|Default|SetbIsAtTop false)
  (Variables|Default|SetbIsMoving true)
  (Variables|Default|SetbIsActivated true)
  (Actor|Tick|SetActorTickEnabled false)
  (Transformation|SetRelativeRotation (Variables|Default|GetLeverPull) "0.000000,-90.000000,140.000000" false false))

(event EventBeginPlay
  ;[0.1216 0.902 0.6627] Initiate Elevators
  (bind _returnvalue (Actor|GetActorOfClass "/Game/ThirdPerson/Blueprints/BP_ThirdPersonCharacter.BP_ThirdPersonCharacter_C"))
  (bind _output_get (Variables|Default|SetPlayerRef _returnvalue))
  (Variables|Default|SetBPLightOrbRef (Variables|/Game/ThirdPerson/Blueprints/BP_ThirdPersonCharacter.BP_ThirdPersonCharacter_C|GetBP_LightOrbRef _output_get))
  (Components|Activation|Deactivate (Variables|Default|GetTop%20Collision)))

(event EventTick
  (params (DeltaSeconds :type Float%20%28single-precision%29))
  (bind _bisattop (Variables|Default|GetbIsAtTop))
  (bind _leverpull (Variables|Default|GetLeverPull))
  (bind _playerref (Variables|Default|GetPlayerRef))
  (bind _playerref_2 (Variables|Default|GetPlayerRef))
  (bind _charactermovement (Variables|/Script/Engine.Character|GetCharacterMovement _playerref))
  ;[0.1216 0.902 0.6627] Elevator Movement Tick
  (if (Variables|/Game/ThirdPerson/Blueprints/BP_ThirdPersonCharacter.BP_ThirdPersonCharacter_C|GetbNearElevator _playerref_2)
    (if (Variables|/Game/ThirdPerson/Blueprints/BP_ThirdPersonCharacter.BP_ThirdPersonCharacter_C|GetbCharacterOnElevator _playerref_2)
      (if (Variables|Default|GetbIsActivated)
        (Utilities|FlowControl|Sequence
          (:then_0
            ;;[0.1216 0.902 0.6627] Lever Movement
            (if (Utilities|Operators|EqualEqual (.Rotation (Math|Transform|BreakTransform (Transformation|GetRelativeTransform _leverpull))) "0.000000,-90.000000,140.000000" 0.1)
              (Transformation|SetRelativeRotation _leverpull "0.000000,-90.000000,30.000000" false false)))
          (:then_1
            (if (Variables|Default|GetbIsMoving)
              (Variables|/Game/MechanicsPlayground/MechanincsBlueprints/BP_LightOrb.BP_LightOrb_C|SetbDecayIsOnHold (Variables|Default|GetBPLightOrbRef) true)
              (Pawn|Components|CharacterMovement|SetMovementMode _charactermovement "MOVE_None" 0)
              (if _bisattop
                ;;[0.1216 0.902 0.6627] Movement Up
                (Utilities|MElevatorMove _bisattop)
                (else
                  ;;[0.1216 0.902 0.6627] Movement Down
                  (Utilities|MElevatorMove _bisattop)))
              (Pawn|Components|CharacterMovement|SetMovementMode _charactermovement "MOVE_Walking" 0))))))))

(fn ConstructionScript)