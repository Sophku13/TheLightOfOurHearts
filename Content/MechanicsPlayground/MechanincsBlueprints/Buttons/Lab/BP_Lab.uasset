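; BP_Lab coordinates a three-room lab button mechanic that moves an orb between a start socket and an end socket.
; On BeginPlay it gives each room's button group the shared SocketMover and gathers unique move coordinates from each group's first listed button.
; Tick polls the mover's active location to set the active room group, calling MoveToLast past the final threshold.
; FirstMove and MoveToFirst handle travel between the start socket and first coordinate.
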(event Custom|SaveTheSteps
  (params (Target :type BP%20Button%20Grouper%20Base%20Object%20Reference))
  ;[1 1 1] Comment
  (bind _asbp_button_teamworker_lab_base (Utilities|Casting|CastToBP_Button_Teamworker_Lab_Base (.Value (Utilities|Map|Find (Variables|/Game/MechanicsPlayground/MechanincsBlueprints/Buttons/Bases/BP_ButtonGrouper_Base.BP_ButtonGrouper_Base_C|GetButtonList Target) 0))))
  (for _array_element (Variables|/Game/MechanicsPlayground/MechanincsBlueprints/Buttons/Lab/BP_Button_Teamworker_Lab_Base.BP_Button_Teamworker_Lab_Base_C|GetMoveCoordinates _asbp_button_teamworker_lab_base)
    (Utilities|Array|AddUnique (Variables|Default|GetallCoordinates) (Variables|/Game/MechanicsPlayground/MechanincsBlueprints/Buttons/Bases/BP_ButtonMoveLocation.BP_ButtonMoveLocation_C|GetMoveLocation _array_element))))

(event Custom|MoveToFirst
  (bind _socketmover (Variables|Default|GetSocketMover))
  ;[1 1 1] Comment
  (Default|MoveOrbtoStart _socketmover (Utilities|Array|Get(acopy) (Variables|Default|GetallCoordinates)) (Variables|/Game/MechanicsPlayground/MechanincsBlueprints/BP_PlaceLightSocket.BP_PlaceLightSocket_C|GetLocationOfSocket (Variables|/Game/MechanicsPlayground/MechanincsBlueprints/BP_MoveBetweenSocketsWithButtons_Lab.BP_MoveBetweenSocketsWithButtons_Lab_C|GetStartSocket _socketmover))))

(event Custom|MoveToLast
  (bind _allcoordinates (Variables|Default|GetallCoordinates))
  (bind _socketmover (Variables|Default|GetSocketMover))
  ;[1 1 1] Comment
  (Default|MoveOrbtoEnd _socketmover (Utilities|Array|Get(acopy) _allcoordinates (- (Utilities|Array|Length _allcoordinates) 1)) (Variables|/Game/MechanicsPlayground/MechanincsBlueprints/BP_PlaceLightSocket.BP_PlaceLightSocket_C|GetLocationOfSocket (Variables|/Game/MechanicsPlayground/MechanincsBlueprints/BP_MoveBetweenSocketsWithButtons_Lab.BP_MoveBetweenSocketsWithButtons_Lab_C|GetEndSocket _socketmover))))

(event Custom|FirstMove
  (bind _socketmover (Variables|Default|GetSocketMover))
  ;[1 1 1] Comment
  (Default|MoveOrbtoEnd _socketmover (Variables|/Game/MechanicsPlayground/MechanincsBlueprints/BP_PlaceLightSocket.BP_PlaceLightSocket_C|GetLocationOfSocket (Variables|/Game/MechanicsPlayground/MechanincsBlueprints/BP_MoveBetweenSocketsWithButtons_Lab.BP_MoveBetweenSocketsWithButtons_Lab_C|GetStartSocket _socketmover)) (Utilities|Array|Get(acopy) (Variables|Default|GetallCoordinates))))

(event EventBeginPlay
  (bind _socketmover (Variables|Default|GetSocketMover))
  ;[1 1 1] Comment
  (Variables|/Game/MechanicsPlayground/MechanincsBlueprints/Buttons/Lab/BP_ButtonGrouper_Lab.BP_ButtonGrouper_Lab_C|SetButtonMover (Variables|Default|GetButtonGroupRoom1) _socketmover)
  (Variables|/Game/MechanicsPlayground/MechanincsBlueprints/Buttons/Lab/BP_ButtonGrouper_Lab.BP_ButtonGrouper_Lab_C|SetButtonMover (Variables|Default|GetButtonGroupRoom2) _socketmover)
  (Variables|/Game/MechanicsPlayground/MechanincsBlueprints/Buttons/Lab/BP_ButtonGrouper_Lab.BP_ButtonGrouper_Lab_C|SetButtonMover (Variables|Default|GetButtonGroupRoom3) _socketmover)
  (bind _activeposition (Default|GetActiveLocation _socketmover))
  (Variables|Default|SetActiveLocation _activeposition)
  (CallFunction|SavetheSteps (Variables|Default|GetButtonGroupRoom1))
  (CallFunction|SavetheSteps (Variables|Default|GetButtonGroupRoom2))
  (CallFunction|SavetheSteps (Variables|Default|GetButtonGroupRoom3)))

(event Collision|EventActorBeginOverlap
  (params (OtherActor :type Actor%20Object%20Reference)))

(event EventTick
  (params (DeltaSeconds :type Float%20%28single-precision%29))
  ;[1 1 1] Comment
  (bind _activeposition (Default|GetActiveLocation (Variables|Default|GetSocketMover)))
  (Variables|Default|SetActiveLocation _activeposition)
  (if (< _activeposition 4)
    (Variables|Default|SetActiveGroup 1)
    (elif (< _activeposition 7)
      (Variables|Default|SetActiveGroup 2)
      (elif (< _activeposition 11)
        (Variables|Default|SetActiveGroup 3)
        (else
          (CallFunction|MovetoLast))))))

(fn ConstructionScript)