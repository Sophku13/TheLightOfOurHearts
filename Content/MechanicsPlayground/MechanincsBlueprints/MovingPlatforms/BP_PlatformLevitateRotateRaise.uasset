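; Moving platform that raises and rotates while a BP_RaiseMechanic actor overlaps its trigger box.
; A timeline lerps the platform to a target location and rotation at a scaled play rate, then activates InterpToMovement.
; When the overlap ends, InterpToMovement stops and the timeline reverses after a delay at its own rate.
; It also attaches a concrete-scrape MetaSound at zero gain and can trigger pulsing on a passed-in light orb.
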(event OnComponentBeginOverlap(Box)
  (params (OverlappedComponent :type Primitive%20Component%20Object%20Reference) (OtherActor :type Actor%20Object%20Reference) (OtherComp :type Primitive%20Component%20Object%20Reference) (OtherBodyIndex :type Integer) (bFromSweep :type Boolean) (SweepResult :type Hit%20Result%20Structure%20%28by%20ref%29))
  (bind _platform (Variables|Default|GetPlatform))
  (bind _moveupdown (Variables|Default|GetMoveUpDown))
  (Utilities|Casting|CastToBP_RaiseMechanic OtherActor)
  (Components|Timeline|SetPlayRate _moveupdown (* (Components|Timeline|GetTimelineLength _moveupdown) (Variables|Default|GetTimeLineLength)))
  (bind (_direction _movement _rotation) (Timeline|MoveUpDown Play)
    (:Update
      (Transformation|SetRelativeLocation _platform (Math|Vector|Lerp(Vector) (Variables|Default|GetInitialLocation) (Variables|Default|GetNewLocation) _movement) false false)
      (Transformation|SetRelativeRotation _platform (Math|Rotator|Lerp(Rotator) (Variables|Default|GetInitialRotation) (Variables|Default|GetNewRotation) _rotation) false false))
    (:Finished
      (Components|Activation|Activate (Variables|Default|GetInterpToMovement) true))))

(event OnComponentEndOverlap(Box)
  (params (OverlappedComponent :type Primitive%20Component%20Object%20Reference) (OtherActor :type Actor%20Object%20Reference) (OtherComp :type Primitive%20Component%20Object%20Reference) (OtherBodyIndex :type Integer))
  (bind _platform (Variables|Default|GetPlatform))
  (bind _moveupdown (Variables|Default|GetMoveUpDown))
  (bind _interptomovement (Variables|Default|GetInterpToMovement))
  (Utilities|Casting|CastToBP_RaiseMechanic OtherActor)
  (Components|Activation|Deactivate _interptomovement)
  (Utilities|FlowControl|Delay (Variables|Default|GetTimeOfDelay))
  (Components|Timeline|SetPlayRate _moveupdown (* (Components|Timeline|GetTimelineLength _moveupdown) (Variables|Default|GetTimeOfFall)))
  (bind (_direction _movement _rotation) (Timeline|MoveUpDown Reverse)
    (:Update
      (Transformation|SetRelativeLocation _platform (Math|Vector|Lerp(Vector) (Variables|Default|GetInitialLocation) (Variables|Default|GetNewLocation) _movement) false false)
      (Transformation|SetRelativeRotation _platform (Math|Rotator|Lerp(Rotator) (Variables|Default|GetInitialRotation) (Variables|Default|GetNewRotation) _rotation) false false))
    (:Finished
      (Components|Activation|Activate _interptomovement true))))

(event EventBeginPlay
  (bind _platform (Variables|Default|GetPlatform))
  (Variables|Default|SetInitialLocation (Variables|/Script/Engine.SceneComponent|GetRelativeLocation _platform))
  (Variables|Default|SetInitialRotation (Variables|/Script/Engine.SceneComponent|GetRelativeRotation _platform))
  (Variables|Default|SetNewLocation (Variables|Default|GetNewLocation))
  (bind _returnvalue (Audio|SpawnSoundAttached "/Game/Audio/Metasounds/Metasound_Concretescrape.Metasound_Concretescrape" (Variables|Default|GetPlatform) "None" "0, 0, 0" "0, 0, 0" "KeepRelativeOffset" false 1.0 1.0 0.0 0 0))
  (bind _output_get (Variables|Default|SetScrapeSound _returnvalue))
  (Audio|Parameter|SetFloatParameter _output_get "GainScrape" 0.0 :!class /Script/Engine.AudioComponent))

(event EventInfluenceLightOrb
  (params (LightOrbRef :type BP%20Light%20Orb%20Object%20Reference) (IsActive :type Boolean))
  ;[1 1 1] Comment
  (Default|LightPulsing LightOrbRef))

(fn ConstructionScript)