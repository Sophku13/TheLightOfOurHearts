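; A moving platform that travels to a target location while a BP_BlowMechanic actor overlaps its Box trigger, and returns when the overlap ends.
; The MoveUpDown timeline lerps the platform's relative location from its initial position, playing on overlap and reversing on exit.
; An attached concrete-scrape MetaSound has its gain raised during motion and muted when the timeline finishes.
; A separate InfluenceLightOrb event triggers pulsing on the passed light orb.
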(event OnComponentBeginOverlap(Box)
  (params (OverlappedComponent :type Primitive%20Component%20Object%20Reference) (OtherActor :type Actor%20Object%20Reference) (OtherComp :type Primitive%20Component%20Object%20Reference) (OtherBodyIndex :type Integer) (bFromSweep :type Boolean) (SweepResult :type Hit%20Result%20Structure%20%28by%20ref%29))
  (Utilities|Casting|CastToBP_BlowMechanic OtherActor)
  (Development|PrintString "IsOverlapping")
  (Audio|Parameter|SetFloatParameter (Variables|Default|GetScrapeSound) "GainScrape" 0.8 :!class /Script/Engine.AudioComponent)
  (bind _movement (Timeline|MoveUpDown Play)
    (:Update
      (Transformation|SetRelativeLocation (Variables|Default|GetPlatform) (Math|Vector|Lerp(Vector) (Variables|Default|GetInitialLocation) (Variables|Default|GetNewLocation) _movement) false false))
    (:Finished
      (Audio|Parameter|SetFloatParameter (Variables|Default|GetScrapeSound) "GainScrape" 0.0 :!class /Script/Engine.AudioComponent))))

(event OnComponentEndOverlap(Box)
  (params (OverlappedComponent :type Primitive%20Component%20Object%20Reference) (OtherActor :type Actor%20Object%20Reference) (OtherComp :type Primitive%20Component%20Object%20Reference) (OtherBodyIndex :type Integer))
  (Utilities|Casting|CastToBP_BlowMechanic OtherActor)
  (Audio|Parameter|SetFloatParameter (Variables|Default|GetScrapeSound) "GainScrape" 0.8 :!class /Script/Engine.AudioComponent)
  (bind _movement (Timeline|MoveUpDown Reverse)
    (:Update
      (Transformation|SetRelativeLocation (Variables|Default|GetPlatform) (Math|Vector|Lerp(Vector) (Variables|Default|GetInitialLocation) (Variables|Default|GetNewLocation) _movement) false false))
    (:Finished
      (Audio|Parameter|SetFloatParameter (Variables|Default|GetScrapeSound) "GainScrape" 0.0 :!class /Script/Engine.AudioComponent))))

(event EventBeginPlay
  (Variables|Default|SetInitialLocation (Variables|/Script/Engine.SceneComponent|GetRelativeLocation (Variables|Default|GetPlatform)))
  (Variables|Default|SetNewLocation (Variables|Default|GetNewLocation))
  (bind _returnvalue (Audio|SpawnSoundAttached "/Game/Audio/Metasounds/Metasound_Concretescrape.Metasound_Concretescrape" (Variables|Default|GetPlatform) "None" "0, 0, 0" "0, 0, 0" "KeepRelativeOffset" false 1.0 1.0 0.0 0 0))
  (bind _output_get (Variables|Default|SetScrapeSound _returnvalue))
  (Audio|Parameter|SetFloatParameter _output_get "GainScrape" 0.0 :!class /Script/Engine.AudioComponent))

(event EventInfluenceLightOrb
  (params (LightOrbRef :type BP%20Light%20Orb%20Object%20Reference) (IsActive :type Boolean))
  ;[1 1 1] Comment
  (Default|LightPulsing LightOrbRef))

(fn ConstructionScript)