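; BP_DarkObj is a dark hazard cube that shifts as the player moves and drains the player's light orb on contact.
; Each tick the player moves horizontally, the cube steps by WhereObjectMoves, flipping direction based on relative X position.
; While DeathCollision overlaps the player, movement stops and a tick counter periodically reduces orb strength.
; A BP_RaiseMechanic entering the Sphere dissolves the cube via timeline and disables collision; leaving restores both.
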(event OnComponentBeginOverlap(Sphere)
  (params (OverlappedComponent :type Primitive%20Component%20Object%20Reference) (OtherActor :type Actor%20Object%20Reference) (OtherComp :type Primitive%20Component%20Object%20Reference) (OtherBodyIndex :type Integer) (bFromSweep :type Boolean) (SweepResult :type Hit%20Result%20Structure%20%28by%20ref%29))
  (bind _cube (Variables|Default|GetCube))
  (Utilities|Casting|CastToBP_RaiseMechanic OtherActor)
  (bind _newtrack_0 (Timeline|DissolveObj PlayFromStart)
    (:Update
      (Rendering|Material|SetScalarParameterValueonMaterials _cube "Opacity" _newtrack_0)
      (Collision|SetCollisionEnabled _cube "NoCollision")
      (Collision|SetCollisionEnabled (Variables|Default|GetDeathCollision) "NoCollision"))))

(event OnComponentEndOverlap(Sphere)
  (params (OverlappedComponent :type Primitive%20Component%20Object%20Reference) (OtherActor :type Actor%20Object%20Reference) (OtherComp :type Primitive%20Component%20Object%20Reference) (OtherBodyIndex :type Integer))
  (bind _cube (Variables|Default|GetCube))
  (Utilities|Casting|CastToBP_RaiseMechanic OtherActor)
  (Rendering|Material|SetScalarParameterValueonMaterials _cube "Opacity" 1.0)
  (Collision|SetCollisionEnabled _cube "QueryAndPhysics")
  (Collision|SetCollisionEnabled (Variables|Default|GetDeathCollision) "QueryAndPhysics"))

(event OnComponentBeginOverlap(DeathCollision)
  (params (OverlappedComponent :type Primitive%20Component%20Object%20Reference) (OtherActor :type Actor%20Object%20Reference) (OtherComp :type Primitive%20Component%20Object%20Reference) (OtherBodyIndex :type Integer) (bFromSweep :type Boolean) (SweepResult :type Hit%20Result%20Structure%20%28by%20ref%29))
  (Utilities|Casting|CastToBP_ThirdPersonCharacter OtherActor)
  (Development|PrintString "Overlaps")
  (Variables|Default|SetPlayerHitByObj true))

(event OnComponentEndOverlap(DeathCollision)
  (params (OverlappedComponent :type Primitive%20Component%20Object%20Reference) (OtherActor :type Actor%20Object%20Reference) (OtherComp :type Primitive%20Component%20Object%20Reference) (OtherBodyIndex :type Integer))
  (Utilities|Casting|CastToBP_ThirdPersonCharacter OtherActor)
  (Development|PrintString "Doesn'tOverlap")
  (Variables|Default|SetPlayerHitByObj false))

(event EventBeginPlay
  (bind _asbp_third_person_character (Utilities|Casting|CastToBP_ThirdPersonCharacter (Game|GetPlayerCharacter 0)))
  (Variables|Default|SetPlayerRef _asbp_third_person_character)
  (Variables|Default|SetWhereObjectMoves (Variables|Default|GetWhereObjectMoves)))

(event Collision|EventActorBeginOverlap
  (params (OtherActor :type Actor%20Object%20Reference)))

(event EventTick
  (params (DeltaSeconds :type Float%20%28single-precision%29))
  (bind _cube (Variables|Default|GetCube))
  (bind _playerref (Variables|Default|GetPlayerRef))
  (bind _whereobjectmoves (Variables|Default|GetWhereObjectMoves))
  (bind _returnvalue (Transformation|GetWorldLocation _cube))
  (bind _bp_lightorbref (Variables|/Game/ThirdPerson/Blueprints/BP_ThirdPersonCharacter.BP_ThirdPersonCharacter_C|GetBP_LightOrbRef _playerref))
  (bind _returnvalue_2 (Math|Vector|MakeVector (.x _returnvalue) (.y _returnvalue) (.z _returnvalue)))
  (if (Variables|Default|GetPlayerHitByObj)
    (bind _result (Math|Integer|IncrementInt (Variables|Default|GetDecayCount))
      (:%20%20
        (if (== (Variables|Default|GetRange) _result)
          (Variables|Default|SetDecayCount 0)
          (bind _lightorbstatus (Default|GetLightOrbStrength _bp_lightorbref))
          (Default|SetLightOrbStrength _bp_lightorbref (- _lightorbstatus 0.1)))))
    (else
      (bind _playerref_2 (Variables|Default|GetPlayerRef)
        (:then
          (if (not (and (Math|Float|NearlyEqual(Float) (.x (Transformation|GetVelocity _playerref_2)) 0.0 0.005) (Math|Float|NearlyEqual(Float) (.y (Transformation|GetVelocity _playerref_2)) 0.0 0.005)))
            (if (< (.x _returnvalue) (.x (Transformation|GetActorLocation (Game|GetPlayerCharacter 0))))
              (Transformation|SetWorldLocation _cube (+ _returnvalue_2 _whereobjectmoves) false false)
              (else
                (Transformation|SetWorldLocation _cube (+ _returnvalue_2 (* _whereobjectmoves -1)) false false)))))
        (:else)))))

(fn ConstructionScript)