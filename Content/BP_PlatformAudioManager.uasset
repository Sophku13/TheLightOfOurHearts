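; Manager actor that plays one shared 2D concrete-scrape MetaSound whenever any raise or reversed-raise platform is moving.
; BeginPlay caches both platform types and spawns the sound silent, then Tick polls their IsPlatformMoving flags.
; A pair of DoOnce gates triggers transitions: GainScrape jumps to full on start and follows a timeline on stop, re-arming the start gate when finished.
; PlatformAudioCheck is an abandoned event-based attempt.
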(event Custom|PlatformAudioCheck
  (params (NewParam :type Boolean))
  (bind _globalscrapesound (Variables|Default|GetGlobalScrapeSound))
  ;[1 1 1] Wanted to remake the function with events but this doesn't really work with the current platform setup
  (Variables|Default|SetbShouldPlaySound false)
  (bind _array_element (Utilities|Array|ForEachLoopwithBreak (Variables|Default|GetOut%20Actors) :!label _label)
    (:LoopBody
      (if (Variables|/Game/MechanicsPlayground/MechanincsBlueprints/MovingPlatforms/BP_PlatformMoveRaiseReversed.BP_PlatformMoveRaiseReversed_C|GetbIsPlatformMoving _array_element)
        (Variables|Default|SetbShouldPlaySound true)
        (goto _label Break)))
    (:Completed
      (if (Variables|Default|GetbShouldPlaySound)
        (Audio|Parameter|SetFloatParameter _globalscrapesound "GainScrape" 1.0 :!class /Script/Engine.AudioComponent)
        (else
          (Audio|Parameter|SetFloatParameter _globalscrapesound "GainScrape" 0.0 :!class /Script/Engine.AudioComponent))))))

(event Custom|PlatformFadeOut
  (Development|PrintString "finished")
  (bind _newtrack_2 (Timeline|Timeline_0 PlayFromStart)
    (:Update
      (Audio|Parameter|SetFloatParameter (Variables|Default|GetGlobalScrapeSound) "GainScrape" _newtrack_2 :!class /Script/Engine.AudioComponent))
    (:Finished
      (CallFunction|Reseton))))

(event Custom|PlatformFadeIn
  (Audio|Parameter|SetFloatParameter (Variables|Default|GetGlobalScrapeSound) "GainScrape" 1.0 :!class /Script/Engine.AudioComponent)
  (CallFunction|ResetOff))

(event Custom|ResetOff
  (Utilities|FlowControl|DoOnce false) ; enters at Reset
)

(event Custom|ResetOn
  (Utilities|FlowControl|DoOnce false) ; enters at Reset
)

(event EventBeginPlay
  (Variables|Default|SetbShouldPlaySound false)
  (bind _outactors (Actor|GetAllActorsOfClass "/Game/MechanicsPlayground/MechanincsBlueprints/MovingPlatforms/BP_PlatformMoveRaiseReversed.BP_PlatformMoveRaiseReversed_C"))
  (Variables|Default|SetOut%20Actors _outactors)
  (bind _outactors_2 (Actor|GetAllActorsOfClass "/Game/MechanicsPlayground/MechanincsBlueprints/MovingPlatforms/BP_PlatformMoveRaise.BP_PlatformMoveRaise_C"))
  (Variables|Default|SetOut%20Actors2 _outactors_2)
  (bind _returnvalue (Audio|SpawnSound2D "/Game/Audio/Metasounds/Metasound_Concretescrape.Metasound_Concretescrape" 1.0 1.0 0.0 0))
  (bind _output_get (Variables|Default|SetGlobalScrapeSound _returnvalue))
  (Audio|Parameter|SetFloatParameter _output_get "GainScrape" 0.0 :!class /Script/Engine.AudioComponent))

(event Collision|EventActorBeginOverlap
  (params (OtherActor :type Actor%20Object%20Reference)))

(event EventTick
  (params (DeltaSeconds :type Float%20%28single-precision%29))
  (Variables|Default|SetbShouldTimelineRun false)
  (Variables|Default|SetbShouldPlaySound false)
  (Utilities|FlowControl|Sequence
    (:then_0
      (bind _array_element (Utilities|Array|ForEachLoopwithBreak (Variables|Default|GetOut%20Actors) :!label _label)
        (:LoopBody
          (if (Variables|/Game/MechanicsPlayground/MechanincsBlueprints/MovingPlatforms/BP_PlatformMoveRaiseReversed.BP_PlatformMoveRaiseReversed_C|GetbIsPlatformMoving _array_element)
            (Variables|Default|SetbShouldPlaySound true)
            (goto _label Break)))))
    (:then_1
      (bind _array_element_2 (Utilities|Array|ForEachLoopwithBreak (Variables|Default|GetOut%20Actors2) :!label _label_2)
        (:LoopBody
          (if (Variables|/Game/MechanicsPlayground/MechanincsBlueprints/MovingPlatforms/BP_PlatformMoveRaise.BP_PlatformMoveRaise_C|GetbIsPlatformMoving _array_element_2)
            (Variables|Default|SetbShouldPlaySound true)
            (goto _label_2 Break)))))
    (:then_2
      (if (Variables|Default|GetbShouldPlaySound)
        (Utilities|FlowControl|DoOnce false
          (:Completed
            (Development|PrintString "On")
            (CallFunction|PlatformFadein)))
        (else
          (Utilities|FlowControl|DoOnce false
            (:Completed
              (Development|PrintString "Off")
              (CallFunction|PlatformFadeOut))))))))

(fn ConstructionScript)