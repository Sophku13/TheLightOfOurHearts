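; Footstep anim notify that plays a surface-specific step sound at the animated mesh owner's location.
; On notify, a DoOnce with no reset gates a downward WorldStatic line trace from the owner, ignoring the player character.
; The hit's physical surface selects a concrete or wood sound, and other surfaces only print a debug string.
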(fn ReceivedNotify
  (params (MeshComp :type Skeletal%20Mesh%20Component%20Object%20Reference) (Animation :type Anim%20Sequence%20Base%20Object%20Reference) (EventReference :type Anim%20Notify%20Event%20Reference%20Structure%20%28by%20ref%29))
  (bind _returnvalue (Components|GetOwner MeshComp))
  (bind _ignorable (Variables|Default|GetIgnorable))
  (bind _returnvalue_2 (Transformation|GetActorLocation _returnvalue))
  (Utilities|FlowControl|DoOnce false
    (:Completed
      (Utilities|Array|Add _ignorable (Game|GetPlayerCharacter 0))
      (bind (_outhit _returnvalue_3) (Collision|LineTraceForObjects _returnvalue_2 (+ _returnvalue_2 (* (Transformation|GetActorUpVector _returnvalue) "0.000000,0.000000,-200.000000")) (Utilities|Array|MakeArray "ObjectTypeQuery1") false _ignorable "None"))
      (if _returnvalue_3
        (switch Utilities|FlowControl|Switch|SwitchonEPhysicalSurface (Collision|GetSurfaceType _outhit)
          (:SurfaceType_Default
            (Development|PrintString "Hello"))
          (:SurfaceType1
            (Audio|PlaySoundatLocation "/Game/Audio/RawAudioFiles/Cue_ConcreteStep.Cue_ConcreteStep" _returnvalue_2 "0, 0, 0" 1.0 1.0 0.0 0 0 0 0))
          (:SurfaceType2
            (Audio|PlaySoundatLocation "/Game/Audio/RawAudioFiles/Audio_Wood_footstep.Audio_Wood_footstep" _returnvalue_2 "0, 0, 0" 1.0 1.0 0.0 0 0 0 0)))
        (return false)))))