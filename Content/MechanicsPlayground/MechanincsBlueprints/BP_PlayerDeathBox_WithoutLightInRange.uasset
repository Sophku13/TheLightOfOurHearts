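; Death volume that kills the player who enters it without the light orb held, eaten or inside the box.
; Box overlaps track the orb's presence and, on a failed check, open the character's death UI, passing itself.
; InfluencingPlayer toggles the box's overlap events, while PlayerDeath hands the player to the death manager's LightAbandonment.
; IsInfluencingThePlayer is a WIP stub that always returns true.
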(event OnComponentBeginOverlap(PlayerDeathBox)
  (params (OverlappedComponent :type Primitive%20Component%20Object%20Reference) (OtherActor :type Actor%20Object%20Reference) (OtherComp :type Primitive%20Component%20Object%20Reference) (OtherBodyIndex :type Integer) (bFromSweep :type Boolean) (SweepResult :type Hit%20Result%20Structure%20%28by%20ref%29))
  ;[0.1216 0.902 0.6627] Kills the player if the light is not in range and the Light is not held or eaten
  (Utilities|Casting|CastToBP_LightOrb OtherActor
    (:then
      (Variables|Default|SetbIsLightInRange true))
    (:CastFailed
      (bind _asbp_third_person_character (Utilities|Casting|CastToBP_ThirdPersonCharacter OtherActor))
      (if (and (Math|Boolean|NORBoolean (Variables|/Game/MechanicsPlayground/MechanincsBlueprints/BP_LightOrb.BP_LightOrb_C|GetbIsHeld (Variables|/Game/ThirdPerson/Blueprints/BP_ThirdPersonCharacter.BP_ThirdPersonCharacter_C|GetBP_LightOrbRef _asbp_third_person_character)) (Variables|/Game/MechanicsPlayground/MechanincsBlueprints/BP_LightOrb.BP_LightOrb_C|GetbIsEaten (Variables|/Game/ThirdPerson/Blueprints/BP_ThirdPersonCharacter.BP_ThirdPersonCharacter_C|GetBP_LightOrbRef _asbp_third_person_character))) (not (Variables|Default|GetbIsLightInRange)))
        (Default|OpenDeathUI _asbp_third_person_character self)))))

(event OnComponentEndOverlap(PlayerDeathBox)
  (params (OverlappedComponent :type Primitive%20Component%20Object%20Reference) (OtherActor :type Actor%20Object%20Reference) (OtherComp :type Primitive%20Component%20Object%20Reference) (OtherBodyIndex :type Integer))
  ;[0.1216 0.902 0.6627] Checks when the light orb leaves the death box
  (Utilities|Casting|CastToBP_LightOrb OtherActor)
  (Variables|Default|SetbIsLightInRange false))

(event EventBeginPlay)

(event EventTick
  (params (DeltaSeconds :type Float%20%28single-precision%29)))

(event Collision|EventActorBeginOverlap
  (params (OtherActor :type Actor%20Object%20Reference)))

(event EventInfluencingPlayer
  (params (PlayerRef :type BP%20Third%20Person%20Character%20Object%20Reference) (bIsInRange :type Boolean))
  (bind _playerdeathbox (Variables|Default|GetPlayerDeathBox))
  ;[1 1 1] Death Connection
  (if bIsInRange
    (Variables|/Script/Engine.PrimitiveComponent|SetbGenerateOverlapEvents _playerdeathbox true)
    (Development|PrintString "Player Is Influenced by PlayerDeathbox_WithoutLightInRange")
    (else
      (Variables|/Script/Engine.PrimitiveComponent|SetbGenerateOverlapEvents _playerdeathbox false))))

(event EventPlayerDeath
  (params (DyingPlayerReference :type BP%20Third%20Person%20Character%20Object%20Reference))
  ;[1 1 1] Death Connection
  (Default|LightAbandonment (Variables|Default|GetDeathManagerRef) DyingPlayerReference)
  (Development|PrintString "Player dying because of PlayerDeathbox_WithoutLightInRange"))

(fn ConstructionScript)

(fn IsInfluencingthePlayer
  (params (PlayerRef :type BP%20Third%20Person%20Character%20Object%20Reference))
  ;[1 1 1] WIP
  (return true))