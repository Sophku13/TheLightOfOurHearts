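; BP_Bunker runs the bunker button puzzle and controls the activation of the button that lets the player leave.
; On BeginPlay it sets every teamworker button in BunkerButtonGroup's list to active and links each back to that group.
; On Tick it polls the group's PuzzleCheck and sends OnActivationMessage to DoorButton on every frame the check passes, with no one-shot guard.
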(event EventBeginPlay
  (bind _bunkerbuttongroup (Variables|Default|GetBunkerButtonGroup))
  (bind _buttonlist (Variables|/Game/MechanicsPlayground/MechanincsBlueprints/Buttons/Bases/BP_ButtonGrouper_Base.BP_ButtonGrouper_Base_C|GetButtonList _bunkerbuttongroup))
  ;[0.1216 0.902 0.6627] Finding All Buttons in the bunker and set them automatically to active since it does not matter if they are active or not since the player need to "activate" the lights to get the solution of the puzzle
  (for _index (range 0 (- (Utilities|Map|Length _buttonlist) 1))
    (bind _asbp_button_teamworker_bunker (Utilities|Casting|CastToBP_Button_Teamworker_Bunker (.Value (Utilities|Map|Find _buttonlist _index))))
    (Variables|/Game/MechanicsPlayground/MechanincsBlueprints/Buttons/Bases/BP_Button_Teamworker_Base.BP_Button_Teamworker_Base_C|SetbIsActive _asbp_button_teamworker_bunker true)
    (Variables|/Game/MechanicsPlayground/MechanincsBlueprints/Buttons/Bunker/BP_Button_Teamworker_Bunker.BP_Button_Teamworker_Bunker_C|SetButtonGroup _asbp_button_teamworker_bunker (Variables|Default|GetBunkerButtonGroup))))

(event Collision|EventActorBeginOverlap
  (params (OtherActor :type Actor%20Object%20Reference)))

(event EventTick
  (params (DeltaSeconds :type Float%20%28single-precision%29))
  ;[0.1216 0.902 0.6627] Event Tick checks regularly if the buttons are pressed in the correct order and if they all are activated and correct it activated the door button to leave the bunker
  (bind _bpuzzlecomplete (Default|PuzzleCheck (Variables|Default|GetBunkerButtonGroup)))
  (if _bpuzzlecomplete
    (Class|BPILightFueledActivation|OnActivation(Message) (Variables|Default|GetDoorButton))))

(fn ConstructionScript)