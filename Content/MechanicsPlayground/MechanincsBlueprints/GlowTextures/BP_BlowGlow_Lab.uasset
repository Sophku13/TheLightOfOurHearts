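; Glow actor for the blow mechanic that shows a timed Niagara effect when a BP_BlowMechanic actor overlaps its Hitbox.
; BeginPlay assigns the system held in the Material variable to TextureGlow, if it is valid.
; The overlap shows the glow and enables Tick, which uses a 15-second Delay as a timer to hide it and disable Tick again.
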(event OnComponentBeginOverlap(Hitbox)
  (params (OverlappedComponent :type Primitive%20Component%20Object%20Reference) (OtherActor :type Actor%20Object%20Reference) (OtherComp :type Primitive%20Component%20Object%20Reference) (OtherBodyIndex :type Integer) (bFromSweep :type Boolean) (SweepResult :type Hit%20Result%20Structure%20%28by%20ref%29))
  (Utilities|Casting|CastToBP_BlowMechanic OtherActor)
  (Rendering|SetVisibility (Variables|Default|GetTextureGlow) true false)
  (Actor|Tick|SetActorTickEnabled true))

(event EventBeginPlay
  (bind _material (Variables|Default|GetMaterial)
    (:then
      (Class|NiagaraComponent|SetAsset (Variables|Default|GetTextureGlow) _material false))
    (:else)))

(event Collision|EventActorBeginOverlap
  (params (OtherActor :type Actor%20Object%20Reference)))

(event EventTick
  (params (DeltaSeconds :type Float%20%28single-precision%29))
  (Utilities|FlowControl|Delay 15.0)
  (Rendering|SetVisibility (Variables|Default|GetTextureGlow) false false)
  (Actor|Tick|SetActorTickEnabled false))

(fn ConstructionScript)