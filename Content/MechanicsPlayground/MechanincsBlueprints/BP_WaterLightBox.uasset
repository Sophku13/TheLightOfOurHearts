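; BP_WaterLightBox is a water volume that weakens the player's light orb.
; When the third-person character enters WaterBox, it stores the player and orb references and enables actor tick.
; Each tick, unless the orb's StatusHidden is set, it applies a -1 strength change via SetLightOrbStrength and refreshes the orb's conditions.
; Tick is disabled when the light orb itself, rather than the character, ends overlap with the box.
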(event OnComponentBeginOverlap(WaterBox)
  (params (OverlappedComponent :type Primitive%20Component%20Object%20Reference) (OtherActor :type Actor%20Object%20Reference) (OtherComp :type Primitive%20Component%20Object%20Reference) (OtherBodyIndex :type Integer) (bFromSweep :type Boolean) (SweepResult :type Hit%20Result%20Structure%20%28by%20ref%29))
  (bind _asbp_third_person_character (Utilities|Casting|CastToBP_ThirdPersonCharacter OtherActor))
  (bind _output_get (Variables|Default|SetPlayerRef _asbp_third_person_character))
  (Variables|Default|SetLightOrbRef (Variables|/Game/ThirdPerson/Blueprints/BP_ThirdPersonCharacter.BP_ThirdPersonCharacter_C|GetBP_LightOrbRef _output_get))
  (Actor|Tick|SetActorTickEnabled true))

(event OnComponentEndOverlap(WaterBox)
  (params (OverlappedComponent :type Primitive%20Component%20Object%20Reference) (OtherActor :type Actor%20Object%20Reference) (OtherComp :type Primitive%20Component%20Object%20Reference) (OtherBodyIndex :type Integer))
  (Utilities|Casting|CastToBP_LightOrb OtherActor)
  (Actor|Tick|SetActorTickEnabled false))

(event EventBeginPlay)

(event Collision|EventActorBeginOverlap
  (params (OtherActor :type Actor%20Object%20Reference)))

(event EventTick
  (params (DeltaSeconds :type Float%20%28single-precision%29))
  (Variables|Default|SetLightOrbRef (Variables|/Game/ThirdPerson/Blueprints/BP_ThirdPersonCharacter.BP_ThirdPersonCharacter_C|GetBP_LightOrbRef (Variables|Default|GetPlayerRef)))
  (if (not (Variables|/Game/MechanicsPlayground/MechanincsBlueprints/BP_LightOrb.BP_LightOrb_C|GetStatusHidden (Variables|Default|GetLightOrbRef)))
    (Default|SetLightOrbStrength (Variables|Default|GetLightOrbRef) -1.0)
    (Default|SetLightOrbConditions (Variables|Default|GetLightOrbRef))))

(fn ConstructionScript)