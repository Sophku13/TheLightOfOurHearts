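; Rotating platform that turns while a BP_RaiseMechanic actor overlaps its trigger box.
; BeginPlay caches the platform's starting world rotation as the interpolation origin.
; Overlap begin prints a debug string and plays the MoveUpDown timeline, which lerps the platform's world rotation toward NewRotation.
; Overlap end stops the timeline in place, so the platform holds its angle rather than rotating back.
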(event OnComponentBeginOverlap(Box)
  (params (OverlappedComponent :type Primitive%20Component%20Object%20Reference) (OtherActor :type Actor%20Object%20Reference) (OtherComp :type Primitive%20Component%20Object%20Reference) (OtherBodyIndex :type Integer) (bFromSweep :type Boolean) (SweepResult :type Hit%20Result%20Structure%20%28by%20ref%29))
  (Utilities|Casting|CastToBP_RaiseMechanic OtherActor)
  (Development|PrintString "IsOverlapping")
  (bind _movement (Timeline|MoveUpDown Play)
    (:Update
      (Transformation|SetWorldRotation (Variables|Default|GetPlatform) (Math|Rotator|Lerp(Rotator) (Variables|Default|GetInitialPosition) (Variables|Default|GetNewRotation) _movement) false false))))

(event OnComponentEndOverlap(Box)
  (params (OverlappedComponent :type Primitive%20Component%20Object%20Reference) (OtherActor :type Actor%20Object%20Reference) (OtherComp :type Primitive%20Component%20Object%20Reference) (OtherBodyIndex :type Integer))
  (Utilities|Casting|CastToBP_RaiseMechanic OtherActor)
  (bind _movement (Timeline|MoveUpDown Stop)
    (:Update
      (Transformation|SetWorldRotation (Variables|Default|GetPlatform) (Math|Rotator|Lerp(Rotator) (Variables|Default|GetInitialPosition) (Variables|Default|GetNewRotation) _movement) false false))))

(event EventBeginPlay
  (Variables|Default|SetInitialPosition (Transformation|GetWorldRotation (Variables|Default|GetPlatform)))
  (Variables|Default|SetNewRotation (Variables|Default|GetNewRotation)))

(fn ConstructionScript)