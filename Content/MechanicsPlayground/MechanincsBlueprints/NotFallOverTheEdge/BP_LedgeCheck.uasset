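; BP_LedgeCheck is a ledge trigger actor that briefly halts the player character when it detects the ledge's Cube underfoot.
; While the player overlaps the Box, a looping timer runs short downward line traces from the player.
; Hitting the Cube sets movement mode to None, then after a delay pauses the timer and restores Walking.
; Leaving the Box also pauses the timer.
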(event OnComponentBeginOverlap(Box)
  (params (OverlappedComponent :type Primitive%20Component%20Object%20Reference) (OtherActor :type Actor%20Object%20Reference) (OtherComp :type Primitive%20Component%20Object%20Reference) (OtherBodyIndex :type Integer) (bFromSweep :type Boolean) (SweepResult :type Hit%20Result%20Structure%20%28by%20ref%29))
  (if (== OtherActor (Variables|Default|GetPlayerRef))
    (Utilities|Time|SetTimerbyFunctionName 0 "CheckLedge" 0.05 true)))

(event OnComponentEndOverlap(Box)
  (params (OverlappedComponent :type Primitive%20Component%20Object%20Reference) (OtherActor :type Actor%20Object%20Reference) (OtherComp :type Primitive%20Component%20Object%20Reference) (OtherBodyIndex :type Integer))
  (if (== (Variables|Default|GetPlayerRef) OtherActor)
    (Class|KismetSystemLibrary|PauseTimer 0 "CheckLedge")))

(event Custom|CheckLedge
  (bind _returnvalue (Game|GetPlayerCharacter 0))
  (bind _playerref (Variables|Default|GetPlayerRef))
  (bind _returnvalue_2 (Transformation|GetActorLocation _playerref))
  (bind _charactermovement (Variables|/Script/Engine.Character|GetCharacterMovement _returnvalue))
  (bind _outhit (Collision|LineTraceByChannel _returnvalue_2 (+ _returnvalue_2 (Math|Vector|MakeVector 0.0 0.0 -1.5e+02)) "TraceTypeQuery1" false (Utilities|Array|MakeArray _playerref) "None" false))
  (if (== (.HitComponent (Collision|BreakHitResult _outhit)) (Variables|Default|GetCube))
    (Pawn|Components|CharacterMovement|SetMovementMode _charactermovement "MOVE_None" 0)
    (Utilities|FlowControl|Delay 0.5)
    (Class|KismetSystemLibrary|PauseTimer 0 "CheckLedge")
    (Pawn|Components|CharacterMovement|SetMovementMode _charactermovement "MOVE_Walking" 0)))

(event EventBeginPlay
  (Variables|Default|SetPlayerRef (Game|GetPlayerCharacter 0)))

(event Collision|EventActorBeginOverlap
  (params (OtherActor :type Actor%20Object%20Reference)))

(event EventTick
  (params (DeltaSeconds :type Float%20%28single-precision%29)))

(fn ConstructionScript)