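; Lab button that toggles the light orb in the lab's socket mover between raised and standard strength.
; Interaction moves the button and runs a task that reaches the orb through the button grouper and, unless it is held, flip-flops its strength, attaching or destroying a raise-mechanic actor.
; Delays and flags block repeat presses.
; BeginPlay spawns a glow sign, and Tick swaps the button material by active state.
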(event EventBeginPlay
  ;[0.1216 0.902 0.6627] Begin Play - Spawn a new Glow Sprites and sets the material
  (|CallParentFunction)
  (bind _returnvalue (Game|SpawnActorfromClass "/Game/MechanicsPlayground/MechanincsBlueprints/GlowTextures/BP_TEMPLATE_BlowGlow_Base.BP_TEMPLATE_BlowGlow_Base_C" (Math|Transform|MakeTransform (+ (.location (Transformation|GetWorldTransform (Variables|Default|GetSignBase))) "0.000000,25.000000,0.000000") "0, 0, 0" "0.500000,0.500000,0.500000") "AlwaysSpawn" "MultiplyWithRoot" 0 0))
  (Variables|Default|SetSignGlow _returnvalue)
  (bind _signglow (Variables|Default|GetSignGlow)
    (:then
      (Class|NiagaraComponent|SetAsset (Variables|/Game/MechanicsPlayground/MechanincsBlueprints/GlowTextures/BP_TEMPLATE_BlowGlow_Base.BP_TEMPLATE_BlowGlow_Base_C|GetTextureGlow _signglow) "/Game/MechanicsPlayground/MechanincsBlueprints/GlowTextures/NiagaraSystems/NS_BlowRevealParticles_Lab.NS_BlowRevealParticles_Lab" false)
      (Rendering|Material|SetMaterial (Variables|Default|GetSignBase) 0 "/Game/MechanicsPlayground/MechanincsBlueprints/GlowTextures/Material/M_GlowMechanic_Lab.M_GlowMechanic_Lab"))
    (:else)))

(event EventTick
  (params (DeltaSeconds :type Float%20%28single-precision%29))
  ;[0.1216 0.902 0.6627] Event Tick sets material depending on active status
  (if (Variables|Default|GetbIsActive)
    (Rendering|Material|SetMaterial (Variables|Default|GetButton) 0 "/Game/Materials/MI_Sphere_Emissive_Red.MI_Sphere_Emissive_Red")
    (else
      (Rendering|Material|SetMaterial (Variables|Default|GetButton) 0 "/Game/Materials/MI_Sphere_Emissive_Red_Off.MI_Sphere_Emissive_Red_Off"))))

(event EventButtonTask
  (params (ButtonGroup :type BP%20Button%20Grouper%20Base%20Object%20Reference))
  ;[0.1216 0.902 0.6627] Button Task Sets the Light Orb strength to high or standard
  (bind _asbp_button_grouper_lab (Utilities|Casting|CastToBP_ButtonGrouper_Lab ButtonGroup))
  (if (not (Variables|Default|GetbIsTasking))
    (Variables|Default|SetbIsTasking true)
    (if (not (Variables|/Game/MechanicsPlayground/MechanincsBlueprints/BP_LightOrb.BP_LightOrb_C|GetbIsHeld (Variables|/Game/MechanicsPlayground/MechanincsBlueprints/BP_MoveBetweenSocketsWithButtons_Lab.BP_MoveBetweenSocketsWithButtons_Lab_C|GetLightOrbRef (Variables|/Game/MechanicsPlayground/MechanincsBlueprints/Buttons/Lab/BP_Lab.BP_Lab_C|GetSocketMover (Variables|/Game/MechanicsPlayground/MechanincsBlueprints/Buttons/Lab/BP_ButtonGrouper_Lab.BP_ButtonGrouper_Lab_C|GetLabRef _asbp_button_grouper_lab)))))
      (Utilities|FlowControl|FlipFlop
        (:A
          ;;[0.1216 0.902 0.6627] Sets Light Status to High- Raised
          (Variables|/Game/MechanicsPlayground/MechanincsBlueprints/BP_LightOrb.BP_LightOrb_C|SetbIsIncreasing (Variables|/Game/MechanicsPlayground/MechanincsBlueprints/BP_MoveBetweenSocketsWithButtons_Lab.BP_MoveBetweenSocketsWithButtons_Lab_C|GetLightOrbRef (Variables|/Game/MechanicsPlayground/MechanincsBlueprints/Buttons/Lab/BP_Lab.BP_Lab_C|GetSocketMover (Variables|/Game/MechanicsPlayground/MechanincsBlueprints/Buttons/Lab/BP_ButtonGrouper_Lab.BP_ButtonGrouper_Lab_C|GetLabRef _asbp_button_grouper_lab))) true)
          (Default|SetLightOrbStrength (Variables|/Game/MechanicsPlayground/MechanincsBlueprints/BP_MoveBetweenSocketsWithButtons_Lab.BP_MoveBetweenSocketsWithButtons_Lab_C|GetLightOrbRef (Variables|/Game/MechanicsPlayground/MechanincsBlueprints/Buttons/Lab/BP_Lab.BP_Lab_C|GetSocketMover (Variables|/Game/MechanicsPlayground/MechanincsBlueprints/Buttons/Lab/BP_ButtonGrouper_Lab.BP_ButtonGrouper_Lab_C|GetLabRef _asbp_button_grouper_lab))) 3.0)
          (Default|SetLightOrbConditions (Variables|/Game/MechanicsPlayground/MechanincsBlueprints/BP_MoveBetweenSocketsWithButtons_Lab.BP_MoveBetweenSocketsWithButtons_Lab_C|GetLightOrbRef (Variables|/Game/MechanicsPlayground/MechanincsBlueprints/Buttons/Lab/BP_Lab.BP_Lab_C|GetSocketMover (Variables|/Game/MechanicsPlayground/MechanincsBlueprints/Buttons/Lab/BP_ButtonGrouper_Lab.BP_ButtonGrouper_Lab_C|GetLabRef _asbp_button_grouper_lab))))
          ;;[0.1216 0.902 0.6627] Spawning a raise mechanic instance and attach it to the light orb and if pressed again it gets deleted again
          (bind _returnvalue (Game|SpawnActorfromClass "/Game/MechanicsPlayground/MechanincsBlueprints/BP_RaiseMechanic.BP_RaiseMechanic_C" (Transformation|GetWorldTransform (Variables|/Game/MechanicsPlayground/MechanincsBlueprints/BP_LightOrb.BP_LightOrb_C|GetM_LightOrb (Variables|/Game/MechanicsPlayground/MechanincsBlueprints/BP_MoveBetweenSocketsWithButtons_Lab.BP_MoveBetweenSocketsWithButtons_Lab_C|GetLightOrbRef (Variables|/Game/MechanicsPlayground/MechanincsBlueprints/Buttons/Lab/BP_Lab.BP_Lab_C|GetSocketMover (Variables|/Game/MechanicsPlayground/MechanincsBlueprints/Buttons/Lab/BP_ButtonGrouper_Lab.BP_ButtonGrouper_Lab_C|GetLabRef _asbp_button_grouper_lab))))) "Undefined" "MultiplyWithRoot" 0 0))
          (Transformation|AttachComponentToComponent _returnvalue (Variables|/Game/MechanicsPlayground/MechanincsBlueprints/BP_LightOrb.BP_LightOrb_C|GetM_LightOrb (Variables|/Game/MechanicsPlayground/MechanincsBlueprints/BP_MoveBetweenSocketsWithButtons_Lab.BP_MoveBetweenSocketsWithButtons_Lab_C|GetLightOrbRef (Variables|/Game/MechanicsPlayground/MechanincsBlueprints/Buttons/Lab/BP_Lab.BP_Lab_C|GetSocketMover (Variables|/Game/MechanicsPlayground/MechanincsBlueprints/Buttons/Lab/BP_ButtonGrouper_Lab.BP_ButtonGrouper_Lab_C|GetLabRef _asbp_button_grouper_lab)))) "None" "SnapToTarget" "SnapToTarget" "KeepRelative" true))
        (:B
          ;;[0.1216 0.902 0.6627] Sets Light status to standard
          (Variables|/Game/MechanicsPlayground/MechanincsBlueprints/BP_LightOrb.BP_LightOrb_C|SetbIsIncreasing (Variables|/Game/MechanicsPlayground/MechanincsBlueprints/BP_MoveBetweenSocketsWithButtons_Lab.BP_MoveBetweenSocketsWithButtons_Lab_C|GetLightOrbRef (Variables|/Game/MechanicsPlayground/MechanincsBlueprints/Buttons/Lab/BP_Lab.BP_Lab_C|GetSocketMover (Variables|/Game/MechanicsPlayground/MechanincsBlueprints/Buttons/Lab/BP_ButtonGrouper_Lab.BP_ButtonGrouper_Lab_C|GetLabRef _asbp_button_grouper_lab))) false)
          (Default|SetLightOrbStrength (Variables|/Game/MechanicsPlayground/MechanincsBlueprints/BP_MoveBetweenSocketsWithButtons_Lab.BP_MoveBetweenSocketsWithButtons_Lab_C|GetLightOrbRef (Variables|/Game/MechanicsPlayground/MechanincsBlueprints/Buttons/Lab/BP_Lab.BP_Lab_C|GetSocketMover (Variables|/Game/MechanicsPlayground/MechanincsBlueprints/Buttons/Lab/BP_ButtonGrouper_Lab.BP_ButtonGrouper_Lab_C|GetLabRef _asbp_button_grouper_lab))) 2.0)
          (Default|SetLightOrbConditions (Variables|/Game/MechanicsPlayground/MechanincsBlueprints/BP_MoveBetweenSocketsWithButtons_Lab.BP_MoveBetweenSocketsWithButtons_Lab_C|GetLightOrbRef (Variables|/Game/MechanicsPlayground/MechanincsBlueprints/Buttons/Lab/BP_Lab.BP_Lab_C|GetSocketMover (Variables|/Game/MechanicsPlayground/MechanincsBlueprints/Buttons/Lab/BP_ButtonGrouper_Lab.BP_ButtonGrouper_Lab_C|GetLabRef _asbp_button_grouper_lab))))
          (Utilities|IsValid _returnvalue
            (:Is%20Valid
              (Actor|DestroyActor _returnvalue))
            (:Is%20Not%20Valid
              _))))
      (Utilities|FlowControl|Delay 1.0)
      (Variables|Default|SetbIsTasking false)
      (else
        (Variables|Default|SetbIsTasking false)))))

(event EventOnInteract
  ;[0.1216 0.902 0.6627] On Interact move button and call the button task
  (Variables|Default|SetbIsButtonPressed true)
  (CallFunction|MoveButton)
  (CallFunction|ButtonTask (Variables|Default|GetButtonGroup))
  (Utilities|FlowControl|Delay 2.0)
  (CallFunction|MoveButton)
  (Variables|Default|SetbIsButtonPressed false))

(fn ConstructionScript
  (|CallParentFunction))

(fn IsInteractable
  (return (and (not (Variables|Default|GetbIsButtonPressed)) (Variables|Default|GetbIsActive))))