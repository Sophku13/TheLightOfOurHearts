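; Actor that carries a light orb from a start socket to an end socket in equal steps.
; Tick starts the move when only the start socket is lit, then a timeline lerps the orb one interval at a time, with a delay before each step.
; On arrival, ExchangeValues hands the orb, timer and player reference to the end socket, and the start socket is unlit and stops ticking.
; A DoOnce re-initializes the path while the start socket is unlit.
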(event EventBeginPlay)

(event Collision|EventActorBeginOverlap
  (params (OtherActor :type Actor%20Object%20Reference)))

(event EventTick
  (params (DeltaSeconds :type Float%20%28single-precision%29))
  (bind _startsocket (Variables|Default|GetStartSocket))
  (if (Variables|/Game/MechanicsPlayground/MechanincsBlueprints/BP_PlaceLightSocket.BP_PlaceLightSocket_C|GetbLightOnSocket (Variables|Default|GetStartSocket))
    (if (not (Variables|/Game/MechanicsPlayground/MechanincsBlueprints/BP_PlaceLightSocket.BP_PlaceLightSocket_C|GetbLightOnSocket (Variables|Default|GetEndSocket)))
      (Variables|Default|SetLightOrbRef (Variables|/Game/MechanicsPlayground/MechanincsBlueprints/BP_PlaceLightSocket.BP_PlaceLightSocket_C|GetLightOrbRef (Variables|Default|GetStartSocket)))
      (if (<= (Variables|Default|GetstepsCompleted) (- (Variables|Default|Getsteps) 1)) :!label _label
        (if (not (Variables|Default|GetbIsMoving))
          (Variables|Default|SetbIsMoving true)
          (Utilities|FlowControl|Delay 2.0)
          (bind _newtrack_0 (Timeline|MoveLightFromStartToEnd PlayFromStart)
            (:Update
              (Transformation|SetActorLocation (Variables|Default|GetLightOrbRef) (Math|Vector|Lerp(Vector) (Variables|Default|GetCurrentLocation) (+ (Variables|Default|GetCurrentLocation) (Variables|Default|GetIntervalPath)) _newtrack_0) false false))
            (:Finished
              (Variables|Default|SetCurrentLocation (+ (Variables|Default|GetCurrentLocation) (Variables|Default|GetIntervalPath)))
              (Variables|Default|SetbIsMoving false)
              (Variables|Default|SetstepsCompleted (+ (Variables|Default|GetstepsCompleted) 1))
              (Utilities|FlowControl|DoOnce false ; enters at Reset
                (:Completed
                  (goto _label))))))
        (elif (Utilities|Operators|EqualEqual (Variables|/Game/MechanicsPlayground/MechanincsBlueprints/BP_PlaceLightSocket.BP_PlaceLightSocket_C|GetLocationOfSocket (Variables|Default|GetEndSocket)) (Variables|Default|GetCurrentLocation) 1.0)
          (CallFunction|ExchangeValues (Variables|Default|GetEndSocket) (Variables|Default|GetStartSocket))
          (Variables|/Game/MechanicsPlayground/MechanincsBlueprints/BP_PlaceLightSocket.BP_PlaceLightSocket_C|SetbLightOnSocket _startsocket false)
          (Actor|Tick|SetActorTickEnabled _startsocket)
          (goto _label_2 Reset))))
    (else
      (Utilities|FlowControl|DoOnce false :!label _label_2
        (:Completed
          (Variables|Default|SetIntervalPath (/ (- (Variables|/Game/MechanicsPlayground/MechanincsBlueprints/BP_PlaceLightSocket.BP_PlaceLightSocket_C|GetLocationOfSocket (Variables|Default|GetEndSocket)) (Variables|/Game/MechanicsPlayground/MechanincsBlueprints/BP_PlaceLightSocket.BP_PlaceLightSocket_C|GetLocationOfSocket (Variables|Default|GetStartSocket))) (Variables|Default|Getsteps)))
          (Variables|Default|SetCurrentLocation (Variables|/Game/MechanicsPlayground/MechanincsBlueprints/BP_PlaceLightSocket.BP_PlaceLightSocket_C|GetLocationOfSocket (Variables|Default|GetStartSocket)))
          (Variables|Default|SetstepsCompleted 0))))))

(fn ConstructionScript)

(fn ExchangeValues
  (params (EndSocket :type BP%20Place%20Light%20Socket%20Object%20Reference) (StartSocket :type BP%20Place%20Light%20Socket%20Object%20Reference))
  (Variables|/Game/MechanicsPlayground/MechanincsBlueprints/BP_PlaceLightSocket.BP_PlaceLightSocket_C|SetTimeOfLightInSocket EndSocket (Variables|/Game/MechanicsPlayground/MechanincsBlueprints/BP_PlaceLightSocket.BP_PlaceLightSocket_C|GetTimeOfLightInSocket StartSocket))
  (Variables|/Game/MechanicsPlayground/MechanincsBlueprints/BP_PlaceLightSocket.BP_PlaceLightSocket_C|SetPlayerRef EndSocket (Variables|/Game/MechanicsPlayground/MechanincsBlueprints/BP_PlaceLightSocket.BP_PlaceLightSocket_C|GetPlayerRef StartSocket))
  (Variables|/Game/MechanicsPlayground/MechanincsBlueprints/BP_PlaceLightSocket.BP_PlaceLightSocket_C|SetLightOrbRef EndSocket (Variables|/Game/MechanicsPlayground/MechanincsBlueprints/BP_PlaceLightSocket.BP_PlaceLightSocket_C|GetLightOrbRef StartSocket))
  (Variables|/Game/MechanicsPlayground/MechanincsBlueprints/BP_PlaceLightSocket.BP_PlaceLightSocket_C|SetbLightOnSocket EndSocket true)
  (Variables|/Game/ThirdPerson/Blueprints/BP_ThirdPersonCharacter.BP_ThirdPersonCharacter_C|SetNearestLightSocketRef (Variables|/Game/MechanicsPlayground/MechanincsBlueprints/BP_PlaceLightSocket.BP_PlaceLightSocket_C|GetPlayerRef EndSocket) EndSocket))