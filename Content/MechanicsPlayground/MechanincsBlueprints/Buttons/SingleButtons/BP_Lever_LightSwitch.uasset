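; Interactable lever switch that activates a list of connected actors and only reports as interactable while active.
; Receiving OnActivation toggles its active state; Tick paints it rusty when inactive, or red when active and not yet moved.
; Interacting flips the lever's rotation and red/green material with a sound and debug print, then sends an OnActivation message to every actor in its Actors array.
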(event Custom|MoveLever
  (bind _buttonbase1 (Variables|Default|GetButtonBase1))
  (bind _button (Variables|Default|GetButton))
  (bind _relativelocation (Variables|/Script/Engine.SceneComponent|GetRelativeLocation _buttonbase1))
  ;[1 1 1] Comment
  (Utilities|FlowControl|FlipFlop
    (:A
      (Development|PrintString "Off")
      (Rendering|Material|SetMaterial _button 0 "/Game/Materials/MI_Sphere_Emissive_Red.MI_Sphere_Emissive_Red")
      (Transformation|SetRelativeRotation _buttonbase1 (Math|Rotator|MakeRotator 0.0 0.0 0.0) false false)
      ;[0 1 0.07555] Herkus Was here
      (Audio|PlaySoundatLocation "/Game/Audio/Cues/lever6_by_mediatheksuche_Cue.lever6_by_mediatheksuche_Cue" _relativelocation "0, 0, 0" 1.0 1.0 0.0 0 0 0 0))
    (:B
      (Development|PrintString "On")
      (Rendering|Material|SetMaterial _button 0 "/Game/Materials/MI_Sphere_Emissive_Green.MI_Sphere_Emissive_Green")
      (Transformation|SetRelativeRotation _buttonbase1 (Math|Rotator|MakeRotator 0.0 1.8e+02 0.0) false false)
      (Audio|PlaySoundatLocation "/Game/Audio/Cues/lever6_by_mediatheksuche_Cue.lever6_by_mediatheksuche_Cue" _relativelocation "0, 0, 0" 1.0 1.0 0.0 0 0 0 0))))

(event EventBeginPlay
  (|CallParentFunction) ; This node is disabled and will not be called.\nDrag off pins to build functionality.
)

(event EventMoveButton
  (bind _buttonbase1 (Variables|Default|GetButtonBase1))
  (bind _button (Variables|Default|GetButton))
  (bind _relativelocation (Variables|/Script/Engine.SceneComponent|GetRelativeLocation _buttonbase1))
  ;[1 1 1] Comment
  (Utilities|FlowControl|FlipFlop
    (:A
      (Development|PrintString "Off")
      (Rendering|Material|SetMaterial _button 0 "/Game/Materials/MI_Sphere_Emissive_Red.MI_Sphere_Emissive_Red")
      (Transformation|SetRelativeRotation _buttonbase1 (Math|Rotator|MakeRotator 0.0 0.0 0.0) false false)
      ;[0 1 0.07555] Herkus Was here
      (Audio|PlaySoundatLocation "/Game/Audio/Cues/lever6_by_mediatheksuche_Cue.lever6_by_mediatheksuche_Cue" _relativelocation "0, 0, 0" 1.0 1.0 0.0 0 0 0 0))
    (:B
      (Development|PrintString "On")
      (Rendering|Material|SetMaterial _button 0 "/Game/Materials/MI_Sphere_Emissive_Green.MI_Sphere_Emissive_Green")
      (Transformation|SetRelativeRotation _buttonbase1 (Math|Rotator|MakeRotator 0.0 1.8e+02 0.0) false false)
      (Audio|PlaySoundatLocation "/Game/Audio/Cues/lever6_by_mediatheksuche_Cue.lever6_by_mediatheksuche_Cue" _relativelocation "0, 0, 0" 1.0 1.0 0.0 0 0 0 0))))

(event EventTick
  (params (DeltaSeconds :type Float%20%28single-precision%29))
  ;[0.1216 0.902 0.6627] Event Tick sets the material of the button depending on the active status of the button
  (if (Variables|Default|GetbIsActive)
    (if (not (Variables|Default|GetbIsMoved))
      (Rendering|Material|SetMaterial (Variables|Default|GetButton) 0 "/Game/Materials/MI_Sphere_Emissive_Red.MI_Sphere_Emissive_Red"))
    (else
      (Rendering|Material|SetMaterial (Variables|Default|GetButton) 0 "/Game/LevelBlockout/AssetsVlad/Materials/Rust_handpaint/M_RustHandPaint_Inst.M_RustHandPaint_Inst"))))

(event EventOnInteract
  ;[0.1216 0.902 0.6627] On interact call the activation function for every actor connected to the button
  (CallFunction|MoveLever)
  (Variables|Default|SetbIsMoved true)
  (for _array_element (Variables|Default|GetActors)
    (Class|BPILightFueledActivation|OnActivation(Message) _array_element)))

(event EventOnActivation
  ;[0.1216 0.902 0.6627] On activation flips the button active status
  (Utilities|FlowControl|FlipFlop
    (:A
      (Variables|Default|SetbIsActive true))
    (:B
      (Variables|Default|SetbIsActive false))))

(fn ConstructionScript
  (|CallParentFunction))

(fn IsInteractable
  (return (Variables|Default|GetbIsActive)))