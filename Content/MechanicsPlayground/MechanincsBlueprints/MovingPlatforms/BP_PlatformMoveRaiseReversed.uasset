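; Moving platform that travels to a target location while a BP_RaiseMechanic actor overlaps its trigger box, and returns after it leaves.
; A Timeline, rate-scaled by TimeLineLength, lerps the platform's relative location from its starting point to NewLocation, reversing one second after overlap ends.
; IsPlatformMoving tracks motion, and InfluenceLightOrb makes the given light orb pulse.
; The MetaSound concrete-scrape logic is disconnected and never runs.
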(event OnComponentBeginOverlap(Box)
  (params (OverlappedComponent :type Primitive%20Component%20Object%20Reference) (OtherActor :type Actor%20Object%20Reference) (OtherComp :type Primitive%20Component%20Object%20Reference) (OtherBodyIndex :type Integer) (bFromSweep :type Boolean) (SweepResult :type Hit%20Result%20Structure%20%28by%20ref%29))
  (bind _timeline (Variables|Default|GetTimeline))
  (Utilities|Casting|CastToBP_RaiseMechanic OtherActor)
  (Development|PrintString "IsOverlapping")
  (Components|Timeline|SetPlayRate _timeline (/ (Components|Timeline|GetTimelineLength _timeline) (Variables|Default|GetTimeLineLength)))
  (Variables|Default|SetbIsPlatformMoving true)
  (bind _movement (Timeline|Timeline Play)
    (:Update
      (Transformation|SetRelativeLocation (Variables|Default|GetPlatform) (Math|Vector|Lerp(Vector) (Variables|Default|GetInitialLocation) (Variables|Default|GetNewLocation) _movement) false false)
      (if (== _movement 0.0)
        (Variables|Default|SetbIsPlatformMoving false)))
    (:Finished
      (Variables|Default|SetbIsPlatformMoving false))))

(event OnComponentEndOverlap(Box)
  (params (OverlappedComponent :type Primitive%20Component%20Object%20Reference) (OtherActor :type Actor%20Object%20Reference) (OtherComp :type Primitive%20Component%20Object%20Reference) (OtherBodyIndex :type Integer))
  (Utilities|Casting|CastToBP_RaiseMechanic OtherActor)
  (Utilities|FlowControl|Delay 1.0)
  (Variables|Default|SetbIsPlatformMoving true)
  (bind _movement (Timeline|Timeline Reverse)
    (:Update
      (Transformation|SetRelativeLocation (Variables|Default|GetPlatform) (Math|Vector|Lerp(Vector) (Variables|Default|GetInitialLocation) (Variables|Default|GetNewLocation) _movement) false false)
      (if (== _movement 0.0)
        (Variables|Default|SetbIsPlatformMoving false)))
    (:Finished
      (Variables|Default|SetbIsPlatformMoving false))))

(event EventBeginPlay
  (Variables|Default|SetInitialLocation (Variables|/Script/Engine.SceneComponent|GetRelativeLocation (Variables|Default|GetPlatform)))
  (Variables|Default|SetNewLocation (Variables|Default|GetNewLocation)))

(event EventInfluenceLightOrb
  (params (LightOrbRef :type BP%20Light%20Orb%20Object%20Reference) (IsActive :type Boolean))
  ;[1 1 1] Comment
  (Default|LightPulsing LightOrbRef))

(fn ConstructionScript)