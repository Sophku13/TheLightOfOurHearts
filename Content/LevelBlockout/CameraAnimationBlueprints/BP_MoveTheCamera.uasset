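; BP_MoveTheCamera is a one-shot trigger that briefly shows the player another camera view.
; On overlap, it freezes character movement, waits briefly if a transition is running, then blends the view to CameraToFind over DurationOfLook.
; After a hold, it blends back to the saved active camera, or calls the character's default-camera message if that is invalid.
; It then destroys itself and restores walking.
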(event OnComponentBeginOverlap(TrigerCameraMovement)
  (params (OverlappedComponent :type Primitive%20Component%20Object%20Reference) (OtherActor :type Actor%20Object%20Reference) (OtherComp :type Primitive%20Component%20Object%20Reference) (OtherBodyIndex :type Integer) (bFromSweep :type Boolean) (SweepResult :type Hit%20Result%20Structure%20%28by%20ref%29))
  (bind _durationoflook (Variables|Default|GetDurationOfLook))
  (bind _asbp_third_person_character (Utilities|Casting|CastToBP_ThirdPersonCharacter OtherActor))
  (bind _output_get (Variables|Default|SetAs%20BP%20Third%20Person%20Character _asbp_third_person_character))
  (Variables|Default|SetCameraToReturnTo (Variables|/Game/ThirdPerson/Blueprints/BP_ThirdPersonCharacter.BP_ThirdPersonCharacter_C|GetActive%20Camera _output_get))
  (Pawn|Components|CharacterMovement|SetMovementMode (Variables|/Script/Engine.Character|GetCharacterMovement _output_get) "MOVE_None" 0)
  (if (Variables|/Game/LevelBlockout/CameraAnimationBlueprints/BP_CameraComponentIn.BP_CameraComponentIn_C|GetInProcessOfTransition (Variables|/Game/ThirdPerson/Blueprints/BP_ThirdPersonCharacter.BP_ThirdPersonCharacter_C|GetActive%20Camera _output_get))
    (Utilities|FlowControl|Delay 3.0))
  (Variables|/Game/LevelBlockout/CameraAnimationBlueprints/BP_CameraComponentIn.BP_CameraComponentIn_C|SetInProcessOfTransition (Variables|/Game/ThirdPerson/Blueprints/BP_ThirdPersonCharacter.BP_ThirdPersonCharacter_C|GetActive%20Camera _output_get) true)
  (Game|Player|SetViewTargetwithBlend (Game|GetPlayerController 0) (Variables|Default|GetCameraToFind) _durationoflook "VTBlend_Cubic" 1e+01 false)
  (Utilities|FlowControl|Delay (+ _durationoflook 2.0))
  (bind _cameratoreturnto (Variables|Default|GetCameraToReturnTo)
    (:then
      (Game|Player|SetViewTargetwithBlend (Game|GetPlayerController 0) _cameratoreturnto 2.0 "VTBlend_Cubic" 1e+01 false)
      (Variables|/Game/LevelBlockout/CameraAnimationBlueprints/BP_CameraComponentIn.BP_CameraComponentIn_C|SetInProcessOfTransition (Variables|/Game/ThirdPerson/Blueprints/BP_ThirdPersonCharacter.BP_ThirdPersonCharacter_C|GetActive%20Camera _output_get) false))
    (:else
      (Class|BPIPlayer|EnableDefaultCharacterCamera(Message) _output_get)))
  (Actor|DestroyActor)
  (Pawn|Components|CharacterMovement|SetMovementMode (Variables|/Script/Engine.Character|GetCharacterMovement _output_get) "MOVE_Walking" 0))

(event EventBeginPlay
  (Variables|Default|SetDurationOfLook (Variables|Default|GetDurationOfLook)))

(fn ConstructionScript)