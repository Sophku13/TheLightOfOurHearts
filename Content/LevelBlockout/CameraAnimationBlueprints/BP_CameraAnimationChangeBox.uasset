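; Trigger volume that changes the third-person character's camera framing while the player stands inside it.
; On begin overlap it caches the Follow Camera and Camera Boom relative transforms and arm length, then applies the configured new values instantly.
; Zero-valued overrides fall back to the cached originals, so only the fields that are set change.
; On end overlap it restores the cached values.
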(event OnComponentBeginOverlap(CameraHitbox)
  (params (OverlappedComponent :type Primitive%20Component%20Object%20Reference) (OtherActor :type Actor%20Object%20Reference) (OtherComp :type Primitive%20Component%20Object%20Reference) (OtherBodyIndex :type Integer) (bFromSweep :type Boolean) (SweepResult :type Hit%20Result%20Structure%20%28by%20ref%29))
  ;[1 1 1] Saving the default values
  (bind _asbp_third_person_character (Utilities|Casting|CastToBP_ThirdPersonCharacter OtherActor))
  (Variables|Default|SetPlayerRef _asbp_third_person_character)
  (Variables|Default|SetOldFollowCameraLocation (Variables|/Script/Engine.SceneComponent|GetRelativeLocation (Variables|/Game/ThirdPerson/Blueprints/BP_ThirdPersonCharacter.BP_ThirdPersonCharacter_C|GetFollowCamera (Variables|Default|GetPlayerRef))))
  (Variables|Default|SetOldFollowCameraRotation (Variables|/Script/Engine.SceneComponent|GetRelativeRotation (Variables|/Game/ThirdPerson/Blueprints/BP_ThirdPersonCharacter.BP_ThirdPersonCharacter_C|GetFollowCamera (Variables|Default|GetPlayerRef))))
  (Variables|Default|SetOldCameraBoomLocation (Variables|/Script/Engine.SceneComponent|GetRelativeLocation (Variables|/Game/ThirdPerson/Blueprints/BP_ThirdPersonCharacter.BP_ThirdPersonCharacter_C|GetCameraBoom (Variables|Default|GetPlayerRef))))
  (Variables|Default|SetOldCamerBoomRotation (Variables|/Script/Engine.SceneComponent|GetRelativeRotation (Variables|/Game/ThirdPerson/Blueprints/BP_ThirdPersonCharacter.BP_ThirdPersonCharacter_C|GetCameraBoom (Variables|Default|GetPlayerRef))))
  (Variables|Default|SetOldCameraBoomArmLength (Variables|/Script/Engine.SpringArmComponent|GetTargetArmLength (Variables|/Game/ThirdPerson/Blueprints/BP_ThirdPersonCharacter.BP_ThirdPersonCharacter_C|GetCameraBoom (Variables|Default|GetPlayerRef))))
  (CallFunction|SetNewValuesforCamera))

(event OnComponentEndOverlap(CameraHitbox)
  (params (OverlappedComponent :type Primitive%20Component%20Object%20Reference) (OtherActor :type Actor%20Object%20Reference) (OtherComp :type Primitive%20Component%20Object%20Reference) (OtherBodyIndex :type Integer))
  (bind _asbp_third_person_character (Utilities|Casting|CastToBP_ThirdPersonCharacter OtherActor))
  (Variables|Default|SetPlayerRef _asbp_third_person_character)
  (CallFunction|ResetBacktoDefaultValuesforCamera))

(event Custom|ResetBackToDefaultValuesForCamera
  ;[1 1 1] Resetting to old Values for the Camera
  ;;[1 1 1] Resetting to old Follow Camera Location and Rotation
  (Transformation|SetRelativeLocationAndRotation (Variables|/Game/ThirdPerson/Blueprints/BP_ThirdPersonCharacter.BP_ThirdPersonCharacter_C|GetFollowCamera (Variables|Default|GetPlayerRef)) (Variables|Default|GetOldFollowCameraLocation) (Variables|Default|GetOldFollowCameraRotation) false false)
  ;;[1 1 1] Resetting to old Camera Boom Location and Rotation
  (Transformation|SetRelativeLocationAndRotation (Variables|/Game/ThirdPerson/Blueprints/BP_ThirdPersonCharacter.BP_ThirdPersonCharacter_C|GetCameraBoom (Variables|Default|GetPlayerRef)) (Variables|Default|GetOldCameraBoomLocation) (Variables|Default|GetOldCamerBoomRotation) false false)
  ;;[1 1 1] Resetting to old Arm Length
  (Variables|/Script/Engine.SpringArmComponent|SetTargetArmLength (Variables|/Game/ThirdPerson/Blueprints/BP_ThirdPersonCharacter.BP_ThirdPersonCharacter_C|GetCameraBoom (Variables|Default|GetPlayerRef)) (Variables|Default|GetOldCameraBoomArmLength)))

(event Custom|SetNewValuesForCamera
  ;[1 1 1] Setting the Values for the Camera
  (CallFunction|CheckFollowCamera)
  ;;[1 1 1] Setting the new Follow Camera Location and Rotation
  (Transformation|SetRelativeLocationAndRotation (Variables|/Game/ThirdPerson/Blueprints/BP_ThirdPersonCharacter.BP_ThirdPersonCharacter_C|GetFollowCamera (Variables|Default|GetPlayerRef)) (Variables|Default|GetNewFollowCameraLocation) (Variables|Default|GetNewFollowCameraRotation) false false)
  (CallFunction|CheckCameraBoom)
  ;;[1 1 1] Setting the new Camera Boom Location and Rotation
  (Transformation|SetRelativeLocationAndRotation (Variables|/Game/ThirdPerson/Blueprints/BP_ThirdPersonCharacter.BP_ThirdPersonCharacter_C|GetCameraBoom (Variables|Default|GetPlayerRef)) (Variables|Default|GetNewCameraBoomLocation) (Variables|Default|GetNewCameraBoomRotation) false false)
  ;;[1 1 1] Setting the new Arm Length
  (Variables|/Script/Engine.SpringArmComponent|SetTargetArmLength (Variables|/Game/ThirdPerson/Blueprints/BP_ThirdPersonCharacter.BP_ThirdPersonCharacter_C|GetCameraBoom (Variables|Default|GetPlayerRef)) (Variables|Default|GetNewCameraBoomArmLength)))

(event Custom|CheckFollowCamera
  ;[1 1 1] Checking the Values of the Follow Camera that they are not empty
  (if (Utilities|Operators|NotEqual(!=) :A (Variables|Default|GetNewFollowCameraRotation))
    _
    (else
      (Variables|Default|SetNewFollowCameraRotation (Variables|Default|GetOldFollowCameraRotation))))
  (if (not (Utilities|Operators|NotEqual(!=) :A (Variables|Default|GetNewFollowCameraLocation)))
    (Variables|Default|SetNewFollowCameraLocation (Variables|Default|GetOldFollowCameraLocation))))

(event Custom|CheckArmLength
  ;[1 1 1] Making sure the Armlength does not get reset when no value change is necessary
  (if (not (> (Variables|Default|GetNewCameraBoomArmLength) 0.0))
    (if (> (Variables|Default|GetOldCameraBoomArmLength) 0.0)
      (Variables|Default|SetNewCameraBoomArmLength (Variables|Default|GetOldCameraBoomArmLength)))))

(event Custom|CheckCameraBoom
  ;[1 1 1] Checking the Values of the Camera Boom that they are not empty
  (if (Utilities|Operators|NotEqual(!=) :A (Variables|Default|GetNewCameraBoomRotation))
    _
    (else
      (Variables|Default|SetNewCameraBoomRotation (Variables|Default|GetOldCamerBoomRotation))))
  (if (Utilities|Operators|NotEqual(!=) :A (Variables|Default|GetNewCameraBoomLocation))
    _
    (else
      (Variables|Default|SetNewCameraBoomLocation (Variables|Default|GetOldCameraBoomLocation))))
  (CallFunction|CheckArmLength))

(fn ConstructionScript)