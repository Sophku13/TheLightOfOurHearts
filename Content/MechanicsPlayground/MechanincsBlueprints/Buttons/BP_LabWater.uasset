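; BP_LabWater is a toggleable water hazard that drains the player's HP while a BP_LightOrb is inside its LightDeathBox.
; OnActivation flip-flops two timelines that sink and flatten the water or restore it, switching the box's collision off or on.
; Orb overlaps enable or disable Tick, which calls ReduceHP on the cached player through InfluencingPlayer.
; PlayerDeath hands the dying player to their death manager's WateryDeath.
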(event OnComponentBeginOverlap(LightDeathBox)
  (params (OverlappedComponent :type Primitive%20Component%20Object%20Reference) (OtherActor :type Actor%20Object%20Reference) (OtherComp :type Primitive%20Component%20Object%20Reference) (OtherBodyIndex :type Integer) (bFromSweep :type Boolean) (SweepResult :type Hit%20Result%20Structure%20%28by%20ref%29))
  ;[1 1 1] Comment
  (Utilities|Casting|CastToBP_LightOrb OtherActor)
  (Actor|Tick|SetActorTickEnabled true)
  (bind _asbp_third_person_character (Utilities|Casting|CastToBP_ThirdPersonCharacter (Game|GetPlayerCharacter 0)))
  (Variables|Default|SetPlayerRef _asbp_third_person_character))

(event OnComponentEndOverlap(LightDeathBox)
  (params (OverlappedComponent :type Primitive%20Component%20Object%20Reference) (OtherActor :type Actor%20Object%20Reference) (OtherComp :type Primitive%20Component%20Object%20Reference) (OtherBodyIndex :type Integer))
  ;[1 1 1] Comment
  (Utilities|Casting|CastToBP_LightOrb OtherActor)
  (Actor|Tick|SetActorTickEnabled false))

(event EventBeginPlay
  ;[1 1 1] Comment
  (Variables|Default|SetStartingTransform (Transformation|GetWorldTransform (Variables|Default|GetWater)))
  (bind _asbp_third_person_character (Utilities|Casting|CastToBP_ThirdPersonCharacter (Game|GetPlayerCharacter 0)))
  (Variables|Default|SetPlayerRef _asbp_third_person_character))

(event Collision|EventActorBeginOverlap
  (params (OtherActor :type Actor%20Object%20Reference)))

(event EventTick
  (params (DeltaSeconds :type Float%20%28single-precision%29))
  ;[1 1 1] Comment
  (if (not (Utilities|Array|IsEmpty (Collision|GetOverlappingActors (Variables|Default|GetLightDeathBox) "/Game/MechanicsPlayground/MechanincsBlueprints/BP_LightOrb.BP_LightOrb_C" :!class /Script/Engine.PrimitiveComponent)))
    (CallFunction|InfluencingPlayer (Variables|Default|GetPlayerRef) false)))

(event EventOnActivation
  (bind _water (Variables|Default|GetWater))
  (bind _water_2 (Variables|Default|GetWater))
  (bind _startingtransform (Variables|Default|GetStartingTransform))
  (bind _startingtransform_2 (Variables|Default|GetStartingTransform))
  (bind _water_3 (Variables|Default|GetWater))
  (bind _returnvalue (Transformation|GetWorldTransform _water))
  (bind (_x _y) (Math|Vector|BreakVector (.scale _startingtransform_2)))
  ;[1 1 1] Comment
  (Utilities|FlowControl|FlipFlop
    (:A
      (bind _newtrack_0 (Timeline|Deactivate PlayFromStart)
        (:Update
          (Transformation|SetWorldLocation _water_3 (Math|Vector|Lerp(Vector) (.location _startingtransform_2) (- (.location _startingtransform_2) "0.000000,0.000000,100.000000") _newtrack_0) false false)
          (Transformation|SetWorldScale3D _water_3 (Math|Vector|Lerp(Vector) (.scale _startingtransform_2) (Math|Vector|MakeVector _x _y 0.0) _newtrack_0))
          (Collision|SetCollisionEnabled (Variables|Default|GetLightDeathBox) "NoCollision"))))
    (:B
      (bind _newtrack_0_2 (Timeline|Activate PlayFromStart)
        (:Update
          (Transformation|SetWorldLocation _water_2 (Math|Vector|Lerp(Vector) (.location _returnvalue) (.location _startingtransform) _newtrack_0_2) false false)
          (Transformation|SetWorldScale3D _water_2 (Math|Vector|Lerp(Vector) (.scale _returnvalue) (.scale _startingtransform) _newtrack_0_2))
          (Collision|SetCollisionEnabled (Variables|Default|GetLightDeathBox) "QueryOnly"))))))

(event EventInfluencingPlayer
  (params (PlayerRef :type BP%20Third%20Person%20Character%20Object%20Reference) (bIsInRange :type Boolean))
  ;[1 1 1] Comment
  (Default|ReduceHP PlayerRef 5.0 bIsInRange self false))

(event EventPlayerDeath
  (params (DyingPlayerReference :type BP%20Third%20Person%20Character%20Object%20Reference))
  ;[1 1 1] Comment
  (Default|WateryDeath (Variables|/Game/ThirdPerson/Blueprints/BP_ThirdPersonCharacter.BP_ThirdPersonCharacter_C|GetDeathManagerRef DyingPlayerReference) DyingPlayerReference true))

(fn ConstructionScript)

(fn IsInfluencingthePlayer
  (params (PlayerRef :type BP%20Third%20Person%20Character%20Object%20Reference))
  (return true))