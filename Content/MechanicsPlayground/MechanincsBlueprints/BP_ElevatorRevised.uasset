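; Light-powered elevator that travels between bottom and top points placed by the construction script from ElevatorHeight.
; Box overlaps detect BP_LightOrb to power it and register it as the third-person character's ActiveElevatorRef, with a colored Visualizer showing state.
; While powered and IsActive, Tick restarts timelines that step the platform by ElevatorSpeed toward the opposite end.
; Losing light mid-travel sends it toward the nearer end.
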(event OnComponentBeginOverlap(Box)
  (params (OverlappedComponent :type Primitive%20Component%20Object%20Reference) (OtherActor :type Actor%20Object%20Reference) (OtherComp :type Primitive%20Component%20Object%20Reference) (OtherBodyIndex :type Integer) (bFromSweep :type Boolean) (SweepResult :type Hit%20Result%20Structure%20%28by%20ref%29))
  (Utilities|Casting|CastToBP_LightOrb OtherActor
    (:then
      (Development|SetHiddeninGame (Variables|Default|GetVisualizer) false false)
      (Variables|Default|SetbIsLightInRange true)
      (Actor|Tick|SetActorTickEnabled true))
    (:CastFailed
      (bind _asbp_third_person_character (Utilities|Casting|CastToBP_ThirdPersonCharacter OtherActor))
      (if (Variables|Default|GetbIsLightInRange)
        (Variables|/Game/ThirdPerson/Blueprints/BP_ThirdPersonCharacter.BP_ThirdPersonCharacter_C|SetActiveElevatorRef _asbp_third_person_character self)
        (Rendering|Material|SetMaterial (Variables|Default|GetVisualizer) 0 "/Game/Materials/MI_Sphere_Emissive_Yellow.MI_Sphere_Emissive_Yellow")))))

(event OnComponentEndOverlap(Box)
  (params (OverlappedComponent :type Primitive%20Component%20Object%20Reference) (OtherActor :type Actor%20Object%20Reference) (OtherComp :type Primitive%20Component%20Object%20Reference) (OtherBodyIndex :type Integer))
  (bind _asbp_light_orb (Utilities|Casting|CastToBP_LightOrb OtherActor)
    (:then
      (Development|SetHiddeninGame (Variables|Default|GetVisualizer) true false)
      (Variables|Default|SetbIsLightInRange false)
      (Variables|/Game/MechanicsPlayground/MechanincsBlueprints/BP_LightOrb.BP_LightOrb_C|SetbDecayIsOnHold _asbp_light_orb false))
    (:CastFailed
      (bind _asbp_third_person_character (Utilities|Casting|CastToBP_ThirdPersonCharacter OtherActor))
      (Rendering|Material|SetMaterial (Variables|Default|GetVisualizer) 0 "/Game/Materials/MI_Sphere_Emissive_Red.MI_Sphere_Emissive_Red")
      (Variables|/Game/ThirdPerson/Blueprints/BP_ThirdPersonCharacter.BP_ThirdPersonCharacter_C|SetActiveElevatorRef _asbp_third_person_character 0))))

(event EventBeginPlay)

(event Collision|EventActorBeginOverlap
  (params (OtherActor :type Actor%20Object%20Reference)))

(event EventTick
  (params (DeltaSeconds :type Float%20%28single-precision%29))
  (bind _platform (Variables|Default|GetPlatform))
  (bind _platform_2 (Variables|Default|GetPlatform))
  (bind _platform_3 (Variables|Default|GetPlatform))
  (bind _platform_4 (Variables|Default|GetPlatform))
  (bind _toplocation (Variables|Default|GetTopLocation))
  (bind _platform_5 (Variables|Default|GetPlatform))
  (bind _platform_6 (Variables|Default|GetPlatform))
  (bind _bottom_location (Variables|Default|GetBottom%20Location))
  (bind _bottom_location_2 (Variables|Default|GetBottom%20Location))
  (bind _toplocation_2 (Variables|Default|GetTopLocation))
  (bind _toplocation_3 (Variables|Default|GetTopLocation))
  (bind _bottom_location_3 (Variables|Default|GetBottom%20Location))
  (bind _platform_7 (Variables|Default|GetPlatform))
  (bind _platform_8 (Variables|Default|GetPlatform))
  (bind _platform_9 (Variables|Default|GetPlatform))
  (bind _platform_10 (Variables|Default|GetPlatform))
  (bind _platform_11 (Variables|Default|GetPlatform))
  (bind _elevatorspeed (Variables|Default|GetElevatorSpeed))
  (bind _elevatorspeed_2 (Variables|Default|GetElevatorSpeed))
  (bind _relativelocation (Variables|/Script/Engine.SceneComponent|GetRelativeLocation _platform_3))
  (bind _relativelocation_2 (Variables|/Script/Engine.SceneComponent|GetRelativeLocation _platform_9))
  (bind _relativelocation_3 (Variables|/Script/Engine.SceneComponent|GetRelativeLocation _toplocation))
  (bind _relativelocation_4 (Variables|/Script/Engine.SceneComponent|GetRelativeLocation _toplocation_2))
  (bind _relativelocation_5 (Variables|/Script/Engine.SceneComponent|GetRelativeLocation _platform_8))
  (bind _relativelocation_6 (Variables|/Script/Engine.SceneComponent|GetRelativeLocation _bottom_location_2))
  (bind _relativelocation_7 (Variables|/Script/Engine.SceneComponent|GetRelativeLocation _bottom_location))
  (bind _relativelocation_8 (Variables|/Script/Engine.SceneComponent|GetRelativeLocation _platform_2))
  (bind _relativelocation_9 (Variables|/Script/Engine.SceneComponent|GetRelativeLocation _platform_6))
  (bind _relativelocation_10 (Variables|/Script/Engine.SceneComponent|GetRelativeLocation _toplocation_3))
  (bind _relativelocation_11 (Variables|/Script/Engine.SceneComponent|GetRelativeLocation _platform))
  (bind _relativelocation_12 (Variables|/Script/Engine.SceneComponent|GetRelativeLocation _bottom_location_3))
  (bind _relativelocation_13 (Variables|/Script/Engine.SceneComponent|GetRelativeLocation _platform_7))
  (bind _relativelocation_14 (Variables|/Script/Engine.SceneComponent|GetRelativeLocation _platform_11))
  (bind _returnvalue (+ (.z _relativelocation_2) _elevatorspeed))
  (bind _returnvalue_2 (- (.z _relativelocation_14) _elevatorspeed_2))
  (if (Variables|Default|GetbIsLightInRange)
    (if (Variables|Default|GetbIsActive)
      (Rendering|Material|SetMaterial (Variables|Default|GetVisualizer) 0 "/Game/Materials/MI_Sphere_Emissive_Green.MI_Sphere_Emissive_Green")
      (if (Variables|Default|GetbIsAtBottom)
        (Variables|Default|SetbIsMoving true)
        (bind _newtrack_0 (Timeline|MoveToTop PlayFromStart)
          (:Update
            (if (> _returnvalue (.z _relativelocation_3))
              (if (>= (- (.z _relativelocation_4) 3e+01) (Math|Float|Lerp (.z _relativelocation_2) (.z _relativelocation_3) _newtrack_0))
                (Transformation|SetRelativeLocation _platform_10 (Math|Vector|MakeVector (.x _relativelocation_2) (.y _relativelocation_2) (Math|Float|Lerp (.z _relativelocation_2) (.z _relativelocation_3) _newtrack_0)) false false)
                (else
                  (Transformation|SetRelativeLocation _platform_10 (Math|Vector|MakeVector (.x _relativelocation_2) (.y _relativelocation_2) (.z _relativelocation_4)) false false)
                  (Variables|Default|SetbIsAtBottom false)
                  (Variables|Default|SetbIsActive false)
                  (Rendering|Material|SetMaterial (Variables|Default|GetVisualizer) 0 "/Game/Materials/MI_Sphere_Emissive_Yellow.MI_Sphere_Emissive_Yellow")))
              (else
                (Transformation|SetRelativeLocation (Variables|Default|GetPlatform) (Math|Vector|MakeVector (.x _relativelocation_5) (.y _relativelocation_5) (Math|Float|Lerp (.z _relativelocation_5) _returnvalue _newtrack_0)) false false)))))
        (else
          (Variables|Default|SetbIsMoving true)
          (bind _newtrack_0_2 (Timeline|MoveToBottom PlayFromStart)
            (:Update
              (if (< _returnvalue_2 (.z _relativelocation_7))
                (if (<= (+ (.z _relativelocation_6) 3e+01) (Math|Float|Lerp (.z _relativelocation_14) (.z _relativelocation_7) _newtrack_0_2))
                  (Transformation|SetRelativeLocation _platform_3 (Math|Vector|MakeVector (.x _relativelocation) (.y _relativelocation) (Math|Float|Lerp (.z _relativelocation_14) (.z _relativelocation_7) _newtrack_0_2)) false false)
                  (else
                    (Transformation|SetRelativeLocation _platform (Math|Vector|MakeVector (.x _relativelocation) (.y _relativelocation) (.z _relativelocation_6)) false false)
                    (Variables|Default|SetbIsAtBottom true)
                    (Variables|Default|SetbIsActive false)
                    (Rendering|Material|SetMaterial (Variables|Default|GetVisualizer) 0 "/Game/Materials/MI_Sphere_Emissive_Yellow.MI_Sphere_Emissive_Yellow")))
                (else
                  (Transformation|SetRelativeLocation _platform (Math|Vector|MakeVector (.x _relativelocation_11) (.y _relativelocation_11) (Math|Float|Lerp (.z (Variables|/Script/Engine.SceneComponent|GetRelativeLocation (Variables|Default|GetPlatform))) _returnvalue_2 _newtrack_0_2)) false false))))))))
    (elif (Variables|Default|GetbIsMoving)
      (if (not (or (Utilities|Operators|EqualEqual (Variables|/Script/Engine.SceneComponent|GetRelativeLocation (Variables|Default|GetBottom%20Location)) _relativelocation_13 1.0) (Utilities|Operators|EqualEqual _relativelocation_13 (Variables|/Script/Engine.SceneComponent|GetRelativeLocation (Variables|Default|GetTopLocation)) 1.0)))
        (Variables|Default|SetbIsMoving true)
        (bind _newtrack_0_3 (Timeline|MoveToBottomOrTop PlayFromStart)
          (:Update
            (if (<= (.z (Variables|/Script/Engine.SceneComponent|GetRelativeLocation (Variables|Default|GetPlatform))) (+ (/ (Variables|Default|GetElevatorHeight) 2) (.z (Variables|/Script/Engine.SceneComponent|GetRelativeLocation (Variables|Default|GetBottom%20Location)))))
              (if (<= (+ (.z _relativelocation_12) 3e+01) (Math|Float|Lerp (.z _relativelocation_8) (.z (Variables|/Script/Engine.SceneComponent|GetRelativeLocation (Variables|Default|GetBottom%20Location))) _newtrack_0_3))
                (Transformation|SetRelativeLocation _platform_4 (Math|Vector|MakeVector (.x _relativelocation_8) (.y _relativelocation_8) (.z _relativelocation_12)) false false)
                (Variables|Default|SetbIsAtBottom true)
                (else
                  (Transformation|SetRelativeLocation _platform_4 (Math|Vector|MakeVector (.x _relativelocation_8) (.y _relativelocation_8) (Math|Float|Lerp (.z _relativelocation_8) (.z (Variables|/Script/Engine.SceneComponent|GetRelativeLocation (Variables|Default|GetBottom%20Location))) _newtrack_0_3)) false false)
                  (Variables|Default|SetbIsMoving false)))
              (elif (>= (- (.z _relativelocation_10) 3e+01) (Math|Float|Lerp (.z _relativelocation_9) (.z (Variables|/Script/Engine.SceneComponent|GetRelativeLocation (Variables|Default|GetTopLocation))) _newtrack_0_3))
                (Transformation|SetRelativeLocation _platform_5 (Math|Vector|MakeVector (.x _relativelocation_9) (.y _relativelocation_9) (.z _relativelocation_10)) false false)
                (Variables|Default|SetbIsAtBottom false)
                (else
                  (Transformation|SetRelativeLocation _platform_5 (Math|Vector|MakeVector (.x _relativelocation_9) (.y _relativelocation_9) (Math|Float|Lerp (.z _relativelocation_9) (.z (Variables|/Script/Engine.SceneComponent|GetRelativeLocation (Variables|Default|GetTopLocation))) _newtrack_0_3)) false false)
                  (Variables|Default|SetbIsMoving false)))))
          (:Finished
            (Variables|Default|SetbIsMoving false)))))))

(fn ConstructionScript
  (bind _bottom_location (Variables|Default|GetBottom%20Location))
  (bind _defaultsceneroot (Variables|Default|GetDefaultSceneRoot))
  (bind _elevatorheight (Variables|Default|GetElevatorHeight))
  (bind _platform (Variables|Default|GetPlatform))
  (bind _returnvalue (Transformation|GetWorldLocation _bottom_location))
  (bind _returnvalue_2 (Transformation|GetWorldLocation _defaultsceneroot))
  (bind _returnvalue_3 (- _elevatorheight 1e+02))
  (bind _relativelocation (Variables|/Script/Engine.SceneComponent|GetRelativeLocation _platform))
  (bind _returnvalue_4 (Math|Vector|MakeVector 0.0 0.0 _returnvalue_3))
  (bind _returnvalue_5 (Math|Float|Absolute(Float) (.z _relativelocation)))
  (bind _returnvalue_6 (+ _returnvalue _returnvalue_4))
  (Transformation|SetWorldLocation (Variables|Default|GetBottom%20Location) (Math|Vector|MakeVector (.x _returnvalue_2) (.y _returnvalue_2) (- (.z _returnvalue_2) _returnvalue_5)) false false)
  (Transformation|SetWorldLocation (Variables|Default|GetTopLocation) _returnvalue_6 false false)
  (Transformation|SetWorldLocation (Variables|Default|GetTopLocator) (+ _returnvalue_6 (Math|Vector|MakeVector 0.0 0.0 (+ _returnvalue_5 1e+02))) false false))