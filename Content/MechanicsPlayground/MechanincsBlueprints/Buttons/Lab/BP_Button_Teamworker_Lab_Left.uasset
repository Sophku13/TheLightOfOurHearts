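; Left-hand lab teamworker button, a child button that drives the lab's orb socket mover when its task fires.
; On BeginPlay it dresses its sign with the straight-arrow glow particles and material, rotated 90 degrees.
; ButtonTask casts the group to BP_ButtonGrouper_Lab, has the lab's SocketMover move the orb from its end location back to its start, then deactivates the grouper.
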(event EventBeginPlay
  (|CallParentFunction)
  (Class|NiagaraComponent|SetAsset (Variables|/Game/MechanicsPlayground/MechanincsBlueprints/GlowTextures/BP_TEMPLATE_BlowGlow_Base.BP_TEMPLATE_BlowGlow_Base_C|GetTextureGlow (Variables|Default|GetSignGlow)) "/Game/MechanicsPlayground/MechanincsBlueprints/GlowTextures/NiagaraSystems/NS_BlowRevealParticles_ArrowStraight.NS_BlowRevealParticles_ArrowStraight" false)
  (Transformation|SetActorRotation (Variables|Default|GetSignGlow) "0.000000,0.000000,90.000000")
  (Rendering|Material|SetMaterial (Variables|Default|GetSignBase) 0 "/Game/MechanicsPlayground/MechanincsBlueprints/GlowTextures/Material/M_GlowMechanic_ArrowStraight.M_GlowMechanic_ArrowStraight")
  (Transformation|SetWorldRotation (Variables|Default|GetSignBase) "0.000000,0.000000,90.000000" false false))

(event Collision|EventActorBeginOverlap
  (params (OtherActor :type Actor%20Object%20Reference))
  (|CallParentFunction OtherActor) ; This node is disabled and will not be called.\nDrag off pins to build functionality.
)

(event EventTick
  (params (DeltaSeconds :type Float%20%28single-precision%29))
  (|CallParentFunction DeltaSeconds) ; This node is disabled and will not be called.\nDrag off pins to build functionality.
)

(event EventButtonTask
  (params (ButtonGroup :type BP%20Button%20Grouper%20Base%20Object%20Reference))
  (bind _movecoordinates (Variables|Default|GetMoveCoordinates))
  (bind _asbp_button_grouper_lab (Utilities|Casting|CastToBP_ButtonGrouper_Lab ButtonGroup))
  (Default|MoveOrbtoStart (Variables|/Game/MechanicsPlayground/MechanincsBlueprints/Buttons/Lab/BP_Lab.BP_Lab_C|GetSocketMover (Variables|/Game/MechanicsPlayground/MechanincsBlueprints/Buttons/Lab/BP_ButtonGrouper_Lab.BP_ButtonGrouper_Lab_C|GetLabRef _asbp_button_grouper_lab)) (Variables|/Game/MechanicsPlayground/MechanincsBlueprints/Buttons/Bases/BP_CoordinateVtoV.BP_CoordinateVtoV_C|GetEndLocation _movecoordinates) (Variables|/Game/MechanicsPlayground/MechanincsBlueprints/Buttons/Bases/BP_CoordinateVtoV.BP_CoordinateVtoV_C|GetStartLocation _movecoordinates))
  (Default|Deactivate _asbp_button_grouper_lab false))

(fn ConstructionScript
  (|CallParentFunction))