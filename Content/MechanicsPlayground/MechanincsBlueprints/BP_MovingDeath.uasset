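; BP_MovingDeath is a lethal water volume that kills the character through the Light Orb.
; HitBox overlap events cache the orb, toggle ticking as it enters or leaves, and track whether the character is inside.
; While the character is inside, Tick tests the orb's MLightOrb component itself, not its collision sphere, against the HitBox.
; On contact it sets orb strength to -1 and updates orb conditions, triggering death.
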(event OnComponentBeginOverlap(HitBox)
  (params (OverlappedComponent :type Primitive%20Component%20Object%20Reference) (OtherActor :type Actor%20Object%20Reference) (OtherComp :type Primitive%20Component%20Object%20Reference) (OtherBodyIndex :type Integer) (bFromSweep :type Boolean) (SweepResult :type Hit%20Result%20Structure%20%28by%20ref%29))
  ;[0.1216 0.902 0.6627] Activating the Tick when the Light Orb is in Range of the Water
  (bind _asbp_light_orb (Utilities|Casting|CastToBP_LightOrb OtherActor)
    (:then
      (Variables|Default|SetLightOrbRef _asbp_light_orb)
      (Components|Tick|SetComponentTickEnabled (Variables|Default|GetHitBox) true)
      (Actor|Tick|SetActorTickEnabled self true)
      (Variables|/Script/Engine.PrimitiveComponent|SetbGenerateOverlapEvents (Variables|/Game/MechanicsPlayground/MechanincsBlueprints/BP_LightOrb.BP_LightOrb_C|GetM_LightOrb (Variables|Default|GetLightOrbRef)) true))
    (:CastFailed
      (Utilities|Casting|CastToBP_ThirdPersonCharacter OtherActor)
      (Variables|Default|SetbCharacterisInside true))))

(event OnComponentEndOverlap(HitBox)
  (params (OverlappedComponent :type Primitive%20Component%20Object%20Reference) (OtherActor :type Actor%20Object%20Reference) (OtherComp :type Primitive%20Component%20Object%20Reference) (OtherBodyIndex :type Integer))
  ;[0.1216 0.902 0.6627] Disabling the Code again, when the Light leaves the range of the Water
  (bind _asbp_light_orb (Utilities|Casting|CastToBP_LightOrb OtherActor)
    (:then
      (Variables|Default|SetLightOrbRef _asbp_light_orb)
      (Components|Tick|SetComponentTickEnabled (Variables|Default|GetHitBox) false)
      (Actor|Tick|SetActorTickEnabled false))
    (:CastFailed
      (Utilities|Casting|CastToBP_ThirdPersonCharacter OtherActor)
      (Variables|Default|SetbCharacterisInside false))))

(event EventBeginPlay)

(event Collision|EventActorBeginOverlap
  (params (OtherActor :type Actor%20Object%20Reference)))

(event EventTick
  (params (DeltaSeconds :type Float%20%28single-precision%29))
  (bind _lightorbref (Variables|Default|GetLightOrbRef))
  ;[0.1216 0.902 0.6627] Tick - if the Actual LightOrb Component (NOT THE COLLISION SPHERE!!) is overlapping with this hitbox. And if they do overlap set the LightOrbStrength to death and initiate the update that will lead to the death of the character
  (if (Variables|Default|GetbCharacterisInside)
    (if (Class|PrimitiveComponent|IsOverlappingComponent (Variables|/Game/MechanicsPlayground/MechanincsBlueprints/BP_LightOrb.BP_LightOrb_C|GetM_LightOrb (Variables|Default|GetLightOrbRef)) (Variables|Default|GetHitBox))
      (Default|SetLightOrbStrength _lightorbref -1.0)
      (Default|SetLightOrbConditions _lightorbref))))

(fn ConstructionScript)