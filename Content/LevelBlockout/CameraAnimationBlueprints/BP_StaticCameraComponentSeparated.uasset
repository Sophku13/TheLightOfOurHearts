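; Trigger volume that switches the third-person player's view to a separate static camera while they are inside it.
; Box begin overlap by BP_ThirdPersonCharacter blends that character's PlayerController view target to CameraToFind, and end overlap blends back to the character.
; Both blends share CameraBlendTime.
; Both handlers also call GetActorOfClass for a CameraActor, but its result is unused.
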(event OnComponentBeginOverlap(Box)
  (params (OverlappedComponent :type Primitive%20Component%20Object%20Reference) (OtherActor :type Actor%20Object%20Reference) (OtherComp :type Primitive%20Component%20Object%20Reference) (OtherBodyIndex :type Integer) (bFromSweep :type Boolean) (SweepResult :type Hit%20Result%20Structure%20%28by%20ref%29))
  (bind _asbp_third_person_character (Utilities|Casting|CastToBP_ThirdPersonCharacter OtherActor))
  (if (Utilities|IsValid _asbp_third_person_character)
    (bind _asplayer_controller (Utilities|Casting|CastToPlayerController (Pawn|GetController _asbp_third_person_character)))
    (if (Utilities|IsValid _asplayer_controller)
      (Actor|GetActorOfClass "/Script/Engine.CameraActor")
      (Game|Player|SetViewTargetwithBlend _asplayer_controller (Variables|Default|GetCameraToFind) (Variables|Default|GetCameraBlendTime) "VTBlend_Linear" 0.0 false))))

(event OnComponentEndOverlap(Box)
  (params (OverlappedComponent :type Primitive%20Component%20Object%20Reference) (OtherActor :type Actor%20Object%20Reference) (OtherComp :type Primitive%20Component%20Object%20Reference) (OtherBodyIndex :type Integer))
  (bind _asbp_third_person_character (Utilities|Casting|CastToBP_ThirdPersonCharacter OtherActor))
  (if (Utilities|IsValid _asbp_third_person_character)
    (bind _asplayer_controller (Utilities|Casting|CastToPlayerController (Pawn|GetController _asbp_third_person_character)))
    (if (Utilities|IsValid _asplayer_controller)
      (Actor|GetActorOfClass "/Script/Engine.CameraActor")
      (Game|Player|SetViewTargetwithBlend _asplayer_controller _asbp_third_person_character (Variables|Default|GetCameraBlendTime) "VTBlend_Linear" 0.0 false))))

(event EventBeginPlay)

(event Collision|EventActorBeginOverlap
  (params (OtherActor :type Actor%20Object%20Reference)))

(event EventTick
  (params (DeltaSeconds :type Float%20%28single-precision%29)))

(fn ConstructionScript)