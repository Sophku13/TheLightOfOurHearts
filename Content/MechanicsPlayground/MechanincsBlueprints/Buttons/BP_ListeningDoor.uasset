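; A door actor that slides open when it receives an activation event.
; OnActivation turns the door light green and plays the Mover timeline, with IsRotated choosing world X or Y as the slide axis.
; Each timeline update lerps from the door's current position toward a small positive offset, so movement accumulates per update instead of blending between fixed endpoints.
; The file has no closing logic.
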(event EventBeginPlay)

(event Collision|EventActorBeginOverlap
  (params (OtherActor :type Actor%20Object%20Reference)))

(event EventTick
  (params (DeltaSeconds :type Float%20%28single-precision%29)))

(event EventOnActivation
  (bind _door (Variables|Default|GetDoor))
  (bind _returnvalue (Transformation|GetWorldLocation _door))
  (bind (_x _y _z) (Math|Vector|BreakVector _returnvalue))
  (bind (_x_2 _y_2 _z_2) (Math|Vector|BreakVector _returnvalue))
  ;[0.1216 0.902 0.6627] If something is activating the door then it will open either on the y or the x axis
  (Rendering|Components|Light|SetLightColor (Variables|Default|GetDoorLight) "(R=0.144904,G=1.000000,B=0.000000,A=1.000000)" true)
  (bind _newtrack_0 (Timeline|Mover Play)
    (:Update
      (if (Variables|Default|GetbIsRotated)
        ;;[0.1216 0.902 0.6627] Setting the new location and moving the door to it
        (Transformation|SetWorldLocation _door (Math|Vector|MakeVector (Math|Float|Lerp _x (+ _x 3.0) _newtrack_0) _y _z) false false)
        (else
          (Transformation|SetWorldLocation _door (Math|Vector|MakeVector _x_2 (Math|Float|Lerp _y_2 (+ _y_2 3.0) _newtrack_0) _z_2) false false))))))

(fn ConstructionScript)