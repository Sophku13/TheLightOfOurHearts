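; Lighthouse hint sprite that brightens as the light orb nears it, judging by its plane's material parameters.
; When a BP_LightOrb overlaps the plane, a fast looping timer maps orb-to-plane distance to Opacity and Emission, both strongest up close and fading toward DistanceOfDissapear.
; Any overlap end pauses the timer, leaving the last values in place.
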(event OnComponentBeginOverlap(Plane)
  (params (OverlappedComponent :type Primitive%20Component%20Object%20Reference) (OtherActor :type Actor%20Object%20Reference) (OtherComp :type Primitive%20Component%20Object%20Reference) (OtherBodyIndex :type Integer) (bFromSweep :type Boolean) (SweepResult :type Hit%20Result%20Structure%20%28by%20ref%29))
  (bind _asbp_light_orb (Utilities|Casting|CastToBP_LightOrb OtherActor))
  (Variables|Default|SetLightOrbRef! _asbp_light_orb)
  (bind _returnvalue (Utilities|Time|SetTimerbyEvent (delegate Custom|UpdateOpacity) 0.01 true))
  (Variables|Default|SetTimer _returnvalue))

(event OnComponentEndOverlap(Plane)
  (params (OverlappedComponent :type Primitive%20Component%20Object%20Reference) (OtherActor :type Actor%20Object%20Reference) (OtherComp :type Primitive%20Component%20Object%20Reference) (OtherBodyIndex :type Integer))
  (Utilities|Time|PauseTimerbyHandle (Variables|Default|GetTimer)))

(event Custom|UpdateOpacity
  (bind _plane (Variables|Default|GetPlane))
  (bind _plane_2 (Variables|Default|GetPlane))
  (bind _lightorbref_ (Variables|Default|GetLightOrbRef!))
  (bind _distanceofdissapear (Variables|Default|GetDistanceOfDissapear))
  (bind _returnvalue (Transformation|GetActorLocation _lightorbref_))
  (bind _returnvalue_2 (Transformation|GetWorldLocation _plane))
  (bind _returnvalue_3 (Math|Vector|Distance(Vector) _returnvalue _returnvalue_2))
  (Rendering|Material|SetScalarParameterValueonMaterials _plane_2 "Opacity" (Math|Float|MapRangeClamped _returnvalue_3 0.0 _distanceofdissapear 1.0 0.0))
  (Rendering|Material|SetScalarParameterValueonMaterials _plane_2 "Emission" (Math|Float|MapRangeClamped _returnvalue_3 0.0 _distanceofdissapear 2e+02 0.0)))

(event Collision|EventActorBeginOverlap
  (params (OtherActor :type Actor%20Object%20Reference)))

(event EventTick
  (params (DeltaSeconds :type Float%20%28single-precision%29)))

(event EventBeginPlay
  (Variables|Default|SetDistanceOfDissapear (Variables|Default|GetDistanceOfDissapear)))

(fn ConstructionScript)