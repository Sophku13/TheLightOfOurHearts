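; Light socket Blueprint that toggles the color of the light orb placed on it when its linked trigger button is pressed.
; On BeginPlay it binds an event to the Trigger, then runs the parent's BeginPlay.
; When pressed with a valid orb on the socket, a FlipFlop alternates the orb's light color and emissive material between yellow and blue.
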(event Custom|ButtonPressed
  (bind _lightorbref (Variables|Default|GetLightOrbRef)
    (:then
      (if (Variables|Default|GetbLightOnSocket)
        (Utilities|FlowControl|FlipFlop
          (:A
            (Rendering|Components|Light|SetLightColor (Variables|/Game/MechanicsPlayground/MechanincsBlueprints/BP_LightOrb.BP_LightOrb_C|GetLightOrb_Lighting _lightorbref) "(R=0.890354,G=1.000000,B=0.000000,A=1.000000)" true)
            (Rendering|Material|SetMaterial (Variables|/Game/MechanicsPlayground/MechanincsBlueprints/BP_LightOrb.BP_LightOrb_C|GetM_LightOrb (Variables|Default|GetLightOrbRef)) 0 "/Game/Materials/MI_Sphere_Emissive_Yellow.MI_Sphere_Emissive_Yellow"))
          (:B
            (Rendering|Components|Light|SetLightColor (Variables|/Game/MechanicsPlayground/MechanincsBlueprints/BP_LightOrb.BP_LightOrb_C|GetLightOrb_Lighting _lightorbref) "(R=0.305882,G=0.603922,B=1.000000,A=1.000000)" true)
            (Rendering|Material|SetMaterial (Variables|/Game/MechanicsPlayground/MechanincsBlueprints/BP_LightOrb.BP_LightOrb_C|GetM_LightOrb (Variables|Default|GetLightOrbRef)) 0 "/Game/Materials/MI_Sphere_Emissive_Inst.MI_Sphere_Emissive_Inst")))))
    (:else)))

(event EventBeginPlay
  (bind _trigger (Variables|Default|GetTrigger)
    (:then
      (EventDispatchers|BindEventtoButtonTriggered _trigger (EventDispatchers|CreateEvent :!event Custom|ButtonPressed)))
    (:else
      _))
  (|CallParentFunction))

(event Collision|EventActorBeginOverlap
  (params (OtherActor :type Actor%20Object%20Reference)))

(event EventTick
  (params (DeltaSeconds :type Float%20%28single-precision%29))
  (|CallParentFunction DeltaSeconds) ; This node is disabled and will not be called.\nDrag off pins to build functionality.
)

(fn ConstructionScript
  (|CallParentFunction))