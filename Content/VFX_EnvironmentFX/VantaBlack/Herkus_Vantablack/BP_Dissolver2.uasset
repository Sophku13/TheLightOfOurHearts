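; BP_Dissolver2 is a box volume actor that publishes its Cube component's transform to the MPC_NewVanta material parameter collection, apparently to drive a Vantablack dissolve effect.
; It writes world location, scale as bounds, and forward, right and up axes as vectors, so materials reading the collection can evaluate an oriented box.
; The Construction Script and Tick repeat the same writes, covering editor placement and runtime movement.
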(event EventBeginPlay)

(event Collision|EventActorBeginOverlap
  (params (OtherActor :type Actor%20Object%20Reference)))

(event EventTick
  (params (DeltaSeconds :type Float%20%28single-precision%29))
  (bind _cube (Variables|Default|GetCube))
  (bind _cube_2 (Variables|Default|GetCube))
  (Rendering|Material|SetVectorParameterValue "/Game/VFX_EnvironmentFX/VantaBlack/Herkus_Vantablack/MPC_NewVanta.MPC_NewVanta" "Location" (Math|Conversions|ToLinearColor(Vector) (Transformation|GetWorldLocation _cube_2)) :!class /Script/Engine.KismetMaterialLibrary)
  (Rendering|Material|SetVectorParameterValue "/Game/VFX_EnvironmentFX/VantaBlack/Herkus_Vantablack/MPC_NewVanta.MPC_NewVanta" "Bounds" (Math|Conversions|ToLinearColor(Vector) (Transformation|GetWorldScale _cube_2)) :!class /Script/Engine.KismetMaterialLibrary)
  (Rendering|Material|SetVectorParameterValue "/Game/VFX_EnvironmentFX/VantaBlack/Herkus_Vantablack/MPC_NewVanta.MPC_NewVanta" "X" (Math|Conversions|ToLinearColor(Vector) (Math|Vector|GetForwardVector _cube)) :!class /Script/Engine.KismetMaterialLibrary)
  (Rendering|Material|SetVectorParameterValue "/Game/VFX_EnvironmentFX/VantaBlack/Herkus_Vantablack/MPC_NewVanta.MPC_NewVanta" "Y" (Math|Conversions|ToLinearColor(Vector) (Math|Vector|GetRightVector _cube)) :!class /Script/Engine.KismetMaterialLibrary)
  (Rendering|Material|SetVectorParameterValue "/Game/VFX_EnvironmentFX/VantaBlack/Herkus_Vantablack/MPC_NewVanta.MPC_NewVanta" "Z" (Math|Conversions|ToLinearColor(Vector) (Math|Vector|GetUpVector _cube)) :!class /Script/Engine.KismetMaterialLibrary))

(fn ConstructionScript
  (bind _cube (Variables|Default|GetCube))
  (bind _cube_2 (Variables|Default|GetCube))
  (Rendering|Material|SetVectorParameterValue "/Game/VFX_EnvironmentFX/VantaBlack/Herkus_Vantablack/MPC_NewVanta.MPC_NewVanta" "Location" (Math|Conversions|ToLinearColor(Vector) (Transformation|GetWorldLocation _cube)) :!class /Script/Engine.KismetMaterialLibrary)
  (Rendering|Material|SetVectorParameterValue "/Game/VFX_EnvironmentFX/VantaBlack/Herkus_Vantablack/MPC_NewVanta.MPC_NewVanta" "Bounds" (Math|Conversions|ToLinearColor(Vector) (Transformation|GetWorldScale _cube)) :!class /Script/Engine.KismetMaterialLibrary)
  (Rendering|Material|SetVectorParameterValue "/Game/VFX_EnvironmentFX/VantaBlack/Herkus_Vantablack/MPC_NewVanta.MPC_NewVanta" "X" (Math|Conversions|ToLinearColor(Vector) (Math|Vector|GetForwardVector _cube_2)) :!class /Script/Engine.KismetMaterialLibrary)
  (Rendering|Material|SetVectorParameterValue "/Game/VFX_EnvironmentFX/VantaBlack/Herkus_Vantablack/MPC_NewVanta.MPC_NewVanta" "Y" (Math|Conversions|ToLinearColor(Vector) (Math|Vector|GetRightVector _cube_2)) :!class /Script/Engine.KismetMaterialLibrary)
  (Rendering|Material|SetVectorParameterValue "/Game/VFX_EnvironmentFX/VantaBlack/Herkus_Vantablack/MPC_NewVanta.MPC_NewVanta" "Z" (Math|Conversions|ToLinearColor(Vector) (Math|Vector|GetUpVector _cube_2)) :!class /Script/Engine.KismetMaterialLibrary))