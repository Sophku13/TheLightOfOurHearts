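; Light actor whose point light pulses while a BP_LightOrb is inside its sphere trigger.
; Orb overlap starts a looping timer that sets intensity from a time-based sine wave, with frequency mapped from orb distance so it rises as the orb nears.
; The amplitude mapping measures the actor against itself, so peak intensity stays constant.
; Any end overlap pauses the timer, and each update prints the sine value.
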(event OnComponentBeginOverlap(Sphere)
  (params (OverlappedComponent :type Primitive%20Component%20Object%20Reference) (OtherActor :type Actor%20Object%20Reference) (OtherComp :type Primitive%20Component%20Object%20Reference) (OtherBodyIndex :type Integer) (bFromSweep :type Boolean) (SweepResult :type Hit%20Result%20Structure%20%28by%20ref%29))
  (bind _asbp_light_orb (Utilities|Casting|CastToBP_LightOrb OtherActor))
  (Variables|Default|SetAs%20BP%20Light%20Orb _asbp_light_orb)
  (bind _returnvalue (Utilities|Time|SetTimerbyEvent (delegate Custom|UpdateIntensity) 0.1 true))
  (Variables|Default|SetTimer _returnvalue))

(event OnComponentEndOverlap(Sphere)
  (params (OverlappedComponent :type Primitive%20Component%20Object%20Reference) (OtherActor :type Actor%20Object%20Reference) (OtherComp :type Primitive%20Component%20Object%20Reference) (OtherBodyIndex :type Integer))
  (Utilities|Time|PauseTimerbyHandle (Variables|Default|GetTimer)))

(event Custom|UpdateIntensity
  (bind _returnvalue (Utilities|Time|GetTimeSeconds))
  (bind _self self)
  (bind _as_bp_light_orb (Variables|Default|GetAs%20BP%20Light%20Orb))
  (bind _returnvalue_2 (Transformation|GetActorLocation _as_bp_light_orb))
  (bind _returnvalue_3 (Transformation|GetActorLocation _self))
  (bind _returnvalue_4 (Math|Vector|Distance(Vector) _returnvalue_2 _returnvalue_3))
  (bind _returnvalue_5 (Math|Float|MapRangeClamped _returnvalue_4 0.0 7e+02 1e+03 0.0))
  (bind _returnvalue_6 (* _returnvalue _returnvalue_5))
  (bind _returnvalue_7 (Math|Trig|Sin(Degrees) _returnvalue_6))
  (Development|PrintString (Utilities|String|ToString(Float) _returnvalue_7) true true "(R=0.000000,G=0.660000,B=1.000000,A=1.000000)" (Utilities|Time|GetWorldDeltaSeconds))
  (Rendering|Components|Light|SetIntensity (Variables|Default|GetPointLight) (* (/ (+ _returnvalue_7 1.0) 2.0) (Math|Float|MapRangeClamped (Math|Vector|Distance(Vector) (Transformation|GetActorLocation) (Transformation|GetActorLocation self)) 0.0 7e+02 2e+04 0.0))))

(fn ConstructionScript)