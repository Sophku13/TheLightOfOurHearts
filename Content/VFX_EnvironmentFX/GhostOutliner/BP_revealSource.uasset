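; Reveal source actor for the GhostOutliner effect that publishes a sphere volume to materials through Material Parameter Collections.
; Tick writes the Sphere's world location and scale to MPC_reveal, while the Construction Script writes the same values to a different collection, MPC_dissolve.
; BeginPlay shows or hides the Sphere from EnergyVisibility.
; Nodes for passing the Sphere's rotation axes to MPC_dissolve exist but are unconnected.
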(event EventBeginPlay
  (Rendering|SetVisibility (Variables|Default|GetSphere) (Variables|Default|GetEnergyVisibility) false))

(event EventTick
  (params (DeltaSeconds :type Float%20%28single-precision%29))
  (Rendering|Material|SetVectorParameterValue "/Game/VFX_EnvironmentFX/GhostOutliner/MPC_reveal.MPC_reveal" "LocationReveal" (Math|Conversions|ToLinearColor(Vector) (Transformation|GetWorldLocation (Variables|Default|GetSphere))) :!class /Script/Engine.KismetMaterialLibrary)
  ;[1 1 1] useless here
  (Rendering|Material|SetVectorParameterValue "/Game/VFX_EnvironmentFX/GhostOutliner/MPC_reveal.MPC_reveal" "BoundReveal" (Math|Conversions|ToLinearColor(Vector) (Transformation|GetWorldScale (Variables|Default|GetSphere))) :!class /Script/Engine.KismetMaterialLibrary))

(fn ConstructionScript
  (bind _sphere (Variables|Default|GetSphere))
  (Rendering|Material|SetVectorParameterValue "/Game/VFX_EnvironmentFX/VantaBlack/Realtime_dissolve/MPC_dissolve.MPC_dissolve" "Location" (Math|Conversions|ToLinearColor(Vector) (Transformation|GetWorldLocation _sphere)) :!class /Script/Engine.KismetMaterialLibrary)
  (Rendering|Material|SetVectorParameterValue "/Game/VFX_EnvironmentFX/VantaBlack/Realtime_dissolve/MPC_dissolve.MPC_dissolve" "Bound" (Math|Conversions|ToLinearColor(Vector) (Transformation|GetWorldScale _sphere)) :!class /Script/Engine.KismetMaterialLibrary))