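; Double door that slides open when a BP_LightOrb enters its trigger Box.
; A Sequence starts two latent MoveComponentTo calls, so DoorL and DoorR ease to fixed relative positions in parallel.
; InProgress blocks retriggering during the move, and IsDoorOpen is set on completion; no logic closes the doors again.
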(event OnComponentBeginOverlap(Box)
  (params (OverlappedComponent :type Primitive%20Component%20Object%20Reference) (OtherActor :type Actor%20Object%20Reference) (OtherComp :type Primitive%20Component%20Object%20Reference) (OtherBodyIndex :type Integer) (bFromSweep :type Boolean) (SweepResult :type Hit%20Result%20Structure%20%28by%20ref%29))
  ;[0.1216 0.902 0.6627] The Doors are reacting to the light source. Both move simultaniously
  (Utilities|Casting|CastToBP_LightOrb OtherActor)
  (if (not (Variables|Default|GetisDoorOpen))
    (if (not (Variables|Default|GetinProgress))
      (Variables|Default|SetinProgress true)
      ;;[0.1216 0.902 0.6627] Parallel Doors opening
      (Utilities|FlowControl|Sequence
        (:then_0
          (Components|MoveComponentTo (Variables|Default|GetDoorL) "0.000000,500.000000,140.000000" "0, 0, 0" true true 5.0 false))
        (:then_1
          (Components|MoveComponentTo (Variables|Default|GetDoorR) "0.000000,100.000000,140.000000" "0, 0, 0" true true 5.0 false)))
      (Variables|Default|SetisDoorOpen true)
      (Variables|Default|SetinProgress false))))

(fn ConstructionScript)