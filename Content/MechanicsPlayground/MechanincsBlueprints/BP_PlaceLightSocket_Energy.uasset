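; BP_PlaceLightSocket_Energy is an energy variant of a light placement socket that activates linked actors once a light sits on it.
; While LightOnSocket is true, Tick sends OnActivationMessage to every entry in Actors, then calls the parent Tick.
; A DoN node with no reset limits this to five frames, repeating activation for a flicker effect, though the graph comment says three times.
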(event EventBeginPlay
  (|CallParentFunction) ; This node is disabled and will not be called.\nDrag off pins to build functionality.
)

(event Collision|EventActorBeginOverlap
  (params (OtherActor :type Actor%20Object%20Reference)))

(event EventTick
  (params (DeltaSeconds :type Float%20%28single-precision%29))
  ;[0.1216 0.902 0.6627] The event tick activates all of the actors connected three times to create a sort of flickering effect
  (if (Variables|Default|GetbLightOnSocket)
    (Utilities|FlowControl|Sequence
      (:then_0
        (Utilities|FlowControl|DoN 5
          (:Exit
            (for _array_element (Variables|Default|GetActors)
              (Class|BPILightFueledActivation|OnActivation(Message) _array_element)))))
      (:then_1
        (|CallParentFunction DeltaSeconds)))))

(fn ConstructionScript
  (|CallParentFunction))