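; BP_LightImpactArea is a box volume that changes how the Light Orb decays while inside it.
; On overlap it stores the orb, applies its decay modifier and activates; on exit it resets the modifier to default.
; While active, Tick drains orb strength only if the orb's tick interval nearly equals a fixed value.
; Player influence and death hooks only print debug text, and the influence check is a WIP stub returning true.
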(event OnComponentEndOverlap(Box)
  (params (OverlappedComponent :type Primitive%20Component%20Object%20Reference) (OtherActor :type Actor%20Object%20Reference) (OtherComp :type Primitive%20Component%20Object%20Reference) (OtherBodyIndex :type Integer))
  ;[0.1216 0.902 0.6627] Sets the Decay Modifier back to its default, when the LightOrb leaves the Range
  (bind _asbp_light_orb (Utilities|Casting|CastToBP_LightOrb OtherActor))
  (Development|PrintString "LightExitedArea")
  (Variables|/Game/MechanicsPlayground/MechanincsBlueprints/BP_LightOrb.BP_LightOrb_C|SetLevelOrbDecayModifier _asbp_light_orb 1.0)
  (Variables|Default|SetbIsActivated false))

(event OnComponentBeginOverlap(Box)
  (params (OverlappedComponent :type Primitive%20Component%20Object%20Reference) (OtherActor :type Actor%20Object%20Reference) (OtherComp :type Primitive%20Component%20Object%20Reference) (OtherBodyIndex :type Integer) (bFromSweep :type Boolean) (SweepResult :type Hit%20Result%20Structure%20%28by%20ref%29))
  ;[0.1216 0.902 0.6627] Reacts to the Light Orb Entering the Box and when it is overlapping it modifies the Decay Rate of the Light
  (bind _asbp_light_orb (Utilities|Casting|CastToBP_LightOrb OtherActor))
  (bind _output_get (Variables|Default|SetLightOrbRef _asbp_light_orb))
  (Variables|/Game/MechanicsPlayground/MechanincsBlueprints/BP_LightOrb.BP_LightOrb_C|SetLevelOrbDecayModifier _output_get (Variables|Default|GetLevel%20Orb%20Decay%20Modifier))
  (Variables|Default|SetbIsActivated true))

(event EventBeginPlay)

(event EventInfluencingPlayer
  (params (PlayerRef :type BP%20Third%20Person%20Character%20Object%20Reference) (bIsInRange :type Boolean))
  ;[1 1 1] Death Connection
  (Development|PrintString "Player Is Influenced by LightImpactArea "))

(event EventTick
  (params (DeltaSeconds :type Float%20%28single-precision%29))
  (bind _lightorbref (Variables|Default|GetLightOrbRef))
  ;[0.1216 0.902 0.6627] Event Tick that decays the light while it is inside this area
  (if (Variables|Default|GetbIsActivated)
    (if (Math|Float|NearlyEqual(Float) (Class|Actor|GetActorTickInterval _lightorbref) 1e+01 0.02)
      (bind _lightorbstatus (Default|GetLightOrbStrength _lightorbref))
      (Default|SetLightOrbStrength _lightorbref (- _lightorbstatus 0.1)))))

(event EventPlayerDeath
  (params (DyingPlayerReference :type BP%20Third%20Person%20Character%20Object%20Reference))
  ;[1 1 1] Death Connection
  (Development|PrintString "Player dying because of LightImpactArea"))

(fn ConstructionScript)

(fn IsInfluencingthePlayer
  (params (PlayerRef :type BP%20Third%20Person%20Character%20Object%20Reference))
  ;[1 1 1] WIP
  (return true))