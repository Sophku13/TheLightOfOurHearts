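; Disappearing block that changes visibility and collision as a BP_LightOrb enters or leaves its Box.
; Each overlap creates a dynamic instance of the ghost material on DisappearCube and plays a timeline that drives its opacity.
; Timeline updates disable collision after begin overlap and restore it after end overlap, acting on the same Box that detects the orb.
; A separate InfluenceLightOrb event calls LightPulsing on a given orb.
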(event OnComponentBeginOverlap(Box)
  (params (OverlappedComponent :type Primitive%20Component%20Object%20Reference) (OtherActor :type Actor%20Object%20Reference) (OtherComp :type Primitive%20Component%20Object%20Reference) (OtherBodyIndex :type Integer) (bFromSweep :type Boolean) (SweepResult :type Hit%20Result%20Structure%20%28by%20ref%29))
  ;[0.1216 0.902 0.6627] On the end of the Hitbox Collision the Cube hides itself and becomes non collidable
  ;;[0.1216 0.902 0.6627] Checking if the LightOrb is entering the range of the Block Collision Box
  (Utilities|Casting|CastToBP_LightOrb OtherActor)
  ;;[1 0.9833 0.5045] Dynamic material
  (bind _returnvalue (Rendering|Material|CreateDynamicMaterialInstance (Variables|Default|GetDisappearCube) 0 "/Game/VFX_EnvironmentFX/GhostOutliner/ParentMaterial/M_ghost_disappear.M_ghost_disappear" "None" :!class /Script/Engine.PrimitiveComponent))
  (bind _opacity_change (Timeline|Opacity Play)
    (:Update
      (Rendering|Material|SetScalarParameterValue _returnvalue "Dynamic_opacity" _opacity_change :!class /Script/Engine.MaterialInstanceDynamic)
      (Collision|SetCollisionEnabled (Variables|Default|GetBox) "NoCollision"))))

(event OnComponentEndOverlap(Box)
  (params (OverlappedComponent :type Primitive%20Component%20Object%20Reference) (OtherActor :type Actor%20Object%20Reference) (OtherComp :type Primitive%20Component%20Object%20Reference) (OtherBodyIndex :type Integer))
  ;[0.1216 0.902 0.6627] On Hitbox Collision the Cube reveals itself and becomes collidable
  ;;[0.1216 0.902 0.6627] Checking if the LightOrb is Leaving the range of the BlockCollisionBox
  (Utilities|Casting|CastToBP_LightOrb OtherActor)
  ;;[0.9978 1 0.452] Gradually visible
  (bind _returnvalue (Rendering|Material|CreateDynamicMaterialInstance (Variables|Default|GetDisappearCube) 0 "/Game/VFX_EnvironmentFX/GhostOutliner/ParentMaterial/M_ghost_disappear.M_ghost_disappear" "None" :!class /Script/Engine.PrimitiveComponent))
  (bind _opacity_change (Timeline|Timeline Play)
    (:Update
      (Rendering|Material|SetScalarParameterValue _returnvalue "Dynamic_opacity" _opacity_change :!class /Script/Engine.MaterialInstanceDynamic)
      (Collision|SetCollisionEnabled (Variables|Default|GetBox) "QueryAndPhysics"))))

(event EventInfluenceLightOrb
  (params (LightOrbRef :type BP%20Light%20Orb%20Object%20Reference) (IsActive :type Boolean))
  ;[1 1 1] Comment
  (Default|LightPulsing LightOrbRef))

(fn ConstructionScript)