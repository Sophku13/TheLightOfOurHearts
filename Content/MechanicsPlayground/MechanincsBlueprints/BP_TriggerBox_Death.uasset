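; BP_TriggerBox_Death is a death trigger box, placed below the level, for players who fall into it.
; Its own overlap event is empty, so it reacts to InfluencingPlayer and PlayerDeath calls.
; InfluencingPlayer stores the in-range state, exposed through IsInfluencingThePlayer, and opens the player's death UI when in range.
; PlayerDeath forwards the player to its DeathManagerRef's FallingTooFar, with debug prints throughout.
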(event EventBeginPlay
  ;[0.1216 0.902 0.6627] Trigger Box when Falling into it cause Player death. Currently below level only
)

(event Collision|EventActorBeginOverlap
  (params (OtherActor :type Actor%20Object%20Reference))
  ;[0.1216 0.902 0.6627] Trigger Box when Falling into it cause Player death. Currently below level only
)

(event EventTick
  (params (DeltaSeconds :type Float%20%28single-precision%29)))

(event EventPlayerDeath
  (params (DyingPlayerReference :type BP%20Third%20Person%20Character%20Object%20Reference))
  ;[0.1216 0.902 0.6627] Comment
  (Default|FallingTooFar (Variables|/Game/ThirdPerson/Blueprints/BP_ThirdPersonCharacter.BP_ThirdPersonCharacter_C|GetDeathManagerRef DyingPlayerReference) DyingPlayerReference)
  (Development|PrintString "You Died to the TriggerBox_Death"))

(event EventInfluencingPlayer
  (params (PlayerRef :type BP%20Third%20Person%20Character%20Object%20Reference) (bIsInRange :type Boolean))
  ;[0.1216 0.902 0.6627] Comment
  (bind _output_get (Variables|Default|SetbIsInfluencing bIsInRange))
  (if _output_get
    (Development|PrintString "Goings On while Player is Influenced by this deathbox")
    (Default|OpenDeathUI PlayerRef self)))

(fn ConstructionScript)

(fn IsInfluencingthePlayer
  (params (PlayerRef :type BP%20Third%20Person%20Character%20Object%20Reference))
  (return (Variables|Default|GetbIsInfluencing)))