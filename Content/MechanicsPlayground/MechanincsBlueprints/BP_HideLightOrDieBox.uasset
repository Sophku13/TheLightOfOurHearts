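; BP_HideLightOrDieBox is a hazard area that kills the player through the LightOrb's death if the orb is not hidden.
; When the character enters DeathBox, it caches the player and their LightOrb reference and enables actor Tick.
; Each tick, an unhidden orb gets a negative strength passed to it and its conditions updated.
; Tick is switched off when the LightOrb, rather than the character, leaves the box.
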(event OnComponentBeginOverlap(DeathBox)
  (params (OverlappedComponent :type Primitive%20Component%20Object%20Reference) (OtherActor :type Actor%20Object%20Reference) (OtherComp :type Primitive%20Component%20Object%20Reference) (OtherBodyIndex :type Integer) (bFromSweep :type Boolean) (SweepResult :type Hit%20Result%20Structure%20%28by%20ref%29))
  ;[0.1216 0.902 0.6627] If the character if entering the area the tick will start
  (bind _asbp_third_person_character (Utilities|Casting|CastToBP_ThirdPersonCharacter OtherActor))
  (bind _output_get (Variables|Default|SetPlayerRef _asbp_third_person_character))
  (Variables|Default|SetLightOrbRef (Variables|/Game/ThirdPerson/Blueprints/BP_ThirdPersonCharacter.BP_ThirdPersonCharacter_C|GetBP_LightOrbRef _output_get))
  (Actor|Tick|SetActorTickEnabled true))

(event OnComponentEndOverlap(DeathBox)
  (params (OverlappedComponent :type Primitive%20Component%20Object%20Reference) (OtherActor :type Actor%20Object%20Reference) (OtherComp :type Primitive%20Component%20Object%20Reference) (OtherBodyIndex :type Integer))
  ;[0.1216 0.902 0.6627] If the Light is Leaving the range we are disabling the tick again so it does not run forever
  (Utilities|Casting|CastToBP_LightOrb OtherActor)
  (Actor|Tick|SetActorTickEnabled false))

(event EventBeginPlay)

(event Collision|EventActorBeginOverlap
  (params (OtherActor :type Actor%20Object%20Reference)))

(event EventTick
  (params (DeltaSeconds :type Float%20%28single-precision%29))
  ;[0.1216 0.902 0.6627] Tick is checking if the LightOrb is hidden or not. If not the character dies through the LightOrb dying.
  ; REMINDER: This is only active when the character is inside of the Area
  (Variables|Default|SetLightOrbRef (Variables|/Game/ThirdPerson/Blueprints/BP_ThirdPersonCharacter.BP_ThirdPersonCharacter_C|GetBP_LightOrbRef (Variables|Default|GetPlayerRef)))
  (if (not (Variables|/Game/MechanicsPlayground/MechanincsBlueprints/BP_LightOrb.BP_LightOrb_C|GetStatusHidden (Variables|Default|GetLightOrbRef)))
    (Default|SetLightOrbStrength (Variables|Default|GetLightOrbRef) -1.0)
    (Default|SetLightOrbConditions (Variables|Default|GetLightOrbRef))))

(fn ConstructionScript)