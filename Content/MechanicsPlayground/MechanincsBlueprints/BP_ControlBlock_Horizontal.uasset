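; Horizontal control block that the player slides along its forward vector while a sufficiently strong light orb is within its trigger box.
; Box overlap toggles ticking and the character's control permission.
; A macro maps orb strength to light and highlight tiers, allowing control only at the top tier.
; While the character controls and moves, Tick reads the forward/backward axis sign and nudges the cube using VInterpTo, without sweep.
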(event OnComponentBeginOverlap(Box)
  (params (OverlappedComponent :type Primitive%20Component%20Object%20Reference) (OtherActor :type Actor%20Object%20Reference) (OtherComp :type Primitive%20Component%20Object%20Reference) (OtherBodyIndex :type Integer) (bFromSweep :type Boolean) (SweepResult :type Hit%20Result%20Structure%20%28by%20ref%29))
  ;[0.1216 0.902 0.6627] Light Orb Overlap. Setting the Object as controllable and giving the character the ability to control
  (bind _asbp_light_orb (Utilities|Casting|CastToBP_LightOrb OtherActor))
  (bind _output_get (Variables|Default|SetBP_Light%20Orb%20Ref _asbp_light_orb))
  (bind _returnvalue (Actor|GetActorOfClass "/Game/ThirdPerson/Blueprints/BP_ThirdPersonCharacter.BP_ThirdPersonCharacter_C"))
  (bind _output_get_2 (Variables|Default|SetCharRef _returnvalue))
  (bind _lightorbstatus (Default|GetLightOrbStrength _output_get))
  (Variables|/Game/ThirdPerson/Blueprints/BP_ThirdPersonCharacter.BP_ThirdPersonCharacter_C|SetbCanControlObj _output_get_2 true)
  (Utilities|MakroAdjustVisuals _lightorbstatus)
  (Actor|Tick|SetActorTickEnabled true))

(event OnComponentEndOverlap(Box)
  (params (OverlappedComponent :type Primitive%20Component%20Object%20Reference) (OtherActor :type Actor%20Object%20Reference) (OtherComp :type Primitive%20Component%20Object%20Reference) (OtherBodyIndex :type Integer))
  (bind _charref (Variables|Default|GetCharRef))
  ;[0.1216 0.902 0.6627] Sever Connection to Light Orb to be able to reestablish it at a later moment
  (Variables|/Game/ThirdPerson/Blueprints/BP_ThirdPersonCharacter.BP_ThirdPersonCharacter_C|SetbCanControlObj _charref false)
  (Variables|/Game/ThirdPerson/Blueprints/BP_ThirdPersonCharacter.BP_ThirdPersonCharacter_C|SetbIsControlling _charref false)
  (Variables|Default|SetbCanBeControlled false)
  (Rendering|SetVisibility (Variables|Default|GetPointLight) false false)
  (Rendering|SetVisibility (Variables|Default|GetHighlight%20FX) false false)
  (Actor|Tick|SetActorTickEnabled false))

(event EventBeginPlay
  ;[0.1216 0.902 0.6627] Create a reference to character and light orb
  (bind _returnvalue (Actor|GetActorOfClass "/Game/ThirdPerson/Blueprints/BP_ThirdPersonCharacter.BP_ThirdPersonCharacter_C"))
  (bind _output_get (Variables|Default|SetCharRef _returnvalue))
  (Variables|Default|SetBP_Light%20Orb%20Ref (Variables|/Game/ThirdPerson/Blueprints/BP_ThirdPersonCharacter.BP_ThirdPersonCharacter_C|GetBP_LightOrbRef _output_get)))

(event EventTick
  (params (DeltaSeconds :type Float%20%28single-precision%29))
  (bind _charref (Variables|Default|GetCharRef))
  (bind _charref_2 (Variables|Default|GetCharRef))
  (bind _bp_light_orb_ref (Variables|Default|GetBP_Light%20Orb%20Ref))
  ;[0.1216 0.902 0.6627] Checking if the Character is controlling. If yes it starts to move the object according to the left and right inputs of the character
  (if (not (Variables|/Game/MechanicsPlayground/MechanincsBlueprints/BP_LightOrb.BP_LightOrb_C|GetbIsDead _bp_light_orb_ref))
    (bind _lightorbstatus (Default|GetLightOrbStrength _bp_light_orb_ref))
    (if (!= _lightorbstatus (Variables|Default|GetfLight%20Orb%20Status))
      (bind _output_get (Variables|Default|SetfLight%20Orb%20Status _lightorbstatus))
      (Utilities|MakroAdjustVisuals _output_get))
    (if (Variables|Default|GetbCanBeControlled)
      (if (Variables|/Game/ThirdPerson/Blueprints/BP_ThirdPersonCharacter.BP_ThirdPersonCharacter_C|GetbCanControlObj _charref_2)
        (if (Variables|/Game/ThirdPerson/Blueprints/BP_ThirdPersonCharacter.BP_ThirdPersonCharacter_C|GetbIsControlling _charref_2)
          (bind _lightorbstatus_2 (Default|GetLightOrbStrength (Variables|Default|GetBP_Light%20Orb%20Ref)))
          (bind _output_get_2 (Variables|Default|SetfLight%20Orb%20Status _lightorbstatus_2))
          (Utilities|MakroAdjustVisuals _output_get_2)
          (if (>= _output_get_2 3.0)
            (if (Variables|/Game/ThirdPerson/Blueprints/BP_ThirdPersonCharacter.BP_ThirdPersonCharacter_C|GetbIsMoving _charref)
              ;;[0.1216 0.902 0.6627] Move the object
              (if (> (Variables|/Game/ThirdPerson/Blueprints/BP_ThirdPersonCharacter.BP_ThirdPersonCharacter_C|GetfForwardBackwardAxis _charref) 0.0)
                (Utilities|MakroMoveDirection true 5e+01)
                (else
                  (Utilities|MakroMoveDirection true -5e+01))))))))))

(fn ConstructionScript)