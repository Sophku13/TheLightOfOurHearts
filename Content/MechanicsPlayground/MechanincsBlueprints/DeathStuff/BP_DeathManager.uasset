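; BP_DeathManager handles the player's deaths from water, falling, eating the light, enemies and loss of light or darkness.
; On BeginPlay it registers itself on the player character, and each cause has its own event taking a player reference.
; Events set a cause message and variously play a death sound, disable input, play a montage or enable ragdoll physics.
; All end in OpeningDeathUI, which pauses the game and shows CWBP_Respawn with that message.
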(event Custom|EatingTooMuch
  (params (PlayerRef :type BP%20Third%20Person%20Character%20Object%20Reference))
  ;[0.1216 0.902 0.6627] Eating Death
  (Variables|Default|SetbIsLight true)
  (Default|DeadbyEatenLight PlayerRef)
  (Utilities|FlowControl|Delay 2.0)
  ;;[1 0.4212 0.3012] Death sound  whatever that will be
  (Audio|PlaySound2D "/Game/Audio/RawAudioFiles/lioh_death1.lioh_death1" 1.0 1.0 0.0 0 0)
  (Input|DisableInput PlayerRef (Game|GetPlayerController 0))
  (Animation|PlayAnimMontage PlayerRef "/Game/Characters/TlooH_Character2/Animations/newAnimation/death_light_Anim_Montage.death_light_Anim_Montage" 1.0 "None")
  (Utilities|FlowControl|Delay 3.08)
  ;;[1 0.5009 0.4211] Open death ui screen and print message?
  (Variables|Default|SetDeathCauseString "The Light was eaten for too long and dissolved you from the inside")
  (CallFunction|OpeningDeathUI PlayerRef)
  (Variables|Default|SetbIsLight false))

(event Custom|VantaDeath
  (params (PlayerRef :type BP%20Third%20Person%20Character%20Object%20Reference))
  ;[1 0.267 0 0.717] Enemy deaths
  ;;[0.1216 0.902 0.6627] Goo Death
  (Variables|Default|SetbIsDarkness true)
  ;;;[1 0.4212 0.3012] Death sound  whatever that will be
  (Audio|PlaySound2D "/Game/Audio/RawAudioFiles/lioh_death1.lioh_death1" 1.0 1.0 0.0 0 0)
  (Input|DisableInput PlayerRef (Game|GetPlayerController 0))
  (bind _returnvalue (Animation|PlayAnimMontage PlayerRef "/Game/Characters/TlooH_Character2/Animations/newAnimation/death_darkness_Anim_Montage.death_darkness_Anim_Montage" 1.0 "None"))
  ;;;[1 0.5009 0.4211] Open death ui screen and print message?
  (Utilities|FlowControl|Delay _returnvalue)
  (Variables|Default|SetDeathCauseString "The Vanta swallowed the light and your life essence")
  (CallFunction|OpeningDeathUI PlayerRef)
  (Variables|Default|SetbIsDarkness false))

(event Custom|Light%20Death
  (params (PlayerRef :type BP%20Third%20Person%20Character%20Object%20Reference))
  ;[1 0.8917 0.002064] Loss of light
  (Variables|Default|SetbIsDarkness true)
  ;;[1 0.4212 0.3012] Death sound  whatever that will be
  (Audio|PlaySound2D "/Game/Audio/RawAudioFiles/lioh_death1.lioh_death1" 1.0 1.0 0.0 0 0)
  (Input|DisableInput PlayerRef (Game|GetPlayerController 0))
  (bind _returnvalue (Animation|PlayAnimMontage PlayerRef "/Game/Characters/TlooH_Character2/Animations/newAnimation/death_darkness_Anim_Montage1.death_darkness_Anim_Montage1" 1.0 "None"))
  (Utilities|FlowControl|Delay _returnvalue)
  ;;[1 0.5009 0.4211] Open death ui screen and print message?
  (Variables|Default|SetDeathCauseString "Your Light died and you got taken over by the darkness.")
  (CallFunction|OpeningDeathUI PlayerRef)
  (Variables|Default|SetbIsDarkness false))

(event Custom|FallingTooFar
  (params (PlayerRef :type BP%20Third%20Person%20Character%20Object%20Reference))
  ;[0.9451 0.04314 1] Comment
  (Physics|SetSimulatePhysics (Variables|/Script/Engine.Character|GetMesh PlayerRef) true)
  (Utilities|FlowControl|Delay 1.0)
  (Variables|Default|SetDeathCauseString "You died because you hit the ground too hard")
  (CallFunction|OpeningDeathUI PlayerRef))

(event Custom|Mold%20Death
  (params (PlayerRef :type BP%20Third%20Person%20Character%20Object%20Reference))
  ;[1 0.267 0 0.717] Enemy deaths
  ;;[0.1216 0.902 0.6627] Mold Death
  (Variables|Default|SetbIsDarkness true)
  ;;;[1 0.4212 0.3012] Death sound  whatever that will be
  (Audio|PlaySound2D "/Game/Audio/RawAudioFiles/lioh_death1.lioh_death1" 1.0 1.0 0.0 0 0)
  (Input|DisableInput PlayerRef (Game|GetPlayerController 0))
  (bind _returnvalue (Animation|PlayAnimMontage PlayerRef "/Game/Characters/TlooH_Character2/Animations/newAnimation/death_darkness_Anim_Montage.death_darkness_Anim_Montage" 1.0 "None"))
  ;;;[1 0.5009 0.4211] Open death ui screen and print message?
  (Utilities|FlowControl|Delay _returnvalue)
  (Variables|Default|SetDeathCauseString "The Mold smothered you to death")
  (CallFunction|OpeningDeathUI PlayerRef)
  (Variables|Default|SetbIsDarkness false))

(event Custom|WateryDeath
  (params (PlayerRef :type BP%20Third%20Person%20Character%20Object%20Reference))
  ;[0.9451 0.04314 1] Water Deaths
  (if (Variables|/Game/MechanicsPlayground/MechanincsBlueprints/BP_LightOrb.BP_LightOrb_C|GetbIsHeld (Variables|/Game/ThirdPerson/Blueprints/BP_ThirdPersonCharacter.BP_ThirdPersonCharacter_C|GetBP_LightOrbRef PlayerRef))
    (Variables|Default|SetDeathCauseString "You died, because the Water extinguished your Light. Make sure to keep it dry!")
    (else
      (Variables|Default|SetDeathCauseString "You drowned")))
  ;;[1 0.4212 0.3012] Death sound  whatever that will be
  (Audio|PlaySound2D "/Game/Audio/RawAudioFiles/lioh_death1.lioh_death1" 1.0 1.0 0.0 0 0)
  ;;[1 0.5009 0.4211] Open death ui screen and print message?
  (CallFunction|OpeningDeathUI PlayerRef))

(event Custom|Goo%20Death
  (params (PlayerRef :type BP%20Third%20Person%20Character%20Object%20Reference))
  ;[1 0.267 0 0.717] Enemy deaths
  ;;[0.1216 0.902 0.6627] Goo Death
  (Variables|Default|SetbIsDarkness true)
  ;;;[1 0.4212 0.3012] Death sound  whatever that will be
  (Audio|PlaySound2D "/Game/Audio/RawAudioFiles/lioh_death1.lioh_death1" 1.0 1.0 0.0 0 0)
  (Input|DisableInput PlayerRef (Game|GetPlayerController 0))
  (bind _returnvalue (Animation|PlayAnimMontage PlayerRef "/Game/Characters/TlooH_Character2/Animations/newAnimation/death_darkness_Anim_Montage1.death_darkness_Anim_Montage1" 1.0 "None"))
  ;;;[1 0.5009 0.4211] Open death ui screen and print message?
  (Utilities|FlowControl|Delay _returnvalue)
  (Variables|Default|SetDeathCauseString "The Goo caught up to you and killed you")
  (CallFunction|OpeningDeathUI PlayerRef)
  (Variables|Default|SetbIsDarkness false))

(event Custom|DarknessSurrounding
  (params (PlayerRef :type BP%20Third%20Person%20Character%20Object%20Reference))
  ;[1 0.8917 0.002064] Loss of light
  ;;[1 1 1] Darkness Surrounding
  (Variables|Default|SetbIsDarkness true)
  ;;;[1 0.4212 0.3012] Death sound  whatever that will be
  (Audio|PlaySound2D "/Game/Audio/RawAudioFiles/lioh_death1.lioh_death1" 1.0 1.0 0.0 0 0)
  (Input|DisableInput PlayerRef (Game|GetPlayerController 0))
  (bind _returnvalue (Animation|PlayAnimMontage PlayerRef "/Game/Characters/TlooH_Character2/Animations/newAnimation/death_darkness_Anim_Montage1.death_darkness_Anim_Montage1" 1.0 "None"))
  (Utilities|FlowControl|Delay _returnvalue)
  ;;;[1 0.5009 0.4211] Open death ui screen and print message?
  (Variables|Default|SetDeathCauseString "You died against too much darkness around")
  (CallFunction|OpeningDeathUI PlayerRef)
  (Variables|Default|SetbIsDarkness false))

(event Custom|LightAbandonment
  (params (PlayerRef :type BP%20Third%20Person%20Character%20Object%20Reference))
  ;[1 0.8917 0.002064] Loss of light
  (Variables|Default|SetbIsDarkness true)
  ;;[1 0.4212 0.3012] Death sound  whatever that will be
  (Audio|PlaySound2D "/Game/Audio/RawAudioFiles/lioh_death1.lioh_death1" 1.0 1.0 0.0 0 0)
  (Input|DisableInput PlayerRef (Game|GetPlayerController 0))
  (bind _returnvalue (Animation|PlayAnimMontage PlayerRef "/Game/Characters/TlooH_Character2/Animations/newAnimation/death_darkness_Anim_Montage1.death_darkness_Anim_Montage1" 1.0 "None"))
  (Utilities|FlowControl|Delay _returnvalue)
  ;;[1 0.5009 0.4211] Open death ui screen and print message?
  (Variables|Default|SetDeathCauseString "You died because you left your light")
  (CallFunction|OpeningDeathUI PlayerRef)
  (Variables|Default|SetbIsDarkness false))

(event EventBeginPlay
  ;[0.8887 0.902 0.892] Saving itself to the Character
  (bind _asbp_third_person_character (Utilities|Casting|CastToBP_ThirdPersonCharacter (Game|GetPlayerCharacter 0)))
  (bind _output_get (Variables|Default|SetPlayerRef _asbp_third_person_character))
  (Variables|/Game/ThirdPerson/Blueprints/BP_ThirdPersonCharacter.BP_ThirdPersonCharacter_C|SetDeathManagerRef _output_get self)
  (Variables|Default|SetIs%20Held (Variables|/Game/ThirdPerson/Blueprints/BP_ThirdPersonCharacter.BP_ThirdPersonCharacter_C|GetIs%20Held _asbp_third_person_character)))

(event Collision|EventActorBeginOverlap
  (params (OtherActor :type Actor%20Object%20Reference)))

(event EventTick
  (params (DeltaSeconds :type Float%20%28single-precision%29)))

(fn ConstructionScript)

(fn OpeningDeathUI
  (params (PlayerRef :type BP%20Third%20Person%20Character%20Object%20Reference))
  (Game|SetGamePaused true)
  ;[1 0.7126 0.6626] open widget, replace textwith given death string
  (Input|EnableInput PlayerRef (Game|GetPlayerController 0))
  (bind _returnvalue (UserInterface|CreateWidget "/Game/UI/CWBP_Respawn.CWBP_Respawn_C"))
  (UserInterface|Viewport|AddtoViewport _returnvalue 0)
  (Variables|/Script/UMG.TextBlock|SetText (Variables|/Game/UI/CWBP_Respawn.CWBP_Respawn_C|GetDeathCauseText _returnvalue) (Utilities|Text|ToText(String) (Variables|Default|GetDeathCauseString))))