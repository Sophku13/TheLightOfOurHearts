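; BP_Lever_OpenDoor is an interactable lever that activates a referenced Door.
; On interact it rotates ButtonBase1, turns green, plays a lever sound and sends the Door an OnActivation message.
; If IsActivatable is set, interaction requires a prior OnActivation call to set IsActive, which IsInteractable also reports.
; Tick reapplies the red (active) or rusty (inactive) material every frame on activatable levers, overriding the green.
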(event EventMoveButton
  (bind _button (Variables|Default|GetButton))
  ;[1 1 1] Comment
  (Rendering|Material|SetMaterial _button 0 "/Game/Materials/MI_Sphere_Emissive_Green.MI_Sphere_Emissive_Green")
  (Transformation|SetRelativeRotation (Variables|Default|GetButtonBase1) (Math|Rotator|MakeRotator 0.0 9e+01 0.0) false false)
  ;;[0 1 0.03888] Herkus was here
  (Audio|PlaySoundatLocation "/Game/Audio/Cues/lever6_by_mediatheksuche_Cue.lever6_by_mediatheksuche_Cue" (Variables|/Script/Engine.SceneComponent|GetRelativeLocation _button) "0, 0, 0" 1.0 1.0 0.0 0 0 0 0))

(event EventTick
  (params (DeltaSeconds :type Float%20%28single-precision%29))
  ;[0.1216 0.902 0.6627] Event Tick sets the material of the button only if the button is activatable in general and if the button is currently active or not
  (if (Variables|Default|GetbIsActivatable)
    (if (Variables|Default|GetbIsActive)
      (Rendering|Material|SetMaterial (Variables|Default|GetButton) 0 "/Game/Materials/MI_Sphere_Emissive_Red.MI_Sphere_Emissive_Red")
      (else
        (Rendering|Material|SetMaterial (Variables|Default|GetButton) 0 "/Game/LevelBlockout/AssetsVlad/Materials/Rust_handpaint/MI_RustHandPaint_Inst.MI_RustHandPaint_Inst")))))

(event EventOnActivation
  ;[0.1216 0.902 0.6627] When called activates the button
  (Variables|Default|SetbIsActive true))

(event EventOnInteract
  ;[0.1216 0.902 0.6627] On Interacted it moves the button and calls the activation of the door. If it is an activatable button then the button has to be active for this to function
  (if (Variables|Default|GetbIsActivatable)
    (if (Variables|Default|GetbIsActive)
      (CallFunction|MoveButton)
      (Class|BPILightFueledActivation|OnActivation(Message) (Variables|Default|GetDoor)))
    (else
      (CallFunction|MoveButton)
      (Class|BPILightFueledActivation|OnActivation(Message) (Variables|Default|GetDoor)))))

(fn ConstructionScript
  (|CallParentFunction))

(fn IsInteractable
  (if (Variables|Default|GetbIsActivatable)
    (return (Variables|Default|GetbIsActive))
    (else
      (return true))))