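; Lab button, a child Blueprint, that toggles the strength of the lab's light orb between two levels when interacted with.
; Interaction moves the button, runs its task and resets after a delay, blocking re-presses meanwhile.
; The task reaches the orb through the button grouper's lab reference, skips it while held, and alternates via FlipFlop.
; BeginPlay spawns a Niagara glow sign; Tick swaps the emissive material by active state.
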(event EventBeginPlay
  ;[1 1 1] Comment
  (|CallParentFunction)
  (bind _returnvalue (Game|SpawnActorfromClass "/Game/MechanicsPlayground/MechanincsBlueprints/GlowTextures/BP_TEMPLATE_BlowGlow_Base.BP_TEMPLATE_BlowGlow_Base_C" (Math|Transform|MakeTransform (+ (.location (Transformation|GetWorldTransform (Variables|Default|GetSignBase))) "0.000000,25.000000,0.000000") "0, 0, 0" "0.500000,0.500000,0.500000") "AlwaysSpawn" "MultiplyWithRoot" 0 0))
  (Variables|Default|SetSignGlow _returnvalue)
  (bind _signglow (Variables|Default|GetSignGlow)
    (:then
      (Class|NiagaraComponent|SetAsset (Variables|/Game/MechanicsPlayground/MechanincsBlueprints/GlowTextures/BP_TEMPLATE_BlowGlow_Base.BP_TEMPLATE_BlowGlow_Base_C|GetTextureGlow _signglow) "/Game/MechanicsPlayground/MechanincsBlueprints/GlowTextures/NiagaraSystems/NS_BlowRevealParticles_Lab.NS_BlowRevealParticles_Lab" false)
      (Rendering|Material|SetMaterial (Variables|Default|GetSignBase) 0 "/Game/MechanicsPlayground/MechanincsBlueprints/GlowTextures/Material/M_GlowMechanic_Lab.M_GlowMechanic_Lab"))
    (:else)))

(event Collision|EventActorBeginOverlap
  (params (OtherActor :type Actor%20Object%20Reference))
  (|CallParentFunction OtherActor) ; This node is disabled and will not be called.\nDrag off pins to build functionality.
)

(event EventTick
  (params (DeltaSeconds :type Float%20%28single-precision%29))
  ;[1 1 1] Comment
  (if (Variables|Default|GetbIsActive)
    (Rendering|Material|SetMaterial (Variables|Default|GetButton) 0 "/Game/Materials/MI_Sphere_Emissive_Red.MI_Sphere_Emissive_Red")
    (else
      (Rendering|Material|SetMaterial (Variables|Default|GetButton) 0 "/Game/Materials/MI_Sphere_Emissive_Red_Off.MI_Sphere_Emissive_Red_Off"))))

(event EventButtonTask
  (params (ButtonGroup :type BP%20Button%20Grouper%20Base%20Object%20Reference))
  ;[1 1 1] Comment
  (bind _asbp_button_grouper_lab (Utilities|Casting|CastToBP_ButtonGrouper_Lab ButtonGroup))
  (if (not (Variables|Default|GetbIsTasking))
    (Variables|Default|SetbIsTasking true)
    (if (not (Variables|/Game/MechanicsPlayground/MechanincsBlueprints/BP_LightOrb.BP_LightOrb_C|GetbIsHeld (Variables|/Game/MechanicsPlayground/MechanincsBlueprints/BP_MoveBetweenSocketsWithButtons_Lab.BP_MoveBetweenSocketsWithButtons_Lab_C|GetLightOrbRef (Variables|/Game/MechanicsPlayground/MechanincsBlueprints/Buttons/Lab/BP_Lab.BP_Lab_C|GetSocketMover (Variables|/Game/MechanicsPlayground/MechanincsBlueprints/Buttons/Lab/BP_ButtonGrouper_Lab.BP_ButtonGrouper_Lab_C|GetLabRef _asbp_button_grouper_lab)))))
      (Utilities|FlowControl|FlipFlop
        (:A
          (Variables|/Game/MechanicsPlayground/MechanincsBlueprints/BP_LightOrb.BP_LightOrb_C|SetbIsIncreasing (Variables|/Game/MechanicsPlayground/MechanincsBlueprints/BP_MoveBetweenSocketsWithButtons_Lab.BP_MoveBetweenSocketsWithButtons_Lab_C|GetLightOrbRef (Variables|/Game/MechanicsPlayground/MechanincsBlueprints/Buttons/Lab/BP_Lab.BP_Lab_C|GetSocketMover (Variables|/Game/MechanicsPlayground/MechanincsBlueprints/Buttons/Lab/BP_ButtonGrouper_Lab.BP_ButtonGrouper_Lab_C|GetLabRef _asbp_button_grouper_lab))) false)
          (Default|SetLightOrbStrength (Variables|/Game/MechanicsPlayground/MechanincsBlueprints/BP_MoveBetweenSocketsWithButtons_Lab.BP_MoveBetweenSocketsWithButtons_Lab_C|GetLightOrbRef (Variables|/Game/MechanicsPlayground/MechanincsBlueprints/Buttons/Lab/BP_Lab.BP_Lab_C|GetSocketMover (Variables|/Game/MechanicsPlayground/MechanincsBlueprints/Buttons/Lab/BP_ButtonGrouper_Lab.BP_ButtonGrouper_Lab_C|GetLabRef _asbp_button_grouper_lab))) 1.0)
          (Default|SetLightOrbConditions (Variables|/Game/MechanicsPlayground/MechanincsBlueprints/BP_MoveBetweenSocketsWithButtons_Lab.BP_MoveBetweenSocketsWithButtons_Lab_C|GetLightOrbRef (Variables|/Game/MechanicsPlayground/MechanincsBlueprints/Buttons/Lab/BP_Lab.BP_Lab_C|GetSocketMover (Variables|/Game/MechanicsPlayground/MechanincsBlueprints/Buttons/Lab/BP_ButtonGrouper_Lab.BP_ButtonGrouper_Lab_C|GetLabRef _asbp_button_grouper_lab)))))
        (:B
          (Variables|/Game/MechanicsPlayground/MechanincsBlueprints/BP_LightOrb.BP_LightOrb_C|SetbIsIncreasing (Variables|/Game/MechanicsPlayground/MechanincsBlueprints/BP_MoveBetweenSocketsWithButtons_Lab.BP_MoveBetweenSocketsWithButtons_Lab_C|GetLightOrbRef (Variables|/Game/MechanicsPlayground/MechanincsBlueprints/Buttons/Lab/BP_Lab.BP_Lab_C|GetSocketMover (Variables|/Game/MechanicsPlayground/MechanincsBlueprints/Buttons/Lab/BP_ButtonGrouper_Lab.BP_ButtonGrouper_Lab_C|GetLabRef _asbp_button_grouper_lab))) true)
          (Default|SetLightOrbStrength (Variables|/Game/MechanicsPlayground/MechanincsBlueprints/BP_MoveBetweenSocketsWithButtons_Lab.BP_MoveBetweenSocketsWithButtons_Lab_C|GetLightOrbRef (Variables|/Game/MechanicsPlayground/MechanincsBlueprints/Buttons/Lab/BP_Lab.BP_Lab_C|GetSocketMover (Variables|/Game/MechanicsPlayground/MechanincsBlueprints/Buttons/Lab/BP_ButtonGrouper_Lab.BP_ButtonGrouper_Lab_C|GetLabRef _asbp_button_grouper_lab))) 2.0)
          (Default|SetLightOrbConditions (Variables|/Game/MechanicsPlayground/MechanincsBlueprints/BP_MoveBetweenSocketsWithButtons_Lab.BP_MoveBetweenSocketsWithButtons_Lab_C|GetLightOrbRef (Variables|/Game/MechanicsPlayground/MechanincsBlueprints/Buttons/Lab/BP_Lab.BP_Lab_C|GetSocketMover (Variables|/Game/MechanicsPlayground/MechanincsBlueprints/Buttons/Lab/BP_ButtonGrouper_Lab.BP_ButtonGrouper_Lab_C|GetLabRef _asbp_button_grouper_lab))))))
      (Utilities|FlowControl|Delay 1.0)
      (Variables|Default|SetbIsTasking false)
      (else
        (Variables|Default|SetbIsTasking false)))))

(event EventOnInteract
  ;[1 1 1] Comment
  (Variables|Default|SetbIsButtonPressed true)
  (CallFunction|MoveButton)
  (CallFunction|ButtonTask (Variables|Default|GetButtonGroup))
  (Utilities|FlowControl|Delay 2.0)
  (CallFunction|MoveButton)
  (Variables|Default|SetbIsButtonPressed false)
  (|CallParentFunction))

(fn ConstructionScript
  (|CallParentFunction))

(fn IsInteractable
  (return (and (not (Variables|Default|GetbIsButtonPressed)) (Variables|Default|GetbIsActive))))