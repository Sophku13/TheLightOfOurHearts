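; Base Blueprint for bunker hints, which shows or hides a hint Plane according to an activation state.
; OnActivation flips IsActivated through a FlipFlop, starting with false.
; Tick applies that state to the Plane's visibility and runs the parent tick only while active.
; Sphere overlaps with the third-person character set the TickEnable flag on entry and clear it on exit, also caching the character on entry.
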(event OnComponentBeginOverlap(Sphere)
  (params (OverlappedComponent :type Primitive%20Component%20Object%20Reference) (OtherActor :type Actor%20Object%20Reference) (OtherComp :type Primitive%20Component%20Object%20Reference) (OtherBodyIndex :type Integer) (bFromSweep :type Boolean) (SweepResult :type Hit%20Result%20Structure%20%28by%20ref%29))
  ;[0.1216 0.902 0.6627] When overlapping with a character the tick gets enabled
  (bind _asbp_third_person_character (Utilities|Casting|CastToBP_ThirdPersonCharacter OtherActor))
  (Variables|Default|SetAs%20BP%20Third%20Person%20Character _asbp_third_person_character)
  (Variables|Default|SetTickEnable true))

(event OnComponentEndOverlap(Sphere)
  (params (OverlappedComponent :type Primitive%20Component%20Object%20Reference) (OtherActor :type Actor%20Object%20Reference) (OtherComp :type Primitive%20Component%20Object%20Reference) (OtherBodyIndex :type Integer))
  ;[0.1216 0.902 0.6627] When overlapping anymore with a character the tick gets disabled
  (Utilities|Casting|CastToBP_ThirdPersonCharacter OtherActor)
  (Variables|Default|SetTickEnable false))

(event EventBeginPlay
  ;[0.1216 0.902 0.6627] Begin Play calling code of Parent Class
  (|CallParentFunction))

(event EventTick
  (params (DeltaSeconds :type Float%20%28single-precision%29))
  (bind _plane (Variables|Default|GetPlane))
  ;[0.1216 0.902 0.6627] Event ticks sets them visible depending on if they are active or not
  (if (Variables|Default|GetbIsActivated)
    (Rendering|SetVisibility _plane true false)
    (|CallParentFunction DeltaSeconds)
    (else
      (Rendering|SetVisibility _plane false false))))

(event EventOnActivation
  ;[0.1216 0.902 0.6627] Flips the active state when the Hint activation is called
  (Utilities|FlowControl|FlipFlop
    (:A
      (Variables|Default|SetbIsActivated false))
    (:B
      (Variables|Default|SetbIsActivated true))))

(fn ConstructionScript
  (|CallParentFunction))