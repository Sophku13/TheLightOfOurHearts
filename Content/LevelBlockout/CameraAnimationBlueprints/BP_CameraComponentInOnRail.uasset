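; Rail camera Blueprint that follows the player character along a spline while ActiveCamera is set.
; Each Tick, GetClosestPositionAlongSpline samples the spline in fixed distance steps to find the point nearest the player.
; The camera then lerps toward a point FollowDistance behind it, clamped at the spline start, at a rate scaled by delta time and FollowSpeed.
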(event EventBeginPlay)

(event Collision|EventActorBeginOverlap
  (params (OtherActor :type Actor%20Object%20Reference))
  ;[1 1 1] Calling a function that calculates the position on spline that is the closest to the character and moving the camera to this posotion
)

(event EventTick
  (params (DeltaSeconds :type Float%20%28single-precision%29))
  (bind _camera (Variables|Default|GetCamera))
  ;[1 1 1] Calling a function that calculates the position on spline that is the closest to the character and moving the camera to this posotion
  (|CallParentFunction DeltaSeconds)
  (if (Variables|Default|GetActiveCamera)
    (bind _pointonsplineatclosestposition (CallFunction|GetClosestPositionAlongSpline (Transformation|GetActorLocation (Game|GetPlayerCharacter 0))))
    (Variables|Default|SetPoint%20on%20Spline%20at%20Closest%20Position _pointonsplineatclosestposition)
    (Transformation|SetWorldLocation _camera (Math|Vector|Lerp(Vector) (Transformation|GetWorldLocation _camera) (Spline|GetLocationatDistanceAlongSpline (Variables|Default|GetSpline) (Math|Float|Max(Float) (- _pointonsplineatclosestposition (Variables|Default|GetFollowDistance)) 0.0) "World") (* (Utilities|Time|GetWorldDeltaSeconds) (Variables|Default|GetFollowSpeed))) false false)))

(fn ConstructionScript
  (|CallParentFunction))

(fn GetClosestPositionAlongSpline
  (params (WhereIsTheCharacter :type Vector))
  (bind _spline (Variables|Default|GetSpline))
  (if (< (LocalVariables|GetCheckLength) (Spline|GetSplineLength _spline)) :!label _label
    (if (> (LocalVariables|GetClosestDistance) (Math|Vector|Distance(Vector) (Spline|GetLocationatDistanceAlongSpline _spline (LocalVariables|GetCheckLength) "World") WhereIsTheCharacter))
      (LocalVariables|SetClosestDistance (Math|Vector|Distance(Vector) (Spline|GetLocationatDistanceAlongSpline _spline (LocalVariables|GetCheckLength) "World") WhereIsTheCharacter))
      (LocalVariables|SetLengthAtClosestDistance (LocalVariables|GetCheckLength)))
    (LocalVariables|SetCheckLength (+ (LocalVariables|GetCheckLength) 5.0))
    (goto _label)
    (else
      (return (LocalVariables|GetLengthAtClosestDistance)))))