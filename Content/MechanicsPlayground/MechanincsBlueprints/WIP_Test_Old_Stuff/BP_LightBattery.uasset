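; BP_LightBattery is a battery that charges while the player's light orb sits in its child-actor socket.
; Each tick it matches the orb's current socket to its own by location, then maps the socket's light timer to fill-status thresholds.
; Level meshes swap materials and a full indicator toggles.
; Without the light, the same timer drives stepwise emptying, with a delayed hold at full charge before draining.
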(event EventBeginPlay
  ;[0.1216 0.902 0.6627] Gets a reference of the Socket that is in this instance of the Battery. This is needed in case there are more than one Socket in a level
  (bind _asbp_place_light_socket (Utilities|Casting|CastToBP_PlaceLightSocket (Variables|/Script/Engine.ChildActorComponent|GetChildActor (Variables|Default|GetBatterySocket))))
  (Variables|Default|SetSocketRef _asbp_place_light_socket))

(event EventTick
  (params (DeltaSeconds :type Float%20%28single-precision%29))
  (bind _socketref (Variables|Default|GetSocketRef))
  ;[0.1216 0.902 0.6627] Event Tick
  ;;[0.1216 0.902 0.6627] Checks if the Character and its Socket Reference are Valid.
  ;; Additionally checks if the location of the battery socket is in the same location as the CurrentSocket Reference of the Light Orb.
  ;; And Checks if the Light is actually still on the Socket
  (bind _playerref (Variables|/Game/MechanicsPlayground/MechanincsBlueprints/BP_PlaceLightSocket.BP_PlaceLightSocket_C|GetPlayerRef _socketref)
    (:then
      (bind _output_get (Variables|Default|SetPlayer%20Ref _playerref))
      (bind _currentsocketref (Variables|/Game/MechanicsPlayground/MechanincsBlueprints/BP_LightOrb.BP_LightOrb_C|GetCurrentSocketRef (Variables|/Game/ThirdPerson/Blueprints/BP_ThirdPersonCharacter.BP_ThirdPersonCharacter_C|GetBP_LightOrbRef _output_get))
        (:then
          (bind _locationofsocket (CallFunction|GetSocketLocation _currentsocketref))
          (if (Utilities|Operators|EqualEqual _locationofsocket (Variables|/Game/MechanicsPlayground/MechanincsBlueprints/BP_PlaceLightSocket.BP_PlaceLightSocket_C|GetLocationOfSocket _socketref) 1.0)
            (if (Variables|/Game/MechanicsPlayground/MechanincsBlueprints/BP_PlaceLightSocket.BP_PlaceLightSocket_C|GetbLightOnSocket _socketref)
              ;;[0.1216 0.902 0.6627] Loading the Battery
              ;;;[0.1216 0.902 0.6627] Filling Status 0 = Empty
              (if (> (Variables|/Game/MechanicsPlayground/MechanincsBlueprints/BP_PlaceLightSocket.BP_PlaceLightSocket_C|GetTimeOfLightInSocket (Variables|Default|GetSocketRef)) 2)
                ;;;[0.1216 0.902 0.6627] Filling Status 1 = Low; From here on and higher always activating the next battery level visualizer so far
                (if (> (Variables|/Game/MechanicsPlayground/MechanincsBlueprints/BP_PlaceLightSocket.BP_PlaceLightSocket_C|GetTimeOfLightInSocket (Variables|Default|GetSocketRef)) 4)
                  ;;;[0.1216 0.902 0.6627] Filling Status 2 = Medium
                  (if (> (Variables|/Game/MechanicsPlayground/MechanincsBlueprints/BP_PlaceLightSocket.BP_PlaceLightSocket_C|GetTimeOfLightInSocket (Variables|Default|GetSocketRef)) 6)
                    ;;;[0.1216 0.902 0.6627] Filling Status 3 = High
                    (if (> (Variables|/Game/MechanicsPlayground/MechanincsBlueprints/BP_PlaceLightSocket.BP_PlaceLightSocket_C|GetTimeOfLightInSocket (Variables|Default|GetSocketRef)) 8)
                      (if (> (Variables|/Game/MechanicsPlayground/MechanincsBlueprints/BP_PlaceLightSocket.BP_PlaceLightSocket_C|GetTimeOfLightInSocket (Variables|Default|GetSocketRef)) 10)
                        ;;;[0.1216 0.902 0.6627] Filling Status 5 = Full
                        (Rendering|SetVisibility (Variables|Default|GetFullyLoaded) true false)
                        (Variables|Default|SetFillingStatus 5)
                        (Variables|Default|SetbIsFullyLoaded true)
                        (else
                          ;;;[0.1216 0.902 0.6627] Filling Status 4 = Almost Full
                          (Rendering|Material|SetMaterial (Variables|Default|GetBatteryLevel4) 0 "/Game/VFX_EnvironmentFX/Light_Reflection/M_Beam.M_Beam")
                          (Variables|Default|SetFillingStatus 4)))
                      (else
                        (Rendering|Material|SetMaterial (Variables|Default|GetBatteryLevel3) 0 "/Game/VFX_EnvironmentFX/Light_Reflection/M_Beam.M_Beam")
                        (Variables|Default|SetFillingStatus 3)))
                    (else
                      (Rendering|Material|SetMaterial (Variables|Default|GetBatteryLevel2) 0 "/Game/VFX_EnvironmentFX/Light_Reflection/M_Beam.M_Beam")
                      (Variables|Default|SetFillingStatus 2)))
                  (else
                    (Rendering|Material|SetMaterial (Variables|Default|GetBatteryLevel1) 0 "/Game/VFX_EnvironmentFX/Light_Reflection/M_Beam.M_Beam")
                    (Variables|Default|SetFillingStatus 1)))
                (else
                  (Variables|Default|SetFillingStatus 0)
                  (Variables|Default|SetbIsEmpty false)))
              (else
                ;;[0.1216 0.902 0.6627] Emptying the Battery over time
                ;;;[0.1216 0.902 0.6627] Empty
                (if (< (Variables|/Game/MechanicsPlayground/MechanincsBlueprints/BP_PlaceLightSocket.BP_PlaceLightSocket_C|GetTimeOfLightInSocket (Variables|Default|GetSocketRef)) 1) :!label _label
                  (Variables|Default|SetbIsEmpty true)
                  (else
                    ;;;[0.1216 0.902 0.6627] Filling Status 0 = Moving to empty
                    (if (< (Variables|/Game/MechanicsPlayground/MechanincsBlueprints/BP_PlaceLightSocket.BP_PlaceLightSocket_C|GetTimeOfLightInSocket (Variables|Default|GetSocketRef)) 2)
                      (Rendering|Material|SetMaterial (Variables|Default|GetBatteryLevel1) 0 "/Game/VFX_EnvironmentFX/Light_VFX/shaderTest/M_Orb.M_Orb")
                      (Variables|Default|SetFillingStatus 0)
                      (else
                        ;;;[0.1216 0.902 0.6627] Filling Status 1 = Moving to Low
                        (if (< (Variables|/Game/MechanicsPlayground/MechanincsBlueprints/BP_PlaceLightSocket.BP_PlaceLightSocket_C|GetTimeOfLightInSocket (Variables|Default|GetSocketRef)) 4)
                          (Rendering|Material|SetMaterial (Variables|Default|GetBatteryLevel2) 0 "/Game/VFX_EnvironmentFX/Light_VFX/shaderTest/M_Orb.M_Orb")
                          (Variables|Default|SetFillingStatus 1)
                          (else
                            ;;;[0.1216 0.902 0.6627] Filling Status 2 = Moving to Medium
                            (if (< (Variables|/Game/MechanicsPlayground/MechanincsBlueprints/BP_PlaceLightSocket.BP_PlaceLightSocket_C|GetTimeOfLightInSocket (Variables|Default|GetSocketRef)) 6)
                              (Rendering|Material|SetMaterial (Variables|Default|GetBatteryLevel3) 0 "/Game/VFX_EnvironmentFX/Light_VFX/shaderTest/M_Orb.M_Orb")
                              (Variables|Default|SetFillingStatus 2)
                              (else
                                ;;;[0.1216 0.902 0.6627] First Status 3 = Moving to High
                                (if (< (Variables|/Game/MechanicsPlayground/MechanincsBlueprints/BP_PlaceLightSocket.BP_PlaceLightSocket_C|GetTimeOfLightInSocket (Variables|Default|GetSocketRef)) 8)
                                  (Rendering|Material|SetMaterial (Variables|Default|GetBatteryLevel4) 0 "/Game/VFX_EnvironmentFX/Light_VFX/shaderTest/M_Orb.M_Orb")
                                  (Variables|Default|SetFillingStatus 3)
                                  (else
                                    ;;;[0.1216 0.902 0.6627] Filling Status 4 = Starting to lose Charge
                                    (if (< (Variables|/Game/MechanicsPlayground/MechanincsBlueprints/BP_PlaceLightSocket.BP_PlaceLightSocket_C|GetTimeOfLightInSocket (Variables|Default|GetSocketRef)) 10)
                                      (Rendering|SetVisibility (Variables|Default|GetFullyLoaded) false false)
                                      (Variables|Default|SetbIsFullyLoaded false)
                                      (Variables|Default|SetFillingStatus 4)
                                      (else
                                        ;;;[0.1216 0.902 0.6627] Holding the Charge when full for a set amount of seconds before starting the losing of charge
                                        (Utilities|FlowControl|Delay 7.0)
                                        (Variables|/Game/MechanicsPlayground/MechanincsBlueprints/BP_PlaceLightSocket.BP_PlaceLightSocket_C|SetTimeOfLightInSocket (Variables|Default|GetSocketRef) 9)))))))))))))))
            (else
              (goto _label))))
        (:else
          (goto _label))))
    (:else)))

(fn ConstructionScript)

(fn GetSocketLocation
  (params (SocketRef :type BP%20Place%20Light%20Socket%20Object%20Reference))
  ;[0.1216 0.902 0.6627] Just a function to make the getting of the Socket Location a bit more streamlined
  (return (Variables|/Game/MechanicsPlayground/MechanincsBlueprints/BP_PlaceLightSocket.BP_PlaceLightSocket_C|GetLocationOfSocket SocketRef)))