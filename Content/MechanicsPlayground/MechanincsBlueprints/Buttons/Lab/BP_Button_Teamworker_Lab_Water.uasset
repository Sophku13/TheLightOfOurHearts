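; Lab button Blueprint that, when interacted with, sends an activation message to its LabWater reference.
; It extends a parent button, running the parent interaction first, then after a three-second delay calls MoveButton and clears the pressed state.
; Tick swaps the button material between lit and unlit red emissive based on IsActive, and the button always reports itself as interactable.
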(event EventBeginPlay
  (|CallParentFunction) ; This node is disabled and will not be called.\nDrag off pins to build functionality.
)

(event Collision|EventActorBeginOverlap
  (params (OtherActor :type Actor%20Object%20Reference))
  (|CallParentFunction OtherActor) ; This node is disabled and will not be called.\nDrag off pins to build functionality.
)

(event EventTick
  (params (DeltaSeconds :type Float%20%28single-precision%29))
  (if (Variables|Default|GetbIsActive)
    (Rendering|Material|SetMaterial (Variables|Default|GetButton) 0 "/Game/Materials/MI_Sphere_Emissive_Red.MI_Sphere_Emissive_Red")
    (else
      (Rendering|Material|SetMaterial (Variables|Default|GetButton) 0 "/Game/Materials/MI_Sphere_Emissive_Red_Off.MI_Sphere_Emissive_Red_Off"))))

(event EventInfluenceLightOrb
  (params (LightOrbRef :type BP%20Light%20Orb%20Object%20Reference) (IsActive :type Boolean))
  (|CallParentFunction LightOrbRef IsActive))

(event EventOnInteract
  (|CallParentFunction)
  (Class|BPILightFueledActivation|OnActivation(Message) (Variables|Default|GetLabWater))
  (Utilities|FlowControl|Delay 3.0)
  (CallFunction|MoveButton)
  (Variables|Default|SetbIsButtonPressed false))

(fn ConstructionScript
  (|CallParentFunction))

(fn IsInteractable
  (return true))