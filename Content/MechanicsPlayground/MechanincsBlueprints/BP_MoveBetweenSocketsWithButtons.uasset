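; Puzzle actor that carries a light orb from a start socket to an end socket in discrete steps, apparently driven by buttons.
; BeginPlay splits the path into step coordinates; Tick detects the socketed orb, makes the first move and pauses its decay.
; MoveOrbToEnd and MoveOrbToStart lerp it via timelines, tracking completed steps.
; On the last step, orb strength is restored and socket state passes to the end socket.
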(event Custom|MoveOrbToStart
  (params (FromVector :type Vector) (ToVector :type Vector))
  ;[0.1216 0.902 0.6627] Is moving the light in the direction of the start socket from the end socket
  (if (not (Variables|Default|GetbIsMoving))
    (Variables|Default|SetbIsMoving true)
    (bind _newtrack_0 (Timeline|ReverseMoveLightFromStartToEnd PlayFromStart)
      (:Update
        (Transformation|SetActorLocation (Variables|Default|GetLightOrbRef) (Math|Vector|Lerp(Vector) FromVector ToVector _newtrack_0) false false))
      (:Finished
        (Variables|Default|SetbIsMoving false)
        (Variables|Default|SetstepsCompleted (- (Variables|Default|GetstepsCompleted) 1))))))

(event Custom|MoveOrbToEnd
  (params (FromVector :type Vector) (ToVector :type Vector))
  ;[0.1216 0.902 0.6627] Is Moving from the start socket in the direction of the end socket.
  (if (not (Variables|Default|GetbIsMoving))
    (Variables|Default|SetbIsMoving true)
    (bind _newtrack_0 (Timeline|MoveLightFromStartToEnd PlayFromStart)
      (:Update
        (Transformation|SetActorLocation (Variables|Default|GetLightOrbRef) (Math|Vector|Lerp(Vector) FromVector ToVector _newtrack_0) false false))
      (:Finished
        (Variables|Default|SetbIsMoving false)
        (bind _output_get (Variables|Default|SetstepsCompleted (+ (Variables|Default|GetstepsCompleted) 1)))
        (if (== (Variables|Default|Getsteps) _output_get)
          (CallFunction|EndReached))))))

(event Custom|EndReached
  (bind _startsocket (Variables|Default|GetStartSocket))
  (bind _lightorbref (Variables|Default|GetLightOrbRef))
  ;[0.1216 0.902 0.6627] Tells the end socket that it is now carrying the Light orb and the player can take it away
  (CallFunction|ExchangeValues (Variables|Default|GetEndSocket) (Variables|Default|GetStartSocket))
  (Variables|/Game/MechanicsPlayground/MechanincsBlueprints/BP_PlaceLightSocket.BP_PlaceLightSocket_C|SetbLightOnSocket _startsocket false)
  (Default|SetLightOrbStrength _lightorbref (Variables|Default|GetLightOrbStrengthSave))
  (Variables|/Game/MechanicsPlayground/MechanincsBlueprints/BP_LightOrb.BP_LightOrb_C|SetbDecayIsOnHold _lightorbref false)
  (Actor|Tick|SetActorTickEnabled _startsocket))

(event EventBeginPlay
  (bind _steps (Variables|Default|Getsteps))
  (bind _tempcoord (Variables|Default|GetTempCoord))
  (bind _returnvalue (- _steps 1))
  ;[0.1216 0.902 0.6627] Begin Play. Saves the new interval paths and the start and end location and adds the coordinated to a list
  (Variables|Default|SetbuttonStationsCount _returnvalue)
  (Variables|Default|SetIntervalPath (/ (- (Variables|/Game/MechanicsPlayground/MechanincsBlueprints/BP_PlaceLightSocket.BP_PlaceLightSocket_C|GetLocationOfSocket (Variables|Default|GetEndSocket)) (Variables|/Game/MechanicsPlayground/MechanincsBlueprints/BP_PlaceLightSocket.BP_PlaceLightSocket_C|GetLocationOfSocket (Variables|Default|GetStartSocket))) (Variables|Default|Getsteps)))
  (for _index (range 0 _returnvalue)
    (Variables|/Game/MechanicsPlayground/MechanincsBlueprints/Buttons/Bases/BP_CoordinateVtoV.BP_CoordinateVtoV_C|SetStartLocation _tempcoord (+ (* (Variables|Default|GetIntervalPath) _index) (Variables|/Game/MechanicsPlayground/MechanincsBlueprints/BP_PlaceLightSocket.BP_PlaceLightSocket_C|GetLocationOfSocket (Variables|Default|GetStartSocket))))
    (Variables|/Game/MechanicsPlayground/MechanincsBlueprints/Buttons/Bases/BP_CoordinateVtoV.BP_CoordinateVtoV_C|SetEndLocation _tempcoord (+ (+ (* (Variables|Default|GetIntervalPath) _index) (Variables|/Game/MechanicsPlayground/MechanincsBlueprints/BP_PlaceLightSocket.BP_PlaceLightSocket_C|GetLocationOfSocket (Variables|Default|GetStartSocket))) (Variables|Default|GetIntervalPath)))
    (Utilities|Map|Add (Variables|Default|GetCoordinates) _index _tempcoord)))

(event Collision|EventActorBeginOverlap
  (params (OtherActor :type Actor%20Object%20Reference)))

(event EventTick
  (params (DeltaSeconds :type Float%20%28single-precision%29))
  (bind _startsocket (Variables|Default|GetStartSocket))
  (bind _locationofsocket (Variables|/Game/MechanicsPlayground/MechanincsBlueprints/BP_PlaceLightSocket.BP_PlaceLightSocket_C|GetLocationOfSocket _startsocket))
  ;[0.1216 0.902 0.6627] Checks if the light is on the socket and if it is makes the first move to get it in the position for buttons to move
  (if (Variables|/Game/MechanicsPlayground/MechanincsBlueprints/BP_PlaceLightSocket.BP_PlaceLightSocket_C|GetbLightOnSocket (Variables|Default|GetStartSocket))
    (if (not (Variables|/Game/MechanicsPlayground/MechanincsBlueprints/BP_PlaceLightSocket.BP_PlaceLightSocket_C|GetbLightOnSocket (Variables|Default|GetEndSocket)))
      (Variables|Default|SetLightOrbRef (Variables|/Game/MechanicsPlayground/MechanincsBlueprints/BP_PlaceLightSocket.BP_PlaceLightSocket_C|GetLightOrbRef (Variables|Default|GetStartSocket)))
      (Utilities|FlowControl|DoOnce false
        (:Completed
          (CallFunction|MoveOrbtoEnd _locationofsocket (+ _locationofsocket (Variables|Default|GetIntervalPath)))
          (bind _lightorbstatus (Default|GetLightOrbStrength (Variables|Default|GetLightOrbRef)))
          (Variables|Default|SetLightOrbStrengthSave _lightorbstatus)
          (Variables|/Game/MechanicsPlayground/MechanincsBlueprints/BP_LightOrb.BP_LightOrb_C|SetbDecayIsOnHold (Variables|Default|GetLightOrbRef) true)
          (Variables|/Game/MechanicsPlayground/MechanincsBlueprints/BP_LightOrb.BP_LightOrb_C|SetbIsIncreasing (Variables|Default|GetLightOrbRef) false)
          (Default|SetLightOrbStrength (Variables|Default|GetLightOrbRef) 2.0)
          (Default|SetLightOrbConditions (Variables|Default|GetLightOrbRef))
          (Math|Integer|IncrementInt (Variables|Default|GetstepsCompleted)))))))

(event EventInfluenceLightOrb
  (params (LightOrbRef :type BP%20Light%20Orb%20Object%20Reference) (IsActive :type Boolean))
  ;[0.1216 0.902 0.6627] Makes the LightOrb React to itself
  (Default|LightPulsing LightOrbRef))

(fn ConstructionScript)

(fn ExchangeValues
  (params (EndSocket :type BP%20Place%20Light%20Socket%20Object%20Reference) (StartSocket :type BP%20Place%20Light%20Socket%20Object%20Reference))
  (Variables|/Game/MechanicsPlayground/MechanincsBlueprints/BP_PlaceLightSocket.BP_PlaceLightSocket_C|SetTimeOfLightInSocket EndSocket (Variables|/Game/MechanicsPlayground/MechanincsBlueprints/BP_PlaceLightSocket.BP_PlaceLightSocket_C|GetTimeOfLightInSocket StartSocket))
  (Variables|/Game/MechanicsPlayground/MechanincsBlueprints/BP_PlaceLightSocket.BP_PlaceLightSocket_C|SetPlayerRef EndSocket (Variables|/Game/MechanicsPlayground/MechanincsBlueprints/BP_PlaceLightSocket.BP_PlaceLightSocket_C|GetPlayerRef StartSocket))
  (Variables|/Game/MechanicsPlayground/MechanincsBlueprints/BP_PlaceLightSocket.BP_PlaceLightSocket_C|SetLightOrbRef EndSocket (Variables|/Game/MechanicsPlayground/MechanincsBlueprints/BP_PlaceLightSocket.BP_PlaceLightSocket_C|GetLightOrbRef StartSocket))
  (Variables|/Game/MechanicsPlayground/MechanincsBlueprints/BP_PlaceLightSocket.BP_PlaceLightSocket_C|SetbLightOnSocket EndSocket true)
  (Variables|/Game/ThirdPerson/Blueprints/BP_ThirdPersonCharacter.BP_ThirdPersonCharacter_C|SetNearestLightSocketRef (Variables|/Game/MechanicsPlayground/MechanincsBlueprints/BP_PlaceLightSocket.BP_PlaceLightSocket_C|GetPlayerRef EndSocket) EndSocket))

(fn GetActiveLocation
  (return (Variables|Default|GetstepsCompleted)))