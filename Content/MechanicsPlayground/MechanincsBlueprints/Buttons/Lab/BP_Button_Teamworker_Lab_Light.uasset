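; Lab light button that toggles the strength of the light orb on the lab's socket mover.
; On BeginPlay it applies the lab reveal-particle effect and glow material to its sign.
; ButtonTask casts the group to BP_ButtonGrouper_Lab, then uses a FlipFlop to alternately raise and lower orb strength and refresh its conditions.
; That toggle sits behind a constant branch condition that never passes, so it does not run as wired.
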(event EventBeginPlay
  (|CallParentFunction)
  (Class|NiagaraComponent|SetAsset (Variables|/Game/MechanicsPlayground/MechanincsBlueprints/GlowTextures/BP_TEMPLATE_BlowGlow_Base.BP_TEMPLATE_BlowGlow_Base_C|GetTextureGlow (Variables|Default|GetSignGlow)) "/Game/MechanicsPlayground/MechanincsBlueprints/GlowTextures/NiagaraSystems/NS_BlowRevealParticles_Lab.NS_BlowRevealParticles_Lab" false)
  (Rendering|Material|SetMaterial (Variables|Default|GetSignBase) 0 "/Game/MechanicsPlayground/MechanincsBlueprints/GlowTextures/Material/M_GlowMechanic_Lab.M_GlowMechanic_Lab"))

(event Collision|EventActorBeginOverlap
  (params (OtherActor :type Actor%20Object%20Reference))
  (|CallParentFunction OtherActor) ; This node is disabled and will not be called.\nDrag off pins to build functionality.
)

(event EventTick
  (params (DeltaSeconds :type Float%20%28single-precision%29))
  (|CallParentFunction DeltaSeconds) ; This node is disabled and will not be called.\nDrag off pins to build functionality.
)

(event EventButtonTask
  (params (ButtonGroup :type BP%20Button%20Grouper%20Base%20Object%20Reference))
  (bind _asbp_button_grouper_lab (Utilities|Casting|CastToBP_ButtonGrouper_Lab ButtonGroup))
  (if (not true)
    (Variables|Default|SetbIsTasking true)
    (Utilities|FlowControl|FlipFlop
      (:A
        (Variables|/Game/MechanicsPlayground/MechanincsBlueprints/BP_LightOrb.BP_LightOrb_C|SetbIsIncreasing (Variables|/Game/MechanicsPlayground/MechanincsBlueprints/BP_MoveBetweenSocketsWithButtons.BP_MoveBetweenSocketsWithButtons_C|GetLightOrbRef (Variables|/Game/MechanicsPlayground/MechanincsBlueprints/Buttons/Lab/BP_Lab.BP_Lab_C|GetSocketMover (Variables|/Game/MechanicsPlayground/MechanincsBlueprints/Buttons/Lab/BP_ButtonGrouper_Lab.BP_ButtonGrouper_Lab_C|GetLabRef _asbp_button_grouper_lab))) true)
        (Default|SetLightOrbStrength (Variables|/Game/MechanicsPlayground/MechanincsBlueprints/BP_MoveBetweenSocketsWithButtons.BP_MoveBetweenSocketsWithButtons_C|GetLightOrbRef (Variables|/Game/MechanicsPlayground/MechanincsBlueprints/Buttons/Lab/BP_Lab.BP_Lab_C|GetSocketMover (Variables|/Game/MechanicsPlayground/MechanincsBlueprints/Buttons/Lab/BP_ButtonGrouper_Lab.BP_ButtonGrouper_Lab_C|GetLabRef _asbp_button_grouper_lab))) 3.0)
        (Default|SetLightOrbConditions (Variables|/Game/MechanicsPlayground/MechanincsBlueprints/BP_MoveBetweenSocketsWithButtons.BP_MoveBetweenSocketsWithButtons_C|GetLightOrbRef (Variables|/Game/MechanicsPlayground/MechanincsBlueprints/Buttons/Lab/BP_Lab.BP_Lab_C|GetSocketMover (Variables|/Game/MechanicsPlayground/MechanincsBlueprints/Buttons/Lab/BP_ButtonGrouper_Lab.BP_ButtonGrouper_Lab_C|GetLabRef _asbp_button_grouper_lab)))))
      (:B
        (Variables|/Game/MechanicsPlayground/MechanincsBlueprints/BP_LightOrb.BP_LightOrb_C|SetbIsIncreasing (Variables|/Game/MechanicsPlayground/MechanincsBlueprints/BP_MoveBetweenSocketsWithButtons.BP_MoveBetweenSocketsWithButtons_C|GetLightOrbRef (Variables|/Game/MechanicsPlayground/MechanincsBlueprints/Buttons/Lab/BP_Lab.BP_Lab_C|GetSocketMover (Variables|/Game/MechanicsPlayground/MechanincsBlueprints/Buttons/Lab/BP_ButtonGrouper_Lab.BP_ButtonGrouper_Lab_C|GetLabRef _asbp_button_grouper_lab))) false)
        (Default|SetLightOrbStrength (Variables|/Game/MechanicsPlayground/MechanincsBlueprints/BP_MoveBetweenSocketsWithButtons.BP_MoveBetweenSocketsWithButtons_C|GetLightOrbRef (Variables|/Game/MechanicsPlayground/MechanincsBlueprints/Buttons/Lab/BP_Lab.BP_Lab_C|GetSocketMover (Variables|/Game/MechanicsPlayground/MechanincsBlueprints/Buttons/Lab/BP_ButtonGrouper_Lab.BP_ButtonGrouper_Lab_C|GetLabRef _asbp_button_grouper_lab))) 2.0)
        (Default|SetLightOrbConditions (Variables|/Game/MechanicsPlayground/MechanincsBlueprints/BP_MoveBetweenSocketsWithButtons.BP_MoveBetweenSocketsWithButtons_C|GetLightOrbRef (Variables|/Game/MechanicsPlayground/MechanincsBlueprints/Buttons/Lab/BP_Lab.BP_Lab_C|GetSocketMover (Variables|/Game/MechanicsPlayground/MechanincsBlueprints/Buttons/Lab/BP_ButtonGrouper_Lab.BP_ButtonGrouper_Lab_C|GetLabRef _asbp_button_grouper_lab))))))
    (Variables|Default|SetbIsTasking false)))

(fn ConstructionScript
  (|CallParentFunction))