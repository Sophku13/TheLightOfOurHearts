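; Death box actor that kills the player on entering it without the light orb held or eaten.
; InfluencingPlayer toggles the box's overlap events by range, and a qualifying overlap opens the character's death UI, passing itself.
; A separate PlayerDeath event hands the dying player to the death manager's DarknessSurrounding.
; IsInfluencingThePlayer is a WIP stub that always returns true.
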(event OnComponentBeginOverlap(PlayerDeathBox)
  (params (OverlappedComponent :type Primitive%20Component%20Object%20Reference) (OtherActor :type Actor%20Object%20Reference) (OtherComp :type Primitive%20Component%20Object%20Reference) (OtherBodyIndex :type Integer) (bFromSweep :type Boolean) (SweepResult :type Hit%20Result%20Structure%20%28by%20ref%29))
  ;[0.1216 0.902 0.6627] When the player is overlapping and the light orb is neither Held nor eaten the player dies
  (bind _asbp_third_person_character (Utilities|Casting|CastToBP_ThirdPersonCharacter OtherActor))
  (if (Math|Boolean|NORBoolean (Variables|/Game/MechanicsPlayground/MechanincsBlueprints/BP_LightOrb.BP_LightOrb_C|GetbIsHeld (Variables|/Game/ThirdPerson/Blueprints/BP_ThirdPersonCharacter.BP_ThirdPersonCharacter_C|GetBP_LightOrbRef _asbp_third_person_character)) (Variables|/Game/MechanicsPlayground/MechanincsBlueprints/BP_LightOrb.BP_LightOrb_C|GetbIsEaten (Variables|/Game/ThirdPerson/Blueprints/BP_ThirdPersonCharacter.BP_ThirdPersonCharacter_C|GetBP_LightOrbRef _asbp_third_person_character)))
    (Default|OpenDeathUI _asbp_third_person_character self)))

(event EventBeginPlay)

(event EventTick
  (params (DeltaSeconds :type Float%20%28single-precision%29)))

(event Collision|EventActorBeginOverlap
  (params (OtherActor :type Actor%20Object%20Reference)))

(event EventInfluencingPlayer
  (params (PlayerRef :type BP%20Third%20Person%20Character%20Object%20Reference) (bIsInRange :type Boolean))
  (bind _playerdeathbox (Variables|Default|GetPlayerDeathBox))
  ;[1 1 1] Death Connection
  (if bIsInRange
    (Variables|/Script/Engine.PrimitiveComponent|SetbGenerateOverlapEvents _playerdeathbox true)
    (Development|PrintString "Player Is Influenced by PlayerDeathbox_WithoutLightInHand")
    (else
      (Variables|/Script/Engine.PrimitiveComponent|SetbGenerateOverlapEvents _playerdeathbox false))))

(event EventPlayerDeath
  (params (DyingPlayerReference :type BP%20Third%20Person%20Character%20Object%20Reference))
  ;[1 1 1] Death Connection
  (Default|DarknessSurrounding (Variables|Default|GetDeathManagerRef) DyingPlayerReference)
  (Development|PrintString "Player dying because of PlayerDeathbox_WithoutLightInHand"))

(fn ConstructionScript)

(fn IsInfluencingthePlayer
  (params (PlayerRef :type BP%20Third%20Person%20Character%20Object%20Reference))
  ;[1 1 1] WIP
  (return true))