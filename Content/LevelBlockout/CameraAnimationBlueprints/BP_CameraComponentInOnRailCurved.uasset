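; Curved variant of an on-rail camera Blueprint that overrides how the parent computes its forward rotation.
; When pre-planned movement is enabled, the rotation looks from player character 0 toward a spline point a short fixed distance ahead of the stored closest position, clamped to the spline's length.
; Otherwise it returns the parent's rotation; all other logic is inherited.
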(event EventBeginPlay
  (|CallParentFunction) ; This node is disabled and will not be called.\nDrag off pins to build functionality.
)

(event Collision|EventActorBeginOverlap
  (params (OtherActor :type Actor%20Object%20Reference))
  (|CallParentFunction OtherActor) ; This node is disabled and will not be called.\nDrag off pins to build functionality.
)

(event EventTick
  (params (DeltaSeconds :type Float%20%28single-precision%29))
  (|CallParentFunction DeltaSeconds) ; This node is disabled and will not be called.\nDrag off pins to build functionality.
)

(fn ConstructionScript
  (|CallParentFunction))

(fn GeForwardtotation
  (bind _spline (Variables|Default|GetSpline))
  (if (Variables|Default|GetUsePrePlannedMovement)
    (return (Math|Rotator|FindLookatRotation (Transformation|GetActorLocation (Game|GetPlayerCharacter 0)) (Spline|GetLocationatDistanceAlongSpline _spline (Math|Float|Min(Float) (+ (Variables|Default|GetPoint%20on%20Spline%20at%20Closest%20Position) 2e+02) (Spline|GetSplineLength _spline)) "World")))
    (else
      (bind _forward (|CallParentFunction))
      (return _forward))))