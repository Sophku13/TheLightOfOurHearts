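; Blockout prop whose platform moves while a BP_BlowMechanic actor overlaps its Box, with a widget prompt for the interaction.
; The overlap plays the MoveUpDown timeline, lerping the platform from its initial to its target relative location, and leaving stops it in place.
; An attached MetaSound scrape plays from BeginPlay, with its gain parameter raised during overlap and zeroed afterward.
; A separate PromptCollision volume shows and hides the widget on any overlap.
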(event OnComponentBeginOverlap(Box)
  (params (OverlappedComponent :type Primitive%20Component%20Object%20Reference) (OtherActor :type Actor%20Object%20Reference) (OtherComp :type Primitive%20Component%20Object%20Reference) (OtherBodyIndex :type Integer) (bFromSweep :type Boolean) (SweepResult :type Hit%20Result%20Structure%20%28by%20ref%29))
  (Utilities|Casting|CastToBP_BlowMechanic OtherActor)
  (Development|PrintString "IsOverlapping")
  (Audio|Parameter|SetFloatParameter (Variables|Default|GetScrapeSound) "GainScrape" 0.8 :!class /Script/Engine.AudioComponent)
  (bind _movement (Timeline|MoveUpDown Play)
    (:Update
      (Transformation|SetRelativeLocation (Variables|Default|GetPlatform) (Math|Vector|Lerp(Vector) (Variables|Default|GetInitialLocation) (Variables|Default|GetNewLocation) _movement) false false))))

(event OnComponentBeginOverlap(PromptCollision)
  (params (OverlappedComponent :type Primitive%20Component%20Object%20Reference) (OtherActor :type Actor%20Object%20Reference) (OtherComp :type Primitive%20Component%20Object%20Reference) (OtherBodyIndex :type Integer) (bFromSweep :type Boolean) (SweepResult :type Hit%20Result%20Structure%20%28by%20ref%29))
  ;[1 1 1] Comment
  (Rendering|SetVisibility (Variables|Default|GetWidget) true false))

(event OnComponentEndOverlap(Box)
  (params (OverlappedComponent :type Primitive%20Component%20Object%20Reference) (OtherActor :type Actor%20Object%20Reference) (OtherComp :type Primitive%20Component%20Object%20Reference) (OtherBodyIndex :type Integer))
  (Utilities|Casting|CastToBP_BlowMechanic OtherActor)
  (Audio|Parameter|SetFloatParameter (Variables|Default|GetScrapeSound) "GainScrape" 0.0 :!class /Script/Engine.AudioComponent)
  (bind _movement (Timeline|MoveUpDown Stop)
    (:Update
      (Transformation|SetRelativeLocation (Variables|Default|GetPlatform) (Math|Vector|Lerp(Vector) (Variables|Default|GetInitialLocation) (Variables|Default|GetNewLocation) _movement) false false))))

(event OnComponentEndOverlap(PromptCollision)
  (params (OverlappedComponent :type Primitive%20Component%20Object%20Reference) (OtherActor :type Actor%20Object%20Reference) (OtherComp :type Primitive%20Component%20Object%20Reference) (OtherBodyIndex :type Integer))
  ;[1 1 1] Comment
  (Rendering|SetVisibility (Variables|Default|GetWidget) false false))

(event EventBeginPlay
  (Variables|Default|SetInitialLocation (Variables|/Script/Engine.SceneComponent|GetRelativeLocation (Variables|Default|GetPlatform)))
  (Variables|Default|SetNewLocation (Variables|Default|GetNewLocation))
  (bind _returnvalue (Audio|SpawnSoundAttached "/Game/Audio/Metasounds/Metasound_Concretescrape.Metasound_Concretescrape" (Variables|Default|GetPlatform) "None" "0, 0, 0" "0, 0, 0" "KeepRelativeOffset" false 1.0 1.0 0.0 0 0))
  (bind _output_get (Variables|Default|SetScrapeSound _returnvalue))
  (Audio|Parameter|SetFloatParameter _output_get "GainScrape" 0.0 :!class /Script/Engine.AudioComponent))

(fn ConstructionScript)