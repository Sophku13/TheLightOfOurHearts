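; Pushable object that the third-person character can push and pull along forward/back and left/right axes while interacting with it.
; Overlapping the Fwd component re-fetches the character (needed after respawn), allows interaction and enables Tick; leaving disables both.
; Tick checks the player is alive and interacting, then maps movement axes to a signed speed.
; SpeedDirection interpolates SMCube along its forward or right vector, without sweep.
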(event OnComponentBeginOverlap(Fwd)
  (params (OverlappedComponent :type Primitive%20Component%20Object%20Reference) (OtherActor :type Actor%20Object%20Reference) (OtherComp :type Primitive%20Component%20Object%20Reference) (OtherBodyIndex :type Integer) (bFromSweep :type Boolean) (SweepResult :type Hit%20Result%20Structure%20%28by%20ref%29))
  (Development|PrintString "Can Interact" true true "(R=0.048799,G=1.000000,B=0.000000,A=1.000000)")
  ;[0.1216 0.902 0.6627] Fixing a problem due to respawn. Need to get the new char reference again. No need to tick before first Overlap!?
  (bind _returnvalue (Actor|GetActorOfClass "/Game/ThirdPerson/Blueprints/BP_ThirdPersonCharacter.BP_ThirdPersonCharacter_C"))
  (bind _output_get (Variables|Default|SetCharRef _returnvalue))
  (Variables|/Game/ThirdPerson/Blueprints/BP_ThirdPersonCharacter.BP_ThirdPersonCharacter_C|SetbCanInteractBox _output_get true)
  (Actor|Tick|SetActorTickEnabled true))

(event OnComponentEndOverlap(Fwd)
  (params (OverlappedComponent :type Primitive%20Component%20Object%20Reference) (OtherActor :type Actor%20Object%20Reference) (OtherComp :type Primitive%20Component%20Object%20Reference) (OtherBodyIndex :type Integer))
  (Development|PrintString "Cant Interact" true true "(R=1.000000,G=0.000000,B=0.000000,A=1.000000)")
  (Variables|/Game/ThirdPerson/Blueprints/BP_ThirdPersonCharacter.BP_ThirdPersonCharacter_C|SetbCanInteractBox (Variables|Default|GetCharREF) false)
  ;[0.1216 0.902 0.6627] Disabling the Tick again when player leaves the area
  (Actor|Tick|SetActorTickEnabled false))

(event EventBeginPlay
  (bind _returnvalue (Actor|GetActorOfClass "/Game/ThirdPerson/Blueprints/BP_ThirdPersonCharacter.BP_ThirdPersonCharacter_C"))
  (Variables|Default|SetCharREF _returnvalue))

(event Collision|EventActorBeginOverlap
  (params (OtherActor :type Actor%20Object%20Reference)))

(event EventTick
  (params (DeltaSeconds :type Float%20%28single-precision%29))
  (bind _charref (Variables|Default|GetCharREF))
  (bind _charref_2 (Variables|Default|GetCharREF))
  (bind _fforwardbackwardaxis (Variables|/Game/ThirdPerson/Blueprints/BP_ThirdPersonCharacter.BP_ThirdPersonCharacter_C|GetfForwardBackwardAxis _charref_2))
  (bind _fleftrightaxis (Variables|/Game/ThirdPerson/Blueprints/BP_ThirdPersonCharacter.BP_ThirdPersonCharacter_C|GetfLeftRightAxis _charref_2))
  ;[0.1216 0.902 0.6627] Checking if the Character is alive atm
  (if (not (Variables|/Game/MechanicsPlayground/MechanincsBlueprints/BP_LightOrb.BP_LightOrb_C|GetbIsDead (Variables|/Game/ThirdPerson/Blueprints/BP_ThirdPersonCharacter.BP_ThirdPersonCharacter_C|GetBP_LightOrbRef (Variables|Default|GetCharREF))))
    (if (Variables|/Game/ThirdPerson/Blueprints/BP_ThirdPersonCharacter.BP_ThirdPersonCharacter_C|GetbIsInteractingBox _charref)
      (if (Variables|/Game/ThirdPerson/Blueprints/BP_ThirdPersonCharacter.BP_ThirdPersonCharacter_C|GetbCanInteractBox _charref)
        (Utilities|FlowControl|Sequence
          (:then_0
            (if (== _fforwardbackwardaxis 0.0)
              (Development|PrintString "Player Is not Moving FWD or BWD" true true "(R=1.000000,G=0.004823,B=0.000000,A=1.000000)")
              (elif (>= _fforwardbackwardaxis 0.1)
                (Development|PrintString "Player is moving FORWARD" true true "(R=0.000000,G=1.000000,B=0.233442,A=1.000000)")
                (Utilities|Speed/Direction true 34.0)
                (else
                  (Development|PrintString "Player Is Moving BACKWARDS" true true "(R=0.000000,G=0.333333,B=0.077814,A=1.000000)")
                  (Utilities|Speed/Direction true -34.0)))))
          (:then_1
            (if (== _fleftrightaxis 0.0)
              (Development|PrintString "Player Is not Moving FWD or BWD" true true "(R=1.000000,G=0.004823,B=0.000000,A=1.000000)")
              (elif (>= _fleftrightaxis 0.1)
                (Development|PrintString "Player is moving RIGHT" true true "(R=0.000000,G=1.000000,B=0.978135,A=1.000000)")
                (Utilities|Speed/Direction false 34.0)
                (else
                  (Development|PrintString "Player is moving LEFT" true true "(R=0.000000,G=0.437500,B=0.427934,A=1.000000)")
                  (Utilities|Speed/Direction false -34.0))))))))))

(fn ConstructionScript)