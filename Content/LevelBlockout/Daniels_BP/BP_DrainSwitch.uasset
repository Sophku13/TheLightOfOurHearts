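; BP_DrainSwitch is an interactable button that the third-person character can press once while nearby.
; HitBox overlaps flag the player as close and toggle Tick, which polls the player's interact flag to fire ButtonClicked.
; Pressing lowers the button, turns its light green and requests the default camera, as does leaving unpressed.
; The press takes its camera target from the end-overlap cast, rather than the stored PlayerRef.
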(event OnComponentBeginOverlap(HitBox)
  (params (OverlappedComponent :type Primitive%20Component%20Object%20Reference) (OtherActor :type Actor%20Object%20Reference) (OtherComp :type Primitive%20Component%20Object%20Reference) (OtherBodyIndex :type Integer) (bFromSweep :type Boolean) (SweepResult :type Hit%20Result%20Structure%20%28by%20ref%29))
  (bind _asbp_third_person_character (Utilities|Casting|CastToBP_ThirdPersonCharacter OtherActor))
  (Development|PrintString "HALLO")
  (bind _output_get (Variables|Default|SetPlayerRef _asbp_third_person_character))
  (Variables|/Game/ThirdPerson/Blueprints/BP_ThirdPersonCharacter.BP_ThirdPersonCharacter_C|SetbCloseToDrainSwitch _output_get true)
  (Actor|Tick|SetActorTickEnabled true))

(event OnComponentEndOverlap(HitBox)
  (params (OverlappedComponent :type Primitive%20Component%20Object%20Reference) (OtherActor :type Actor%20Object%20Reference) (OtherComp :type Primitive%20Component%20Object%20Reference) (OtherBodyIndex :type Integer))
  (bind _asbp_third_person_character (Utilities|Casting|CastToBP_ThirdPersonCharacter OtherActor))
  (Development|PrintString "BYE")
  (Variables|/Game/ThirdPerson/Blueprints/BP_ThirdPersonCharacter.BP_ThirdPersonCharacter_C|SetbCloseToDrainSwitch (Variables|Default|GetPlayerRef) false)
  (Actor|Tick|SetActorTickEnabled false)
  (if (not (Variables|Default|GetbIsButtonPressed))
    (Class|BPIPlayer|EnableDefaultCharacterCamera(Message) _asbp_third_person_character)))

(event Custom|ButtonClicked
  (bind _button (Variables|Default|GetButton))
  (Transformation|SetRelativeLocation _button (+ (Variables|/Script/Engine.SceneComponent|GetRelativeLocation _button) "0.000000,0.000000,-2.000000") false false)
  (Variables|Default|SetbIsButtonPressed true)
  (Rendering|Components|Light|SetLightColor (Variables|Default|GetPointLight) "(R=0.000000,G=1.000000,B=0.014971,A=1.000000)" true)
  (Class|BPIPlayer|EnableDefaultCharacterCamera(Message) (stale OnComponentEndOverlap(HitBox) _asbp_third_person_character)))

(event EventTick
  (params (DeltaSeconds :type Float%20%28single-precision%29))
  (if (Variables|/Game/ThirdPerson/Blueprints/BP_ThirdPersonCharacter.BP_ThirdPersonCharacter_C|GetbInteractWithDrainSwitch (Variables|Default|GetPlayerRef))
    (if (not (Variables|Default|GetbIsButtonPressed))
      (CallFunction|ButtonClicked))))

(fn ConstructionScript)