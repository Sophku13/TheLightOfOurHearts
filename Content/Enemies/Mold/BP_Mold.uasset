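; BP_Mold is an enemy that drifts toward the player's light orb and eats its light.
; Player overlap while the orb is held and the player isn't hiding starts timelines that lerp the NSMold component above the orb, then drain its strength.
; Delayed checks destroy the mold if the player is blowing; it also destroys itself once drained strength drops below zero.
; Tick re-finds orb, player and spawner with GetAllActorsOfClass every frame.
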(event OnComponentBeginOverlap(CollisionBox)
  (params (OverlappedComponent :type Primitive%20Component%20Object%20Reference) (OtherActor :type Actor%20Object%20Reference) (OtherComp :type Primitive%20Component%20Object%20Reference) (OtherBodyIndex :type Integer) (bFromSweep :type Boolean) (SweepResult :type Hit%20Result%20Structure%20%28by%20ref%29))
  (bind _asbp_blow_mechanic (Utilities|Casting|CastToBP_BlowMechanic OtherActor))
  (Utilities|IsValid _asbp_blow_mechanic
    (:Is%20Valid
      (CallFunction|MoldDestroy))))

(event Custom|StartDecreaseLightOrbStrength
  (bind _lightorbref (Variables|Default|GetLightOrbRef))
  (bind _lightorbref_2 (Variables|Default|GetLightOrbRef))
  ;[1 0 1] Eating Light
  (Utilities|IsValid _lightorbref_2
    (:Is%20Valid
      (bind _lightorbstatus (Default|GetLightOrbStrength _lightorbref_2))
      (Variables|Default|SetInitialLightOrbStrength _lightorbstatus)
      (bind _interpvalue (Timeline|LightOrbStrengthDecrease PlayFromStart)
        (:Update
          (Utilities|IsValid _lightorbref
            (:Is%20Valid
              (Default|SetLightOrbStrength _lightorbref (Math|Float|Lerp (Variables|Default|GetInitialLightOrbStrength) (Variables|Default|GetTargetLightOrbStrength) _interpvalue))
              (CallFunction|MoldDestroy)
              (if (< (Math|Float|Lerp (Variables|Default|GetInitialLightOrbStrength) (Variables|Default|GetTargetLightOrbStrength) _interpvalue) -0.01)
                (Actor|DestroyActor)
                (Variables|Default|SetisAlive false)))))))))

(event Custom|MoldDestroy
  (bind _playerref (Variables|Default|GetPlayerRef))
  ;[1 0 1] Mold Destroy
  (Utilities|FlowControl|Delay 3.0)
  (Utilities|IsValid _playerref
    (:Is%20Valid
      (if (Variables|/Game/ThirdPerson/Blueprints/BP_ThirdPersonCharacter.BP_ThirdPersonCharacter_C|GetbIsBlowing _playerref)
        (Variables|Default|SetcanBeKilled true)
        (Development|PrintString "Blowing for 3 Sec" true true "(R=0.000000,G=1.000000,B=0.111812,A=1.000000)")
        (Actor|DestroyActor)
        (Variables|Default|SetisAlive false)
        (Development|PrintString "MOLD is NOT Alive" true true "(R=0.710703,G=1.000000,B=0.000000,A=1.000000)")
        (else
          (Variables|Default|SetcanBeKilled false))))))

(event EventBeginPlay)

(event Collision|EventActorBeginOverlap
  (params (OtherActor :type Actor%20Object%20Reference))
  (bind _asbp_third_person_character (Utilities|Casting|CastToBP_ThirdPersonCharacter OtherActor))
  (Utilities|IsValid _asbp_third_person_character
    (:Is%20Valid
      (bind _output_get (Variables|Default|SetPlayerRef _asbp_third_person_character))
      (Variables|Default|SetIntitialNSMoldPosition (Transformation|GetWorldLocation (Variables|Default|GetNS_Mold)))
      (bind _outactors (Actor|GetAllActorsOfClass "/Game/MechanicsPlayground/MechanincsBlueprints/BP_LightOrb.BP_LightOrb_C"))
      (for _array_element _outactors
        (Utilities|IsValid _array_element
          (:Is%20Valid
            (Variables|Default|SetLightOrbRef _array_element)
            (if (and (Variables|/Game/MechanicsPlayground/MechanincsBlueprints/BP_LightOrb.BP_LightOrb_C|GetbIsHeld (Variables|Default|GetLightOrbRef)) (not (Variables|/Game/ThirdPerson/Blueprints/BP_ThirdPersonCharacter.BP_ThirdPersonCharacter_C|GetbIsHiding (Variables|Default|GetPlayerRef))))
              (Utilities|FlowControl|Delay 1.5)
              (bind _alpha (Timeline|MoveNSMold Play)
                (:Update
                  (Variables|Default|SetAlpha _alpha)
                  (Variables|Default|SetisFollowingPlayer true)
                  (Utilities|IsValid _output_get
                    (:Is%20Valid
                      (CallFunction|MoldDestroy)
                      (Utilities|FlowControl|Delay 3.0)
                      (CallFunction|StartDecreaseLightOrbStrength))))
                (:Finished
                  (Development|PrintString "TIMELINE ENDED" true true "(R=1.000000,G=0.036710,B=0.000000,A=1.000000)"))))))))))

(event EventTick
  (params (DeltaSeconds :type Float%20%28single-precision%29))
  (bind _outactors (Actor|GetAllActorsOfClass "/Game/MechanicsPlayground/MechanincsBlueprints/BP_LightOrb.BP_LightOrb_C"))
  (for _array_element _outactors
    (Utilities|IsValid _array_element
      (:Is%20Valid
        (bind _output_get (Variables|Default|SetLightOrbRef _array_element))
        (Variables|Default|SetTargetPosition (+ (Transformation|GetActorLocation _output_get) "0.000000,0.000000,250.000000"))
        (bind _outactors_2 (Actor|GetAllActorsOfClass "/Game/ThirdPerson/Blueprints/BP_ThirdPersonCharacter.BP_ThirdPersonCharacter_C"))
        (for _array_element_2 _outactors_2
          (Utilities|IsValid _array_element_2
            (:Is%20Valid
              (Variables|Default|SetPlayerRef _array_element_2)
              (if (Variables|Default|GetisFollowingPlayer)
                (CallFunction|UpdateMoldPosition)
                (bind _outactors_3 (Actor|GetAllActorsOfClass "/Game/Enemies/Mold/BP_MoldSpawner.BP_MoldSpawner_C"))
                (for _array_element_3 _outactors_3
                  (Utilities|IsValid _array_element_3
                    (:Is%20Valid
                      (Variables|Default|SetMoldSpawnerRef _array_element_3))))))))))))

(fn ConstructionScript)

(fn UpdateMoldPosition
  (Transformation|SetWorldLocation (Variables|Default|GetNS_Mold) (Math|Vector|Lerp(Vector) (Variables|Default|GetIntitialNSMoldPosition) (Variables|Default|GetTargetPosition) (Variables|Default|GetAlpha)) true false))