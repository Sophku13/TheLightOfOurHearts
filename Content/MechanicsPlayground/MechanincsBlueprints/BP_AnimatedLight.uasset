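; BP_AnimatedLight is a light actor whose point light brightens as a BP_LightOrb gets closer.
; When an orb enters the sphere, it stores the orb and starts a looping timer.
; Each tick of the timer maps orb distance inversely to intensity with a clamped range, applies it and prints it for debugging.
; Any end overlap on the sphere pauses the timer, without checking for the orb.
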(event OnComponentBeginOverlap(Sphere)
  (params (OverlappedComponent :type Primitive%20Component%20Object%20Reference) (OtherActor :type Actor%20Object%20Reference) (OtherComp :type Primitive%20Component%20Object%20Reference) (OtherBodyIndex :type Integer) (bFromSweep :type Boolean) (SweepResult :type Hit%20Result%20Structure%20%28by%20ref%29))
  (bind _asbp_light_orb (Utilities|Casting|CastToBP_LightOrb OtherActor))
  (Variables|Default|SetAs%20BP%20Light%20Orb _asbp_light_orb)
  (bind _returnvalue (Utilities|Time|SetTimerbyEvent (delegate Custom|UpdateIntensity) 0.1 true))
  (Variables|Default|SetTimer _returnvalue))

(event OnComponentEndOverlap(Sphere)
  (params (OverlappedComponent :type Primitive%20Component%20Object%20Reference) (OtherActor :type Actor%20Object%20Reference) (OtherComp :type Primitive%20Component%20Object%20Reference) (OtherBodyIndex :type Integer))
  (Utilities|Time|PauseTimerbyHandle (Variables|Default|GetTimer)))

(event Custom|UpdateIntensity
  (bind _self self)
  (bind _as_bp_light_orb (Variables|Default|GetAs%20BP%20Light%20Orb))
  (bind _returnvalue (Transformation|GetActorLocation _as_bp_light_orb))
  (bind _returnvalue_2 (Transformation|GetActorLocation _self))
  (bind _returnvalue_3 (Math|Vector|Distance(Vector) _returnvalue _returnvalue_2))
  (bind _returnvalue_4 (Math|Float|MapRangeClamped _returnvalue_3 0.0 7e+02 2e+04 0.0))
  (Rendering|Components|Light|SetIntensity (Variables|Default|GetPointLight) _returnvalue_4)
  (Development|PrintString (Utilities|String|ToString(Float) _returnvalue_4)))

(event Collision|EventActorBeginOverlap
  (params (OtherActor :type Actor%20Object%20Reference)))

(fn ConstructionScript)