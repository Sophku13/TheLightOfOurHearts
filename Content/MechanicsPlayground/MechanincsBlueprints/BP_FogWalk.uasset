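; BP_FogWalk is a fog area actor that registers with the light orb and affects the player's movement.
; Box overlaps set the orb's LatestFog and an activation flag, and orb exit clears the player's MovementReduction.
; InfluencingPlayer applies that reduction and toggles Tick, whose damage call is disconnected.
; PlayerDeath triggers LightDeath on the player's death manager, while IsInfluencingThePlayer is a WIP stub returning true.
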(event OnComponentEndOverlap(Box)
  (params (OverlappedComponent :type Primitive%20Component%20Object%20Reference) (OtherActor :type Actor%20Object%20Reference) (OtherComp :type Primitive%20Component%20Object%20Reference) (OtherBodyIndex :type Integer))
  ;[0.1216 0.902 0.6627] Sets the Decay Modifier back to its default, when the LightOrb leaves the Range
  (Utilities|Casting|CastToBP_LightOrb OtherActor)
  (Development|PrintString "LightExitedArea")
  (Variables|Default|SetbIsActivated false)
  (bind _player_ref (Variables|Default|GetPlayer%20Ref)
    (:then
      (Variables|/Game/ThirdPerson/Blueprints/BP_ThirdPersonCharacter.BP_ThirdPersonCharacter_C|SetMovementReduction _player_ref 0.0))
    (:else)))

(event OnComponentBeginOverlap(Box)
  (params (OverlappedComponent :type Primitive%20Component%20Object%20Reference) (OtherActor :type Actor%20Object%20Reference) (OtherComp :type Primitive%20Component%20Object%20Reference) (OtherBodyIndex :type Integer) (bFromSweep :type Boolean) (SweepResult :type Hit%20Result%20Structure%20%28by%20ref%29))
  ;[0.1216 0.902 0.6627] Reacts to the Light Orb Entering the Box and when it is overlapping it modifies the Decay Rate of the Light
  (bind _asbp_light_orb (Utilities|Casting|CastToBP_LightOrb OtherActor))
  (bind _output_get (Variables|Default|SetLightOrbRef _asbp_light_orb))
  (Variables|/Game/MechanicsPlayground/MechanincsBlueprints/BP_LightOrb.BP_LightOrb_C|SetLatestFog _output_get self)
  (Variables|Default|SetbIsActivated true))

(event EventBeginPlay)

(event EventInfluencingPlayer
  (params (PlayerRef :type BP%20Third%20Person%20Character%20Object%20Reference) (bIsInRange :type Boolean))
  ;[0.1216 0.902 0.6627] Death Connection
  (Variables|Default|SetPlayer%20Ref PlayerRef)
  (if bIsInRange
    (Actor|Tick|SetActorTickEnabled true)
    (Variables|/Game/ThirdPerson/Blueprints/BP_ThirdPersonCharacter.BP_ThirdPersonCharacter_C|SetMovementReduction PlayerRef 1e+02)
    (Development|PrintString "Player Is Influenced by LightImpactArea ")
    (else
      (Actor|Tick|SetActorTickEnabled false))))

(event EventTick
  (params (DeltaSeconds :type Float%20%28single-precision%29))
  ;[0.1216 0.902 0.6627] Event Tick that decays the light while it is inside this area
  (Actor|Tick|SetActorTickInterval (Variables|Default|GetLevel%20Orb%20Decay%20Modifier))
  (if (Variables|Default|GetbIsActivated)
    _))

(event EventPlayerDeath
  (params (DyingPlayerReference :type BP%20Third%20Person%20Character%20Object%20Reference))
  ;[0.1216 0.902 0.6627] Death Connection
  (Default|LightDeath (Variables|/Game/ThirdPerson/Blueprints/BP_ThirdPersonCharacter.BP_ThirdPersonCharacter_C|GetDeathManagerRef DyingPlayerReference))
  (Development|PrintString "Player dying because of LightImpactArea"))

(fn ConstructionScript)

(fn IsInfluencingthePlayer
  (params (PlayerRef :type BP%20Third%20Person%20Character%20Object%20Reference))
  ;[1 1 1] WIP
  (return true))