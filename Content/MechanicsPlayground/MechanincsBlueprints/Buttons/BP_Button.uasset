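; Interactable world button that the third-person character presses while standing inside its trigger box.
; Overlap stores the player, sets its CloseToButton flag and enables Tick, which polls the player's InteractingWithButton flag until exit disables it.
; A press sinks the button, turns it green and calls ButtonClick, an empty function here.
; After a short delay it rises, turns red and can be pressed again.
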(event OnComponentBeginOverlap(Button_Box)
  (params (OverlappedComponent :type Primitive%20Component%20Object%20Reference) (OtherActor :type Actor%20Object%20Reference) (OtherComp :type Primitive%20Component%20Object%20Reference) (OtherBodyIndex :type Integer) (bFromSweep :type Boolean) (SweepResult :type Hit%20Result%20Structure%20%28by%20ref%29))
  (bind _asbp_third_person_character (Utilities|Casting|CastToBP_ThirdPersonCharacter OtherActor))
  (bind _output_get (Variables|Default|SetPlayerRef _asbp_third_person_character))
  (bind _output_get_2 (Variables|/Game/ThirdPerson/Blueprints/BP_ThirdPersonCharacter.BP_ThirdPersonCharacter_C|SetbCloseToButton _output_get true))
  (Variables|Default|SetbPlayerInRange _output_get_2)
  (Actor|Tick|SetActorTickEnabled true))

(event OnComponentEndOverlap(Button_Box)
  (params (OverlappedComponent :type Primitive%20Component%20Object%20Reference) (OtherActor :type Actor%20Object%20Reference) (OtherComp :type Primitive%20Component%20Object%20Reference) (OtherBodyIndex :type Integer))
  (Utilities|Casting|CastToBP_ThirdPersonCharacter OtherActor)
  (bind _output_get (Variables|/Game/ThirdPerson/Blueprints/BP_ThirdPersonCharacter.BP_ThirdPersonCharacter_C|SetbCloseToButton (Variables|Default|GetPlayerRef) false))
  (Variables|Default|SetbPlayerInRange _output_get)
  (Actor|Tick|SetActorTickEnabled false))

(event EventBeginPlay)

(event Collision|EventActorBeginOverlap
  (params (OtherActor :type Actor%20Object%20Reference)))

(event EventTick
  (params (DeltaSeconds :type Float%20%28single-precision%29))
  (if (Variables|/Game/ThirdPerson/Blueprints/BP_ThirdPersonCharacter.BP_ThirdPersonCharacter_C|GetbInteractingWithButton (Variables|Default|GetPlayerRef))
    (if (not (Variables|Default|GetbIsButtonPressed))
      (CallFunction|ButtonFunctionality))))

(event EventButtonFunctionality
  (bind _button (Variables|Default|GetButton))
  (bind _button_2 (Variables|Default|GetButton))
  (Variables|Default|SetbIsButtonPressed true)
  (Transformation|SetRelativeLocation _button_2 (+ (Variables|/Script/Engine.SceneComponent|GetRelativeLocation _button_2) "0.000000,0.000000,-2.000000") false false)
  (Rendering|Material|SetMaterial (Variables|Default|GetButton) 0 "/Game/Materials/MI_Sphere_Emissive_Green.MI_Sphere_Emissive_Green")
  (CallFunction|ButtonClick)
  (Utilities|FlowControl|Delay 2.0)
  (Transformation|SetRelativeLocation _button (+ (Variables|/Script/Engine.SceneComponent|GetRelativeLocation _button) "0.000000,0.000000,2.000000") false false)
  (Rendering|Material|SetMaterial (Variables|Default|GetButton) 0 "/Game/Materials/MI_Sphere_Emissive_Red.MI_Sphere_Emissive_Red")
  (Variables|Default|SetbIsButtonPressed false))

(fn ConstructionScript)

(fn ButtonClick)