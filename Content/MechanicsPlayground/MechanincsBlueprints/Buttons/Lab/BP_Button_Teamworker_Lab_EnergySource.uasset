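; Lab button Blueprint that toggles an energy source on the light orb when interacted with.
; ButtonTask uses a FlipFlop to spawn and attach BP_EnergySource to the orb, reached through the button grouper's lab reference, or destroy it.
; After a two-second delay the button moves and can be pressed again if active.
; Tick sets the on/off material from IsActive and destroys any energy source while inactive.
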(event EventBeginPlay
  ;[0.1216 0.902 0.6627] Begin Play spawns a glowsprite after the execution of the parent beginplay
  (|CallParentFunction))

(event Collision|EventActorBeginOverlap
  (params (OtherActor :type Actor%20Object%20Reference))
  (|CallParentFunction OtherActor) ; This node is disabled and will not be called.\nDrag off pins to build functionality.
)

(event EventTick
  (params (DeltaSeconds :type Float%20%28single-precision%29))
  ;[0.1216 0.902 0.6627] Event Tick sets the material of the button on or off and if it is turned off and an energy source was spawned it also gets destroyed
  (if (Variables|Default|GetbIsActive)
    ;;[0.1216 0.902 0.6627] On
    (Rendering|Material|SetMaterial (Variables|Default|GetButton) 0 "/Game/Materials/MI_Sphere_Emissive_Red.MI_Sphere_Emissive_Red")
    (else
      ;;[0.1216 0.902 0.6627] Off
      (Rendering|Material|SetMaterial (Variables|Default|GetButton) 0 "/Game/Materials/MI_Sphere_Emissive_Red_Off.MI_Sphere_Emissive_Red_Off")
      (bind _energysource (Variables|Default|GetEnergySource)
        (:then
          (Actor|DestroyActor _energysource))
        (:else)))))

(event EventButtonTask
  (params (ButtonGroup :type BP%20Button%20Grouper%20Base%20Object%20Reference))
  ;[0.1216 0.902 0.6627] Button Task either spawns a new Energy Source and attaches it to the light orb traveling through the lab or destroys it if one is already existing
  (bind _asbp_button_grouper_lab (Utilities|Casting|CastToBP_ButtonGrouper_Lab ButtonGroup))
  (Utilities|FlowControl|FlipFlop
    (:A
      (bind _energysource (Variables|Default|GetEnergySource)
        (:then
          (Actor|DestroyActor _energysource :!label _label))
        (:else
          (bind _returnvalue (Game|SpawnActorfromClass "/Game/VFX_EnvironmentFX/VantaBlack/Realtime_dissolve/BP_EnergySource.BP_EnergySource_C" (Math|Transform|MakeTransform (.location (Transformation|GetActorTransform (Variables|/Game/MechanicsPlayground/MechanincsBlueprints/BP_MoveBetweenSocketsWithButtons_Lab.BP_MoveBetweenSocketsWithButtons_Lab_C|GetLightOrbRef (Variables|/Game/MechanicsPlayground/MechanincsBlueprints/Buttons/Lab/BP_Lab.BP_Lab_C|GetSocketMover (Variables|/Game/MechanicsPlayground/MechanincsBlueprints/Buttons/Lab/BP_ButtonGrouper_Lab.BP_ButtonGrouper_Lab_C|GetLabRef _asbp_button_grouper_lab))))) (.rotation (Transformation|GetActorTransform (Variables|/Game/MechanicsPlayground/MechanincsBlueprints/BP_MoveBetweenSocketsWithButtons_Lab.BP_MoveBetweenSocketsWithButtons_Lab_C|GetLightOrbRef (Variables|/Game/MechanicsPlayground/MechanincsBlueprints/Buttons/Lab/BP_Lab.BP_Lab_C|GetSocketMover (Variables|/Game/MechanicsPlayground/MechanincsBlueprints/Buttons/Lab/BP_ButtonGrouper_Lab.BP_ButtonGrouper_Lab_C|GetLabRef _asbp_button_grouper_lab))))) "1.000000,1.000000,1.000000") "Undefined" "MultiplyWithRoot" 0 0))
          (bind _output_get (Variables|Default|SetEnergySource _returnvalue))
          (Transformation|AttachComponentToComponent _output_get (Variables|/Game/MechanicsPlayground/MechanincsBlueprints/BP_LightOrb.BP_LightOrb_C|GetM_LightOrb (Variables|/Game/MechanicsPlayground/MechanincsBlueprints/BP_MoveBetweenSocketsWithButtons_Lab.BP_MoveBetweenSocketsWithButtons_Lab_C|GetLightOrbRef (Variables|/Game/MechanicsPlayground/MechanincsBlueprints/Buttons/Lab/BP_Lab.BP_Lab_C|GetSocketMover (Variables|/Game/MechanicsPlayground/MechanincsBlueprints/Buttons/Lab/BP_ButtonGrouper_Lab.BP_ButtonGrouper_Lab_C|GetLabRef _asbp_button_grouper_lab)))) "None" "SnapToTarget" "SnapToTarget" "KeepRelative" false))))
    (:B
      (goto _label))))

(event EventOnInteract
  ;[0.1216 0.902 0.6627] On Interact the button gets moved and the task gets called
  (|CallParentFunction)
  (CallFunction|ButtonTask (Variables|Default|GetButtonGroup))
  (Utilities|FlowControl|Delay 2.0)
  (CallFunction|MoveButton)
  (Variables|Default|SetbIsButtonPressed false))

(fn ConstructionScript
  (|CallParentFunction))

(fn IsInteractable
  (return (and (not (Variables|Default|GetbIsButtonPressed)) (Variables|Default|GetbIsActive))))