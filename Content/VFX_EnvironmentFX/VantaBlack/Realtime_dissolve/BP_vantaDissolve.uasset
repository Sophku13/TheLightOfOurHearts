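; BP_vantaDissolve is a sphere-based actor that feeds a dissolve volume to materials and destroys itself when another actor overlaps it.
; Its construction script writes the Sphere's world location and scale to the MPC_dissolve parameter collection as Location and Bound.
; Those values are not updated at runtime, and the nodes that would pass the sphere's rotation axes are left disconnected.
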(event EventBeginPlay)

(event Collision|EventActorBeginOverlap
  (params (OtherActor :type Actor%20Object%20Reference))
  (Actor|DestroyActor))

(event EventTick
  (params (DeltaSeconds :type Float%20%28single-precision%29)))

(fn ConstructionScript
  (bind _sphere (Variables|Default|GetSphere))
  (Rendering|Material|SetVectorParameterValue "/Game/VFX_EnvironmentFX/VantaBlack/Realtime_dissolve/MPC_dissolve.MPC_dissolve" "Location" (Math|Conversions|ToLinearColor(Vector) (Transformation|GetWorldLocation _sphere)) :!class /Script/Engine.KismetMaterialLibrary)
  (Rendering|Material|SetVectorParameterValue "/Game/VFX_EnvironmentFX/VantaBlack/Realtime_dissolve/MPC_dissolve.MPC_dissolve" "Bound" (Math|Conversions|ToLinearColor(Vector) (Transformation|GetWorldScale _sphere)) :!class /Script/Engine.KismetMaterialLibrary))