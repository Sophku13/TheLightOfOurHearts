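; Light orb actor whose strength decays on tick while held or overheating, can be raised or reduced, and kills or overheats at its extremes.
; SetLightOrbConditions detects strength thresholds and runs ConditionChange, which timeline-lerps intensity and radius from per-tier maps while resizing the collision sphere and particle rate.
; Sphere overlaps send influence messages to other actors.
; Hiding and eaten states save or suppress the light, with a function restoring saved values.
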(event OnComponentBeginOverlap(LightOrb_CollisionSphere)
  (params (OverlappedComponent :type Primitive%20Component%20Object%20Reference) (OtherActor :type Actor%20Object%20Reference) (OtherComp :type Primitive%20Component%20Object%20Reference) (OtherBodyIndex :type Integer) (bFromSweep :type Boolean) (SweepResult :type Hit%20Result%20Structure%20%28by%20ref%29))
  (if (not (Variables|Default|GetIsBeingInfluenced))
    (Variables|Default|SetIsBeingInfluenced true)
    (Class|BPIDetect|InfluenceLightOrb(Message) OtherActor self true)))

(event OnComponentEndOverlap(LightOrb_CollisionSphere)
  (params (OverlappedComponent :type Primitive%20Component%20Object%20Reference) (OtherActor :type Actor%20Object%20Reference) (OtherComp :type Primitive%20Component%20Object%20Reference) (OtherBodyIndex :type Integer))
  (Class|BPIDetect|InfluenceLightOrb(Message) OtherActor self false))

(event Custom|TimelineLightChange
  (params (LightIntensityBefore :type Float%20%28double-precision%29) (LightIntensityAfter :type Float%20%28double-precision%29) (AttenuationRadiusBefore :type Float%20%28double-precision%29) (AttenuationRadiusAfter :type Float%20%28double-precision%29))
  (bind _lightorb_lighting (Variables|Default|GetLightOrb_Lighting))
  (bind _newtrack_0 (Timeline|TimelineLight PlayFromStart)
    (:Update
      (Rendering|Components|Light|SetIntensity _lightorb_lighting (Math|Float|Lerp LightIntensityBefore LightIntensityAfter _newtrack_0))
      (Rendering|Lighting|SetAttenuationRadius _lightorb_lighting (Math|Float|Lerp AttenuationRadiusBefore AttenuationRadiusAfter _newtrack_0)))))

(event Custom|Light%20trembling
  ;[1 0.9568 0.4122] Light trembling with danger           (no matter how strong it is)
  (Components|Activation|SetActive (Variables|Default|GetNS_Trembling) true true)
  (Development|PrintString "Danger!"))

(event Custom|Light%20Pulsing
  ;[1 0.9568 0.4122] Light pulsing for interactable           (no matter how strong it is)
  ;;[1 0.9566 0.5877] activate multiple times
  (Components|Activation|SetActive (Variables|Default|GetNS_Pulsing) true true)
  (Development|PrintString "Interact"))

(event EventBeginPlay
  ;[0.1216 0.902 0.6627] Light Orb Initiator
  (CallFunction|SetLightOrbConditions)
  (Variables|Default|SetOrb%20LightingObj (Variables|Default|GetLightOrb_Lighting))
  (Variables|Default|SetOrb%20Light%20Collision%20SphereObj (Variables|Default|GetLightOrb_CollisionSphere))
  (bind _returnvalue (Actor|GetActorOfClass "/Game/MechanicsPlayground/MechanincsBlueprints/DetectMechanic/BP_Detect.BP_Detect_C"))
  (Variables|Default|SetBP_DetectRevealPlatformRef _returnvalue))

(event EventTick
  (params (DeltaSeconds :type Float%20%28single-precision%29))
  ;[0.1216 0.902 0.6627] The Tick is counting slowly down and is reducing the light orb strength bit by bit. Creating a small buffer at the maximum to not lose it directly after one tick | Currently 5 seconds p.Tick and reducing by .1 per tick
  (if (Variables|Status|GetbIsHeld)
    (if (not (Variables|Status|GetbDecayIsOnHold))
      (Actor|Tick|SetActorTickInterval (/ 1e+01 (Variables|Values|GetLevelOrbDecayModifier)))
      (if (== (Variables|Values|GetLightOrbStatus) 3.0) :!label _label
        (Utilities|FlowControl|Delay 1e+01))
      (Variables|Values|SetLightOrbStatus (- (Variables|Values|GetLightOrbStatus) 0.1))
      (CallFunction|SetLightOrbConditions))
    (elif (Variables|Status|GetIsOverheating)
      (goto _label))))

(fn ConstructionScript)

(fn AddLightOrbStrength
  ;[0.1216 0.902 0.6627] Adding Strength to the Light to a maximum of 3
  (if (< (Variables|Values|GetLightOrbStatus) 0.0)
    (CallFunction|SetLightOrbConditions)
    (elif (>= (Variables|Values|GetLightOrbStatus) 3.0)
      (if (>= (Variables|Values|GetLightOrbStatus) 3.5)
        (if (Variables|Status|GetIsOverheating)
          (Variables|Values|SetLightOrbStatus (+ (Variables|Values|GetLightOrbStatus) 0.03))
          (CallFunction|SetLightOrbConditions :!label _label))
        (else
          (Variables|Values|SetLightOrbStatus (+ (Variables|Values|GetLightOrbStatus) 0.05))
          (goto _label)))
      (else
        (Variables|Values|SetLightOrbStatus (+ (Variables|Values|GetLightOrbStatus) 0.1))
        (goto _label)))))

(fn HideandReduceLightOrb
  ;[0.1216 0.902 0.6627] Reducing Strength to the Light to a minimum of 1
  (if (Variables|Status|GetStatusHidden)
    (if (>= (Variables|Values|GetLightOrbStatus) 1.0)
      (Variables|Values|SetLightOrbStatus (- (Variables|Values|GetLightOrbStatus) 0.1))
      (CallFunction|SetLightOrbConditions))))

(fn GetLightOrbStrength
  ;[0.1216 0.902 0.6627] Get Function for the Light Orb Status
  (return (Variables|Values|GetLightOrbStatus)))

(fn SetLightOrbConditions
  ;[0.1216 0.902 0.6627] Setting the new Conditions for the light when the light strength has changed
  ;;[0.1216 0.902 0.6627] Light is Dead and so is the Character, Orb Status > 0
  (if (not (Variables|Status|GetStatusHidden))
    (if (< (Variables|Values|GetLightOrbStatus) 0.0)
      (Development|PrintText "Ded")
      (if (not (Variables|Status|GetbLightOrbSwitchProcess))
        (Variables|Status|SetbLightOrbSwitchProcess true)
        (Rendering|Components|Light|SetIntensity (Variables|Default|GetLightOrb_Lighting) 0.5)
        (Rendering|Lighting|SetAttenuationRadius (Variables|Default|GetLightOrb_Lighting) 1e+01)
        (Components|Sphere|SetSphereRadius (Variables|Default|GetLightOrb_CollisionSphere) 0.0 true)
        (Variables|Status|SetIsOverheating false)
        (Variables|Status|SetbLightOrbSwitchProcess false)
        (bind _output_get (Variables|Status|SetbIsDead true))
        (return _output_get))
      (else
        ;;[1 1 1] Comment
        (if (Math|Float|NearlyEqual(Float) (Variables|Values|GetLightOrbStatus) 1.0 0.05)
          (if (not (Variables|Status|GetbLightOrbSwitchProcess))
            (Variables|Status|SetbLightOrbSwitchProcess true)
            (CallFunction|ConditionChange (Variables|Status|GetStatus0To1Values) (Variables|Status|GetStatus1To2Values) (Variables|Status|GetbIsIncreasing))
            (Variables|Status|SetbLightOrbSwitchProcess false)
            (return _output_get))
          (else
            ;;[1 1 1] Comment
            (if (Math|Float|NearlyEqual(Float) (Variables|Values|GetLightOrbStatus) 2.0 0.05)
              (if (not (Variables|Status|GetbLightOrbSwitchProcess))
                (Variables|Status|SetbLightOrbSwitchProcess true)
                (CallFunction|ConditionChange (Variables|Status|GetStatus1To2Values) (Variables|Status|GetStatus2To3Values) (Variables|Status|GetbIsIncreasing))
                (Variables|Status|SetbLightOrbSwitchProcess false)
                (return _output_get))
              (elif (Math|Float|NearlyEqual(Float) (Variables|Values|GetLightOrbStatus) 3.0 0.05)
                (if (not (Variables|Status|GetbLightOrbSwitchProcess))
                  (Variables|Status|SetbLightOrbSwitchProcess true)
                  (CallFunction|ConditionChange (Variables|Status|GetStatus2To3Values) (Variables|Status|GetStatus3AndMoreValues) (Variables|Status|GetbIsIncreasing))
                  (Variables|Status|SetbLightOrbSwitchProcess false)
                  (return _output_get))
                (else
                  ;;[1 1 1] Comment
                  (if (> (Variables|Values|GetLightOrbStatus) 3.5)
                    (if (not (Variables|Status|GetbLightOrbSwitchProcess))
                      (Variables|Status|SetbLightOrbSwitchProcess true)
                      (Rendering|Components|Light|SetLightColor (Variables|Default|GetLightOrb_Lighting) "(R=1.000000,G=0.000000,B=0.034294,A=1.000000)" true)
                      ;;;[0.1216 0.902 0.6627] Maximum Light -> Too much. Makes the Player drop the light
                      (Variables|Status|SetIsOverheating true)
                      (Variables|Status|SetbLightOrbSwitchProcess false)
                      (return _output_get))))))))))
    (else
      ;;[1 1 1] Comment
      (if (Math|Float|NearlyEqual(Float) (Variables|Values|GetLightOrbStatus) 1.0 0.05)
        (CallFunction|SaveLightOrbConditionsatMechanicUse true)
        (return _output_get)
        (else
          ;;[1 1 1] Comment
          (if (Math|Float|NearlyEqual(Float) (Variables|Values|GetLightOrbStatus) 2.0 0.05)
            (CallFunction|SaveLightOrbConditionsatMechanicUse true 1)
            (return _output_get)
            (else
              ;;[1 1 1] Comment
              (if (Math|Float|NearlyEqual(Float) (Variables|Values|GetLightOrbStatus) 3.0 0.05)
                (CallFunction|SaveLightOrbConditionsatMechanicUse true 2)
                (return _output_get)))))))))

(fn SetLightOrbStrength
  (params (LightOrbStatus :type Float%20%28double-precision%29))
  ;[0.1216 0.902 0.6627] Just a Function to call from the outside to set the sStrength of the Light Orb
  (Variables|Values|SetLightOrbStatus LightOrbStatus))

(fn SetLightOrbHidden
  ;[0.1216 0.902 0.6627] Sets the Light Orb as Hidden, because the SetLightOrbConditions is only happening when the Light Orb is not hidden. This is because we dont want the Light Orb to change Conditions while we are hiding it
  (if (not (Variables|Status|GetStatusHidden))
    (if (not (Variables|Status|GetbLightOrbSwitchProcess))
      (Variables|Status|SetbLightOrbSwitchProcess true)
      (CallFunction|SaveLightOrbConditionsatMechanicUse false)
      (Rendering|Components|Light|SetIntensity (Variables|Default|GetLightOrb_Lighting) 1.0)
      (Rendering|Lighting|SetAttenuationRadius (Variables|Default|GetLightOrb_Lighting) 5e+01)
      (Components|Sphere|SetSphereRadius (Variables|Default|GetLightOrb_CollisionSphere) 1e+01 true)
      (Variables|Status|SetIsOverheating false)
      (Variables|Status|SetbLightOrbSwitchProcess false)
      (Variables|Status|SetStatusHidden true))))

(fn SetLightOrbEaten
  (params (Condition :type Boolean) (NewParam :type BP%20Third%20Person%20Character%20Object%20Reference))
  (bind _m_lightorb (Variables|Default|GetM_LightOrb))
  (bind _m_lightorb_2 (Variables|Default|GetM_LightOrb))
  (bind _highlight_fx (Variables|Default|GetHighlight%20FX))
  (bind _output_get (Variables|Status|SetbIsEaten Condition))
  (if _output_get
    (Collision|SetCollisionEnabled (Variables|Default|GetLightOrb_CollisionSphere) "NoCollision")
    (Development|SetHiddeninGame (Variables|Default|GetLightOrb_Lighting) true false)
    (Collision|SetCollisionEnabled _m_lightorb_2 "NoCollision")
    (Development|SetHiddeninGame _m_lightorb_2 true false)
    (Development|SetHiddeninGame _highlight_fx true false)
    (Variables|Status|SetbDecayIsOnHold true)
    (else
      (Collision|SetCollisionEnabled (Variables|Default|GetLightOrb_CollisionSphere) "QueryOnly")
      (Development|SetHiddeninGame (Variables|Default|GetLightOrb_Lighting) false false)
      (Collision|SetCollisionEnabled _m_lightorb "QueryAndPhysics")
      (Development|SetHiddeninGame _m_lightorb false false)
      (Development|SetHiddeninGame _highlight_fx false false)
      (Variables|Status|SetbDecayIsOnHold false))))

(fn SetLightOrbConditionsAfterMechanicUse
  (bind _lightorb_lighting (Variables|Default|GetLightOrb_Lighting))
  (if (not (Variables|Status|GetbLightOrbSwitchProcess))
    (Variables|Status|SetbLightOrbSwitchProcess true)
    (CallFunction|TimelineLightChange (Variables|/Script/Engine.LightComponentBase|GetIntensity _lightorb_lighting) (Variables|Values|GetLightIntensitySave) (Variables|/Script/Engine.LocalLightComponent|GetAttenuationRadius _lightorb_lighting) (Variables|Values|GetLightAttenuationRadiusSave))
    (Components|Sphere|SetSphereRadius (Variables|Default|GetLightOrb_CollisionSphere) (Variables|Values|GetLightSphereRadiusSave) true)
    (Variables|Status|SetbLightOrbSwitchProcess false)
    (return)))

(fn SaveLightOrbConditionsatMechanicUse
  (params (isDuringMechanic :type Boolean) (orbStatus :type Integer))
  (bind _lightorb_lighting (Variables|Default|GetLightOrb_Lighting))
  (bind _status0to1values (Variables|Status|GetStatus0To1Values))
  (bind _status1to2values (Variables|Status|GetStatus1To2Values))
  (bind _status2to3values (Variables|Status|GetStatus2To3Values))
  (if isDuringMechanic
    (if (== orbStatus 0)
      (Variables|Values|SetLightIntensitySave (.Value (Utilities|Map|Find _status0to1values 0)))
      (Variables|Values|SetLightAttenuationRadiusSave (.Value (Utilities|Map|Find _status0to1values 1)))
      (Variables|Values|SetLightSphereRadiusSave (.Value (Utilities|Map|Find _status0to1values 2)))
      (return)
      (elif (== orbStatus 1)
        (Variables|Values|SetLightIntensitySave (.Value (Utilities|Map|Find _status1to2values 0)))
        (Variables|Values|SetLightAttenuationRadiusSave (.Value (Utilities|Map|Find _status1to2values 1)))
        (Variables|Values|SetLightSphereRadiusSave (.Value (Utilities|Map|Find _status1to2values 2)))
        (return)
        (elif (== orbStatus 2)
          (Variables|Values|SetLightIntensitySave (.Value (Utilities|Map|Find _status2to3values 0)))
          (Variables|Values|SetLightAttenuationRadiusSave (.Value (Utilities|Map|Find _status2to3values 1)))
          (Variables|Values|SetLightSphereRadiusSave (.Value (Utilities|Map|Find _status2to3values 2)))
          (return))))
    (else
      (Variables|Values|SetLightIntensitySave (Variables|/Script/Engine.LightComponentBase|GetIntensity _lightorb_lighting))
      (Variables|Values|SetLightAttenuationRadiusSave (Variables|/Script/Engine.LocalLightComponent|GetAttenuationRadius _lightorb_lighting))
      (Variables|Values|SetLightSphereRadiusSave (Variables|/Script/Engine.SphereComponent|GetSphereRadius (Variables|Default|GetLightOrb_CollisionSphere)))
      (return))))

(fn ConditionChange
  (params (LowerStatus :type Map%20of%20Integers%20to%20Reals) (HigherStatus :type Map%20of%20Integers%20to%20Reals) (bIsIncreasing :type Boolean))
  (bind _highlight_fx (Variables|Default|GetHighlight%20FX))
  (bind _lightorb_collisionsphere (Variables|Default|GetLightOrb_CollisionSphere))
  (if bIsIncreasing
    (CallFunction|TimelineLightChange (.Value (Utilities|Map|Find LowerStatus 0)) (.Value (Utilities|Map|Find HigherStatus 0)) (.Value (Utilities|Map|Find LowerStatus 1)) (.Value (Utilities|Map|Find HigherStatus 1)))
    (Components|Sphere|SetSphereRadius _lightorb_collisionsphere (.Value (Utilities|Map|Find HigherStatus 2)) true)
    ;[1 0.9864 0.3301] change particle amount
    ; 3 key (10,50,100,150)
    (Niagara|SetNiagaraVariable(Float) _highlight_fx "SpawnRate" (.Value (Utilities|Map|Find HigherStatus 3)))
    (else
      (CallFunction|TimelineLightChange (.Value (Utilities|Map|Find HigherStatus 0)) (.Value (Utilities|Map|Find LowerStatus 0)) (.Value (Utilities|Map|Find HigherStatus 1)) (.Value (Utilities|Map|Find LowerStatus 1)))
      (Components|Sphere|SetSphereRadius _lightorb_collisionsphere (.Value (Utilities|Map|Find LowerStatus 2)) true)
      (Niagara|SetNiagaraVariable(Float) _highlight_fx "SpawnRate" (.Value (Utilities|Map|Find LowerStatus 3)))))
  (Variables|Status|SetIsOverheating false)
  (return))