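; Lab puzzle actor that moves a light orb step by step from a start socket to an end socket via externally triggered events.
; When the start socket gets the orb, Tick notifies BP_Lab once, saves the orb's strength, overrides it and pauses decay.
; Timelines lerp the orb between given vectors, counting steps forward or back.
; At step eleven, socket state transfers to the end socket and orb strength and decay are restored.
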(event Custom|MoveOrbToStart
  (params (FromVector :type Vector) (ToVector :type Vector))
  ;[1 1 1] Comment
  (if (not (Variables|Default|GetbIsMoving))
    (Variables|Default|SetbIsMoving true)
    (bind _newtrack_0 (Timeline|ReverseMoveLightFromStartToEnd PlayFromStart)
      (:Update
        (Transformation|SetActorLocation (Variables|Default|GetLightOrbRef) (Math|Vector|Lerp(Vector) FromVector ToVector _newtrack_0) false false))
      (:Finished
        (Variables|Default|SetbIsMoving false)
        (bind _output_get (Variables|Default|SetstepsCompleted (- (Variables|Default|GetstepsCompleted) 1)))
        (if (< _output_get 0)
          _)))))

(event Custom|MoveOrbToEnd
  (params (FromVector :type Vector) (ToVector :type Vector))
  ;[1 1 1] Comment
  (if (not (Variables|Default|GetbIsMoving))
    (Variables|Default|SetbIsMoving true)
    (bind _newtrack_0 (Timeline|MoveLightFromStartToEnd PlayFromStart)
      (:Update
        (Transformation|SetActorLocation (Variables|Default|GetLightOrbRef) (Math|Vector|Lerp(Vector) FromVector ToVector _newtrack_0) false false))
      (:Finished
        (Variables|Default|SetbIsMoving false)
        (bind _output_get (Variables|Default|SetstepsCompleted (+ (Variables|Default|GetstepsCompleted) 1)))
        (if (== 11 _output_get)
          (CallFunction|EndReached))))))

(event Custom|EndReached
  (bind _startsocket (Variables|Default|GetStartSocket))
  (bind _lightorbref (Variables|Default|GetLightOrbRef))
  ;[1 1 1] Comment
  (CallFunction|ExchangeValues (Variables|Default|GetEndSocket) (Variables|Default|GetStartSocket))
  (Variables|/Game/MechanicsPlayground/MechanincsBlueprints/BP_PlaceLightSocket.BP_PlaceLightSocket_C|SetbLightOnSocket _startsocket false)
  (Default|SetLightOrbStrength _lightorbref (Variables|Default|GetLightOrbStrengthSave))
  (Variables|/Game/MechanicsPlayground/MechanincsBlueprints/BP_LightOrb.BP_LightOrb_C|SetbDecayIsOnHold _lightorbref false)
  (Actor|Tick|SetActorTickEnabled _startsocket))

(event Collision|EventActorBeginOverlap
  (params (OtherActor :type Actor%20Object%20Reference)))

(event EventTick
  (params (DeltaSeconds :type Float%20%28single-precision%29))
  ;[1 1 1] Comment
  (if (Variables|/Game/MechanicsPlayground/MechanincsBlueprints/BP_PlaceLightSocket.BP_PlaceLightSocket_C|GetbLightOnSocket (Variables|Default|GetStartSocket))
    (if (not (Variables|/Game/MechanicsPlayground/MechanincsBlueprints/BP_PlaceLightSocket.BP_PlaceLightSocket_C|GetbLightOnSocket (Variables|Default|GetEndSocket)))
      (Variables|Default|SetLightOrbRef (Variables|/Game/MechanicsPlayground/MechanincsBlueprints/BP_PlaceLightSocket.BP_PlaceLightSocket_C|GetLightOrbRef (Variables|Default|GetStartSocket)))
      (Utilities|FlowControl|DoOnce false
        (:Completed
          (bind _returnvalue (Actor|GetActorOfClass "/Game/MechanicsPlayground/MechanincsBlueprints/Buttons/Lab/BP_Lab.BP_Lab_C"))
          (Default|FirstMove _returnvalue)
          (bind _lightorbstatus (Default|GetLightOrbStrength (Variables|Default|GetLightOrbRef)))
          (Variables|Default|SetLightOrbStrengthSave _lightorbstatus)
          (Variables|/Game/MechanicsPlayground/MechanincsBlueprints/BP_LightOrb.BP_LightOrb_C|SetbDecayIsOnHold (Variables|Default|GetLightOrbRef) true)
          (Variables|/Game/MechanicsPlayground/MechanincsBlueprints/BP_LightOrb.BP_LightOrb_C|SetbIsIncreasing (Variables|Default|GetLightOrbRef) false)
          (Default|SetLightOrbStrength (Variables|Default|GetLightOrbRef) 2.0)
          (Default|SetLightOrbConditions (Variables|Default|GetLightOrbRef)))))))

(fn ConstructionScript)

(fn ExchangeValues
  (params (EndSocket :type BP%20Place%20Light%20Socket%20Object%20Reference) (StartSocket :type BP%20Place%20Light%20Socket%20Object%20Reference))
  (Variables|/Game/MechanicsPlayground/MechanincsBlueprints/BP_PlaceLightSocket.BP_PlaceLightSocket_C|SetTimeOfLightInSocket EndSocket (Variables|/Game/MechanicsPlayground/MechanincsBlueprints/BP_PlaceLightSocket.BP_PlaceLightSocket_C|GetTimeOfLightInSocket StartSocket))
  (Variables|/Game/MechanicsPlayground/MechanincsBlueprints/BP_PlaceLightSocket.BP_PlaceLightSocket_C|SetPlayerRef EndSocket (Variables|/Game/MechanicsPlayground/MechanincsBlueprints/BP_PlaceLightSocket.BP_PlaceLightSocket_C|GetPlayerRef StartSocket))
  (Variables|/Game/MechanicsPlayground/MechanincsBlueprints/BP_PlaceLightSocket.BP_PlaceLightSocket_C|SetLightOrbRef EndSocket (Variables|/Game/MechanicsPlayground/MechanincsBlueprints/BP_PlaceLightSocket.BP_PlaceLightSocket_C|GetLightOrbRef StartSocket))
  (Variables|/Game/MechanicsPlayground/MechanincsBlueprints/BP_PlaceLightSocket.BP_PlaceLightSocket_C|SetbLightOnSocket EndSocket true)
  (Variables|/Game/ThirdPerson/Blueprints/BP_ThirdPersonCharacter.BP_ThirdPersonCharacter_C|SetNearestLightSocketRef (Variables|/Game/MechanicsPlayground/MechanincsBlueprints/BP_PlaceLightSocket.BP_PlaceLightSocket_C|GetPlayerRef EndSocket) EndSocket))

(fn GetActiveLocation
  (return (Variables|Default|GetstepsCompleted)))