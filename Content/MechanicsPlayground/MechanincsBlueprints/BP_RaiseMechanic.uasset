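; BP_RaiseMechanic is a mechanics-playground actor that stays lit while active and can damage actors overlapping it, excluding the player character.
; On overlap, it casts player 0's pawn to BP_ThirdPersonCharacter and, if DoesDamage is set, applies BaseDamage to any other actor.
; Tick polls IsActive, showing RaisedLight while true; once false, it hides the light and destroys the actor.
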(event EventBeginPlay)

(event Collision|EventActorBeginOverlap
  (params (OtherActor :type Actor%20Object%20Reference))
  (bind _asbp_third_person_character (Utilities|Casting|CastToBP_ThirdPersonCharacter (Game|GetPlayerCharacter 0)))
  (if (!= OtherActor _asbp_third_person_character)
    (if (Variables|Default|GetbDoesDamage)
      (Game|Damage|ApplyDamage OtherActor (Variables|Default|GetBaseDamage) 0 0))))

(event EventTick
  (params (DeltaSeconds :type Float%20%28single-precision%29))
  (if (Variables|Default|GetbIsActive)
    (Rendering|SetVisibility (Variables|Default|GetRaisedLight) true false)
    (else
      (Rendering|SetVisibility (Variables|Default|GetRaisedLight) false false)
      (Actor|DestroyActor))))

(fn ConstructionScript)