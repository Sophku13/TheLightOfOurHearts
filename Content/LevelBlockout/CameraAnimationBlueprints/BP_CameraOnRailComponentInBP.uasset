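; Camera-on-rail actor that slides its Camera along a Spline to follow the player character while ActiveCamera is set.
; Each tick, GetClosestPositionAlongSpline samples the spline at fixed intervals to find the distance nearest the player.
; The camera lerps toward a point slightly before that distance, using frame delta time as alpha for smoothing, and changes only its location.
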(event EventBeginPlay
  (|CallParentFunction) ; This node is disabled and will not be called.\nDrag off pins to build functionality.
)

(event Collision|EventActorBeginOverlap
  (params (OtherActor :type Actor%20Object%20Reference))
  (|CallParentFunction OtherActor) ; This node is disabled and will not be called.\nDrag off pins to build functionality.
)

(event EventTick
  (params (DeltaSeconds :type Float%20%28single-precision%29))
  (bind _camera (Variables|Default|GetCamera))
  (|CallParentFunction DeltaSeconds)
  (if (Variables|Default|GetActiveCamera)
    (bind _lengthatclosestposition (CallFunction|GetClosestPositionAlongSpline (Transformation|GetActorLocation (Game|GetPlayerCharacter 0))))
    (Transformation|SetWorldLocation _camera (Math|Vector|Lerp(Vector) (Transformation|GetWorldLocation _camera) (Spline|GetLocationatDistanceAlongSpline (Variables|Default|GetSpline) (Math|Float|Max(Float) (- _lengthatclosestposition 1e+01) 0.0) "World") (* (Utilities|Time|GetWorldDeltaSeconds) 1.0)) false false)))

(fn ConstructionScript
  (|CallParentFunction))

(fn GetClosestPositionAlongSpline
  (params (ThePlayerIsHere :type Vector))
  (bind _spline (Variables|Default|GetSpline))
  (if (< (LocalVariables|GetCheckingWhereWeAreAtSpline) (Spline|GetSplineLength _spline)) :!label _label
    (if (> (LocalVariables|GetClosestDistanceBetweenPlayerAndCamera) (Math|Vector|Distance(Vector) (Spline|GetLocationatDistanceAlongSpline _spline (LocalVariables|GetCheckingWhereWeAreAtSpline) "World") ThePlayerIsHere))
      (LocalVariables|SetClosestDistanceBetweenPlayerAndCamera (Math|Vector|Distance(Vector) (Spline|GetLocationatDistanceAlongSpline _spline (LocalVariables|GetCheckingWhereWeAreAtSpline) "World") ThePlayerIsHere))
      (LocalVariables|SetPositionOnSplineAtClosest (LocalVariables|GetCheckingWhereWeAreAtSpline)))
    (LocalVariables|SetCheckingWhereWeAreAtSpline (+ (LocalVariables|GetCheckingWhereWeAreAtSpline) 1e+02))
    (goto _label)
    (else
      (return (LocalVariables|GetPositionOnSplineAtClosest)))))