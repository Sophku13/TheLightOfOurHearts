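; A single-button actor that sends an activation message to a linked Door when the player interacts with it.
; If flagged activatable, it works and reports as interactable only after OnActivation sets it active; otherwise it always works.
; Each valid press calls MoveButton, messages the Door, then calls MoveButton again after a short delay.
; Tick swaps the button's red emissive material between on and off for activatable buttons.
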(event EventBeginPlay
  (|CallParentFunction) ; This node is disabled and will not be called.\nDrag off pins to build functionality.
)

(event Collision|EventActorBeginOverlap
  (params (OtherActor :type Actor%20Object%20Reference))
  (|CallParentFunction OtherActor) ; This node is disabled and will not be called.\nDrag off pins to build functionality.
)

(event EventTick
  (params (DeltaSeconds :type Float%20%28single-precision%29))
  (if (Variables|Default|GetbIsActivatable)
    (if (Variables|Default|GetbIsActive)
      (Rendering|Material|SetMaterial (Variables|Default|GetButton) 0 "/Game/Materials/MI_Sphere_Emissive_Red.MI_Sphere_Emissive_Red")
      (else
        (Rendering|Material|SetMaterial (Variables|Default|GetButton) 0 "/Game/Materials/MI_Sphere_Emissive_Red_Off.MI_Sphere_Emissive_Red_Off")))))

(event EventOnActivation
  (Variables|Default|SetbIsActive true))

(event EventOnInteract
  (if (Variables|Default|GetbIsActivatable)
    (if (Variables|Default|GetbIsActive)
      (CallFunction|MoveButton)
      (Class|BPILightFueledActivation|OnActivation(Message) (Variables|Default|GetDoor))
      (Utilities|FlowControl|Delay 2.0 :!label _label)
      (CallFunction|MoveButton))
    (else
      (CallFunction|MoveButton)
      (Class|BPILightFueledActivation|OnActivation(Message) (Variables|Default|GetDoor))
      (goto _label))))

(fn ConstructionScript
  (|CallParentFunction))

(fn IsInteractable
  (if (Variables|Default|GetbIsActivatable)
    (return (Variables|Default|GetbIsActive))
    (else
      (return true))))